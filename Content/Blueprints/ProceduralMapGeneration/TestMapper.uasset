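; TestMapper is a debug test actor for procedural map generation that visualizes a point-based map layout.
; On BeginPlay it scatters about a hundred random, vertically flattened points, then builds a 2D Delaunay triangulation and derives a Voronoi diagram with a circumcenter distance cap.
; It draws both edge sets as colored debug lines.
; An unused branch connects ranked points and spawns TestIsl actors scaled by rank.
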(event EventBeginPlay
  (bind _self self)
  (for _index (range 0 100)
    (bind _returnvalue (Utilities|Array|Add (Variables|Default|GetMapPoints) (* (* (Math|Random|RandomUnitVector) (Math|Vector|MakeVector (Math|Random|RandomFloatinRange 3.0 4.0) (Math|Random|RandomFloatinRange 3.0 4.0) (Math|Random|RandomFloatinRange 0.1 0.75))) 1e+05))))
  (bind (_tris _edges) (Class|WorldGenFuncLib|Delaunay2D _self (Variables|Default|GetMapPoints)))
  (for _array_element _edges
    (Rendering|Debug|DrawDebugLine (.A (Utilities|Struct|BreakSpanEdge _array_element)) (.B (Utilities|Struct|BreakSpanEdge _array_element)) "(R=0.000000,G=1.000000,B=1.000000,A=1.000000)" 1e+04 1e+03))
  (bind _outvoronoi (Class|WorldGenFuncLib|Delaunay2DtoVoronoi2D _self _tris 1.75e+05))
  (for _array_element_2 _outvoronoi
    (Rendering|Debug|DrawDebugLine (.A (Utilities|Struct|BreakSpanEdge _array_element_2)) (.B (Utilities|Struct|BreakSpanEdge _array_element_2)) "(R=1.000000,G=0.000000,B=0.000000,A=1.000000)" 1e+04 1e+03)))

(fn ConstructionScript)