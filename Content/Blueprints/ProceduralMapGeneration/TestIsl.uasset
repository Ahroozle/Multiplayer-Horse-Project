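; TestIsl is a procedural island shape prototype that, as wired, only draws a debug cone on BeginPlay to show its bounds.
; Disconnected generation logic builds randomized point rings that taper along EndPoint, linking them with debug lines into a wireframe hull.
; That logic uses SpawnHullPoint for jittered ring points and can randomly call SpawnSmaller to spawn scaled, tilted child TestIsl actors that cannot branch further.
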(event EventBeginPlay
  (bind _returnvalue (Transformation|GetActorScale3D))
  (bind _returnvalue_2 (Transformation|GetActorUpVector))
  (bind _mainradius (Variables|Default|GetMainRadius))
  (bind _endpoint (Variables|Default|GetEndPoint))
  (bind _secondaryradiusrange (Variables|Default|GetSecondaryRadiusRange))
  (bind _returnvalue_3 (Math|Vector|GetMaxElement _returnvalue))
  (bind _returnvalue_4 (Math|Vector|VectorLength _endpoint))
  (bind _returnvalue_5 (+ _mainradius (.y _secondaryradiusrange)))
  (bind _returnvalue_6 (* _returnvalue_4 _returnvalue_3))
  (bind _returnvalue_7 (* _returnvalue_3 _returnvalue_5))
  (bind _returnvalue_8 (/ _returnvalue_7 _returnvalue_6))
  (bind _returnvalue_9 (Class|KismetMathLibrary|DegAtan _returnvalue_8))
  (Class|KismetSystemLibrary|DrawDebugConeinDegrees (- (Transformation|GetActorLocation) (* _returnvalue_2 _returnvalue_6)) _returnvalue_2 _returnvalue_6 _returnvalue_9 _returnvalue_9 12 "(R=1.000000,G=0.000000,B=0.000000,A=1.000000)" 1e+04 1e+03))

(fn ConstructionScript)

(fn SpawnHullPoint
  (bind _rootdir (Variables|Default|GetRootDir))
  (bind _secondaryradiusrange (Variables|Default|GetSecondaryRadiusRange))
  (bind _secondaryanglerange (Variables|Default|GetSecondaryAngleRange))
  (bind _returnvalue (Math|Random|RandomFloatinRange (.x _secondaryanglerange) (.y _secondaryanglerange)))
  (bind _returnvalue_2 (Math|Vector|RotateVectorAroundAxis _rootdir _returnvalue "0, 0,1.000000"))
  (return (+ (* (* (+ (* (Variables|Default|GetRootDir) (Variables|Default|GetMainRadius)) (* (Math|Vector|SelectVector _returnvalue_2 (Math|Vector|NegateVector _returnvalue_2) (Math|Random|RandomBool)) (Math|Random|RandomFloatinRange (.x _secondaryradiusrange) (.y _secondaryradiusrange)))) (- 1.0 (/ (Math|Conversions|ToFloat(Integer) (Variables|Default|GetCurrSlice)) (Math|Conversions|ToFloat(Integer) (Variables|Default|GetSlices))))) (Transformation|GetActorScale3D)) (+ (Transformation|GetActorLocation) (* (Variables|Default|GetCurrPoint) (Transformation|GetActorScale3D))))))

(fn SpawnSmaller
  (bind _returnvalue (Transformation|GetActorLocation))
  (bind _returnvalue_2 (Transformation|GetActorScale3D))
  (bind _currpoint (Variables|Default|GetCurrPoint))
  (bind _returnvalue_3 (* _returnvalue_2 _currpoint))
  (bind _returnvalue_4 (+ _returnvalue _returnvalue_3))
  (LocalVariables|SetScale (- 1.0 (/ (Math|Conversions|ToFloat(Integer) (Variables|Default|GetCurrSlice)) (Math|Conversions|ToFloat(Integer) (Variables|Default|GetSlices)))))
  (bind _output_get (LocalVariables|SetChildLoc (+ (Transformation|GetActorLocation) (* (Transformation|GetActorScale3D) (+ (Variables|Default|GetCurrPoint) (* (Math|Vector|Normalize (* (Math|Random|RandomUnitVector) "1.000000,1.000000, 0")) (* (* (Variables|Default|GetMainRadius) 0.5) (LocalVariables|GetScale))))))))
  (Rendering|Debug|DrawDebugArrow :LineStart _output_get :LineEnd _returnvalue_4 :ArrowSize 1e+01 :Duration 1e+04 :Thickness 1e+01)
  (Game|SpawnActorfromClass "TestIsl_C" (Math|Transform|MakeTransform (LocalVariables|GetChildLoc) (Math|Vector|RotatorfromAxisandAngle (Math|Vector|RotateVectorAroundAxis (Math|Vector|Normalize (- (LocalVariables|GetChildLoc) _returnvalue_4)) 9e+01 "0, 0,1.000000") (Math|Random|RandomFloatinRange 0.0 -15.0)) (Math|Vector|MakeVector (.x (/ (Math|Conversions|ToVector(Float) (LocalVariables|GetScale)) 2.0)) (.y (/ (Math|Conversions|ToVector(Float) (LocalVariables|GetScale)) 2.0)) (.z (/ (Math|Conversions|ToVector(Float) (LocalVariables|GetScale)) 1.5)))) "Undefined" 0 false (+ (Variables|Default|GetCurrIteration) 1)))