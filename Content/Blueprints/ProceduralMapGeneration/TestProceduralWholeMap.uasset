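; Test actor that generates a procedural map from a random seed and visualizes its output maps on preview planes.
; After a startup delay it creates dynamic materials for the planes, binds the generation-finished delegate and calls Build.
; On completion it feeds height, color and offset textures to top and bottom terrain materials, and elevation, falloff, offset and steepness maps to debug planes.
; After another delay it requests the terrain isosurface on a procedural mesh.
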(event Custom|GenerationFinishedDelegate_Event_0
  (bind _botdyn (Variables|Default|GetBotDyn))
  (bind _topdyn (Variables|Default|GetTopDyn))
  (bind _topdyn_2 (Variables|Default|GetTopDyn))
  (Utilities|FlowControl|Sequence
    (:then_0
      (Rendering|Material|SetTextureParameterValue _topdyn "ColorMap" (Variables|Default|GetTopHeightMapColorTexture))
      (Rendering|Material|SetTextureParameterValue _topdyn "HeightMap" (Variables|Default|GetTopHeightMapTexture))
      (Rendering|Material|SetTextureParameterValue _botdyn "ColorMap" (Variables|Default|GetBottomHeightMapColorTexture))
      (Rendering|Material|SetTextureParameterValue _botdyn "HeightMap" (Variables|Default|GetBottomHeightMapTexture))
      (Rendering|Material|SetTextureParameterValue _topdyn_2 "OffsetMap" (Variables|Default|GetOffsetMapTexture))
      (Rendering|Material|SetScalarParameterValue _topdyn_2 "ZScale" (.z (Transformation|GetWorldScale (Variables|Default|GetAll))) :!class /Script/Engine.MaterialInstanceDynamic))
    (:then_1
      (Rendering|Material|SetTextureParameterValue (Variables|Default|GetElevTopDyn) "Map" (Variables|Default|GetTopHeightMapTexture))
      (Rendering|Material|SetTextureParameterValue (Variables|Default|GetElevBotDyn) "Map" (Variables|Default|GetBottomHeightMapTexture)))
    (:then_2
      (Rendering|Material|SetTextureParameterValue (Variables|Default|GetFalloffDyn) "Map" (Variables|Default|GetFalloffMapTexture))
      (Rendering|Material|SetTextureParameterValue (Variables|Default|GetOffsetDyn) "Map" (Variables|Default|GetOffsetMapTexture))
      (Rendering|Material|SetTextureParameterValue (Variables|Default|GetSteepnessDyn) "Map" (Variables|Default|GetSteepnessMapTexture)))
    (:then_3
      (Utilities|FlowControl|Delay 5.0)
      (Class|ProceduralWholeMap|GetTerrainIsosurface (Variables|Default|GetProceduralMesh1)))))

(event EventBeginPlay
  (Utilities|FlowControl|Delay 5.0)
  (Utilities|FlowControl|Sequence
    (:then_0
      (bind _returnvalue (Rendering|Material|CreateDynamicMaterialInstance (Variables|Default|GetTopPlane) 0 0 :!class /Script/Engine.PrimitiveComponent))
      (Variables|Default|SetTopDyn _returnvalue)
      (bind _returnvalue_2 (Rendering|Material|CreateDynamicMaterialInstance (Variables|Default|GetBottomPlane) 0 0 :!class /Script/Engine.PrimitiveComponent))
      (Variables|Default|SetBotDyn _returnvalue_2))
    (:then_1
      (bind _returnvalue_3 (Rendering|Material|CreateDynamicMaterialInstance (Variables|Default|GetTopElev) 0 0 :!class /Script/Engine.PrimitiveComponent))
      (Variables|Default|SetElevTopDyn _returnvalue_3)
      (bind _returnvalue_4 (Rendering|Material|CreateDynamicMaterialInstance (Variables|Default|GetBotElev) 0 0 :!class /Script/Engine.PrimitiveComponent))
      (Variables|Default|SetElevBotDyn _returnvalue_4))
    (:then_2
      (bind _returnvalue_5 (Rendering|Material|CreateDynamicMaterialInstance (Variables|Default|GetFalloff) 0 0 :!class /Script/Engine.PrimitiveComponent))
      (Variables|Default|SetFalloffDyn _returnvalue_5)
      (bind _returnvalue_6 (Rendering|Material|CreateDynamicMaterialInstance (Variables|Default|GetOffset) 0 0 :!class /Script/Engine.PrimitiveComponent))
      (Variables|Default|SetOffsetDyn _returnvalue_6)
      (bind _returnvalue_7 (Rendering|Material|CreateDynamicMaterialInstance (Variables|Default|GetSteepness) 0 0 :!class /Script/Engine.PrimitiveComponent))
      (Variables|Default|SetSteepnessDyn _returnvalue_7))
    (:then_3
      (EventDispatchers|AssignGenerationFinishedDelegate (delegate Custom|GenerationFinishedDelegate_Event_0))
      (Class|ProceduralWholeMap|Build (Math|Random|RandomInteger 2147483647)))))

(fn ConstructionScript)