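; Island shape function for procedural map generation that decides whether each map cell is ground, using a radial sine-based outline.
; Initialize draws bump count, start angle, and dip angle and width from the seeded world random stream.
; CellIsGround converts the cell center to angle and blended distance, then compares it against two wavy radii, flattened inside the dip.
; IslandFactor sets the gap between inner landmass and outer ring.
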(event EventInitialize
  (bind _returnvalue (Class|WorldGenFuncLib|GetWorldRandom))
  (Variables|Default|SetBumps (Math|Random|RandomIntegerinRangefromStream (Variables|Default|GetMinBumps) (Variables|Default|GetMaxBumps) _returnvalue))
  (Variables|Default|SetStartAngle (Math|Random|RandomFloatinRangefromStream 0.0 (* (Math|Trig|GetPI) (Math|Float|MakeLiteralFloat 2.0)) _returnvalue))
  (Variables|Default|SetDipAngle (Math|Random|RandomFloatinRangefromStream 0.0 (* (Math|Trig|GetPI) (Math|Float|MakeLiteralFloat 2.0)) _returnvalue))
  (Variables|Default|SetDipWidth (Math|Random|RandomFloatinRangefromStream (Variables|Default|GetMinWidth) (Variables|Default|GetMaxWidth) _returnvalue)))

(fn CellIsGround
  (params (Cell :type World%20Cell%20Object%20Reference))
  (bind _returnvalue (Math|Trig|GetPI))
  (bind _returnvalue_2 (Math|Float|MakeLiteralFloat 2.0))
  (bind _celldata (Variables|/Script/MPHorso.WorldCell|GetCellData Cell))
  (bind _returnvalue_3 (Math|Conversions|ToVector2D(Vector) (.shapedata_center _celldata)))
  (bind _returnvalue_4 (* _returnvalue _returnvalue_2))
  (bind (_x _y) (Math|Vector2D|BreakVector2D _returnvalue_3))
  (LocalVariables|Setangle (Math|Trig|Atan2(Radians) _x _y))
  (LocalVariables|Setlength (* (Math|Float|MakeLiteralFloat 0.5) (+ (Math|Float|Max(Float) (Math|Float|Absolute(Float) _x) (Math|Float|Absolute(Float) _y)) (Math|Vector2D|Vector2DLength _returnvalue_3))))
  (if (Math|Boolean|ORBoolean (< (Math|Float|Absolute(Float) (- (LocalVariables|Getangle) (Variables|Default|GetDipAngle))) (Variables|Default|GetDipWidth)) (< (Math|Float|Absolute(Float) (+ (- (LocalVariables|Getangle) (Variables|Default|GetDipAngle)) _returnvalue_4)) (Variables|Default|GetDipWidth)) (< (Math|Float|Absolute(Float) (- (- (LocalVariables|Getangle) (Variables|Default|GetDipAngle)) _returnvalue_4)) (Variables|Default|GetDipWidth)))
    (bind _output_get (LocalVariables|Setr1 (Math|Float|MakeLiteralFloat 0.2)))
    (LocalVariables|Setr2 _output_get)
    (else
      (LocalVariables|Setr1 (+ (Math|Float|MakeLiteralFloat 0.5) (* (Math|Float|MakeLiteralFloat 0.4) (Math|Trig|Sin(Radians) (+ (Variables|Default|GetStartAngle) (* (Variables|Default|GetBumps) (LocalVariables|Getangle)) (* (Math|Trig|Cos(Radians) (Math|Conversions|ToFloat(Integer) (+ (Variables|Default|GetBumps) (Class|KismetSystemLibrary|MakeLiteralInteger 3)))) (LocalVariables|Getangle)))))))
      (LocalVariables|Setr2 (- (Math|Float|MakeLiteralFloat 0.7) (* (Math|Float|MakeLiteralFloat 0.2) (Math|Trig|Sin(Radians) (+ (Variables|Default|GetStartAngle) (* (Variables|Default|GetBumps) (LocalVariables|Getangle)) (* (Math|Trig|Cos(Radians) (Math|Conversions|ToFloat(Integer) (+ (Variables|Default|GetBumps) (Class|KismetSystemLibrary|MakeLiteralInteger 2)))) (LocalVariables|Getangle)))))))))
  (return (or (< (LocalVariables|Getlength) (LocalVariables|Getr1)) (and (> (LocalVariables|Getlength) (* (LocalVariables|Getr1) (Variables|Default|GetIslandFactor))) (< (LocalVariables|Getlength) (LocalVariables|Getr2))))))