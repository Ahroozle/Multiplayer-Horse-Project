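; World shape function for procedural map generation that decides whether a 2D point is ground, using ANL noise.
; Initialize resets the noise kernel and averages domain-scaled simplex and linear gradient noise, both seeded from the world random stream.
; CellIsGround remaps the noise to 0–1 and compares it to a threshold rising with squared distance from the origin, favoring a central island-like landmass.
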(event EventInitialize
  (Class|ANLFacadeLib|ANLResetNoiseKernel)
  (bind _returnvalue (Class|WorldGenFuncLib|GetWorldRandom))
  (bind _returnvalue_2 (Class|ANLFacadeLib|ANLSimplexBasis (Class|ANLFacadeLib|ANLSeed (Class|KismetMathLibrary|RandomIntegerfromStream 1073741823 _returnvalue))))
  (bind _returnvalue_3 (Class|ANLFacadeLib|ANLGradientBasis (Class|ANLFacadeLib|ANLConstant (Math|Conversions|ToFloat(Byte) (Utilities|Enum|LiteralenumEANL_InterpType "INTERP_LINEAR"))) (Class|ANLFacadeLib|ANLSeed (Class|KismetMathLibrary|RandomIntegerfromStream 1073741823 _returnvalue))))
  (Variables|Default|SetTest (Class|ANLFacadeLib|ANLDivide (Class|ANLFacadeLib|ANLAdd (Class|ANLFacadeLib|ANLScaleDomain _returnvalue_2 (Class|ANLFacadeLib|ANLConstant 2.5)) (Class|ANLFacadeLib|ANLScaleDomain _returnvalue_3 (Class|ANLFacadeLib|ANLConstant 3.0))) (Class|ANLFacadeLib|ANLConstant 2.0))))

(fn CellIsGround
  (params (Pt :type Vector))
  (bind _returnvalue (Math|Conversions|ToVector2D(Vector) Pt))
  (bind (_x _y) (Math|Vector2D|BreakVector2D _returnvalue))
  (bind _returnvalue_2 (Class|ANLFacadeLib|ANLEvaluateScalar 2 _x _y 0.0 0.0 0.0 0.0 (Variables|Default|GetTest)))
  (bind _output_get (LocalVariables|SetRes (* (+ _returnvalue_2 1.0) 0.5)))
  (return (> _output_get (+ 0.3 (* 0.3 (Class|KismetMathLibrary|VSize2DSquared _returnvalue))))))