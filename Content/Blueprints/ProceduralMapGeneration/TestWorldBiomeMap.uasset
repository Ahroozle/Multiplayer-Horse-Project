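; TestWorldBiomeMap is a procedural map generation Blueprint that assigns a final biome from a preliminary biome and environment data.
; DetermineBiome splits ground into four elevation bands, then picks a biome by moisture within each, in the style of a Whittaker diagram.
; Water becomes marsh at very low elevation and ice at high elevation; other water and all other preliminary biomes pass through unchanged.
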(fn DetermineBiome
  (params (PreBiome :type EBiomeType%20Enum%20%28by%20ref%29 :default "BIOME_HOLE") (EnvironmentData :type Environment%20Data%20Structure%20%28by%20ref%29))
  (bind (_elevation _moisture) (Utilities|Struct|BreakEnvironmentData EnvironmentData))
  (if (Utilities|Enum|Equal(Enum) PreBiome (Utilities|Enum|LiteralenumEBiomeType "BIOME_GROUND"))
    (if (> _elevation 0.8)
      (if (> _moisture 0.5)
        (return "BIOME_SNOW")
        (elif (> _moisture 0.33)
          (return "BIOME_TUNDRA")
          (elif (> _moisture 0.16)
            (return "BIOME_BARE")
            (else
              (return "BIOME_SCORCHED")))))
      (elif (> _elevation 0.6)
        (if (> _moisture 0.66)
          (return "BIOME_TAIGA")
          (elif (> _moisture 0.33)
            (return "BIOME_SHRUBLAND")
            (else
              (return "BIOME_TEMP_DESERT"))))
        (elif (> _elevation 0.3)
          (if (> _moisture 0.83)
            (return "BIOME_TEMP_RAINFOREST")
            (elif (> _moisture 0.5)
              (return "BIOME_TEMP_DECID_FOREST")
              (elif (> _moisture 0.16)
                (return "BIOME_GRASSLAND")
                (else
                  (return "BIOME_TEMP_DESERT")))))
          (elif (> _moisture 0.66)
            (return "BIOME_TROP_RAINFOREST")
            (elif (> _moisture 0.33)
              (return "BIOME_TROP_SEASONAL_FOREST")
              (elif (> _moisture 0.16)
                (return "BIOME_GRASSLAND")
                (else
                  (return "BIOME_SUBTROP_DESERT"))))))))
    (else
      (if (Utilities|Enum|Equal(Enum) PreBiome (Utilities|Enum|LiteralenumEBiomeType "BIOME_WATER"))
        (if (< _elevation 0.1)
          (return "BIOME_MARSH")
          (elif (> _elevation 0.8)
            (return "BIOME_ICE")
            (else
              _))))
      (return PreBiome))))