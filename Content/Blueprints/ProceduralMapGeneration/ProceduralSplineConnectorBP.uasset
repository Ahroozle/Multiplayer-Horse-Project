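; Procedural map generation Blueprint that lines a spline with spline mesh segments, split into consecutive sections by mesh type.
; ConstructMeshes divides the points across MeshData entries and creates each segment with a seeded random mesh from its section.
; UpdateMeshes compares point counts, adds one segment to a smallest section or removes one from a largest, then refits segments to the spline.
; Per-section index arrays shift to track inserts and removals.
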(fn ConstructionScript
  (|CallParentFunction))

(fn ConstructMeshes
  (params (RandStream :type Random%20Stream%20Structure%20%28by%20ref%29))
  (bind _rootspline (Variables|Default|GetRootSpline))
  (bind _rootspline_2 (Variables|Default|GetRootSpline))
  (bind _returnvalue (Spline|GetNumberOfSplinePoints _rootspline_2))
  (Utilities|FlowControl|Sequence
    (:then_0
      (Variables|Default|SetPreviousNumPoints _returnvalue)
      (LocalVariables|SetPointOffs (Math|Float|Floor (/ (Math|Conversions|ToFloat(Integer) _returnvalue) (Math|Conversions|ToFloat(Integer) (Utilities|Array|Length (Variables|Default|GetMeshData))))))
      (for _index (range 1 (Utilities|Array|LastIndex (Variables|Default|GetMeshData)))
        (Utilities|Array|Add (LocalVariables|GetMeshChangePoints) (* _index (LocalVariables|GetPointOffs)))))
    (:then_1
      (for _index_2 (range 0 (- (Spline|GetNumberOfSplinePoints (Variables|Default|GetRootSpline)) 2))
        (if (== _index_2 (Utilities|Array|Get(acopy) (LocalVariables|GetMeshChangePoints)))
          (Math|Integer|IncrementInt (LocalVariables|GetCurrMeshInd)
            (:%20%20
              (Utilities|Array|RemoveIndex (LocalVariables|GetMeshChangePoints)))))
        (Utilities|Array|Add (Utilities|Struct|BreakSplineConnectorMeshData (Utilities|Array|Get(acopy) (Variables|Default|GetMeshData) (LocalVariables|GetCurrMeshInd))) _index_2)
        (bind _newsplinemesh (CallFunction|CreateMeshComponent (LocalVariables|GetCurrMeshInd) RandStream))
        (SplineMesh|SetStartandEnd _newsplinemesh (.Location (Spline|GetLocationandTangentatSplinePoint _rootspline _index_2 "Local")) (.Tangent (Spline|GetLocationandTangentatSplinePoint _rootspline _index_2 "Local")) (.Location (Spline|GetLocationandTangentatSplinePoint _rootspline (+ _index_2 1) "Local")) (.Tangent (Spline|GetLocationandTangentatSplinePoint _rootspline (+ _index_2 1) "Local")) true :!class /Script/Engine.SplineMeshComponent)
        (Utilities|Array|Add (Variables|Default|GetCreatedMeshComponents) _newsplinemesh))
      (return true))))

(fn UpdateMeshes
  (params (RandStream :type Random%20Stream%20Structure%20%28by%20ref%29))
  (bind _rootspline (Variables|Default|GetRootSpline))
  (Math|Integer|CompareInt (Spline|GetNumberOfSplinePoints (Variables|Default|GetRootSpline)) (Variables|Default|GetPreviousNumPoints)
    (:>
      (CallFunction|AddMesh RandStream))
    (:==
      _)
    (:<
      (CallFunction|RemoveMesh RandStream)))
  ;[1 1 1] Update all of the mesh components to accomodate the new positioning
  (for _index (range 0 (- (Spline|GetNumberOfSplinePoints (Variables|Default|GetRootSpline)) 2))
    (SplineMesh|SetStartandEnd (Utilities|Array|Get(acopy) (Variables|Default|GetSpawnedMeshComponents) _index) (.Location (Spline|GetLocationandTangentatSplinePoint _rootspline _index "Local")) (.Tangent (Spline|GetLocationandTangentatSplinePoint _rootspline _index "Local")) (.Location (Spline|GetLocationandTangentatSplinePoint _rootspline (+ _index 1) "Local")) (.Tangent (Spline|GetLocationandTangentatSplinePoint _rootspline (+ _index 1) "Local")) true :!class /Script/Engine.SplineMeshComponent))
  (return true))

(fn CreateMeshComponent
  (params (MeshDataIndex :type Integer) (RandStream :type Random%20Stream%20Structure%20%28by%20ref%29))
  (bind _meshdata (Variables|Default|GetMeshData))
  (bind _item (Utilities|Array|Get(acopy) _meshdata MeshDataIndex))
  (bind _segmentmeshes (Utilities|Struct|BreakSplineConnectorMeshData _item))
  (bind _returnvalue (AddComponent|AddSplineMeshComponent false))
  (Components|StaticMesh|SetStaticMesh _returnvalue (Utilities|Array|Get(acopy) _segmentmeshes (Math|Random|RandomIntegerinRangefromStream 0 (Utilities|Array|LastIndex _segmentmeshes) RandStream)))
  (Transformation|AttachComponentToComponent _returnvalue 0 "None" "KeepRelative" "KeepRelative" "KeepRelative" true)
  (return _returnvalue))

(fn AddMesh
  (params (RandStream :type Random%20Stream%20Structure%20%28by%20ref%29))
  ;[1 1 1] Spawn a new splinemeshcomponent to fill the new gap created by the added point.
  (bind _outsmallest (Class|ProceduralSplineConnector|GetSmallestMeshTypeSectionIndices))
  (LocalVariables|SetRelevantIndex (Utilities|Array|Get(acopy) _outsmallest (Math|Random|RandomIntegerinRangefromStream 0 (Utilities|Array|LastIndex _outsmallest) RandStream)))
  (bind _newsplinemesh (CallFunction|CreateMeshComponent (LocalVariables|GetRelevantIndex) RandStream))
  (LocalVariables|SetRelevantMesh _newsplinemesh)
  (if (== (LocalVariables|GetRelevantIndex) (Utilities|Array|LastIndex (Variables|Default|GetMeshData)))
    ;[1 1 1] Early-Out in case the smallest index is the last one; No indices in front need to be updated.
    (bind _returnvalue (Utilities|Array|Add (Variables|Default|GetSpawnedMeshComponents) (LocalVariables|GetRelevantMesh)))
    (Utilities|Array|Add (Utilities|Struct|BreakSplineConnectorMeshData (Utilities|Array|Get(acopy) (Variables|Default|GetMeshData) (LocalVariables|GetRelevantIndex))) _returnvalue)
    (else
      ;[1 1 1] Inserts the newly-spawned mesh at the index right after the last index in the relevant data's index array.
      (Utilities|Array|Insert (Variables|Default|GetSpawnedMeshComponents) (LocalVariables|GetRelevantMesh) (Utilities|Array|Get(acopy) (Utilities|Struct|BreakSplineConnectorMeshData (Utilities|Array|Get(acopy) (Variables|Default|GetMeshData) (+ (LocalVariables|GetRelevantIndex) 1)))))
      (Utilities|Array|Add (Utilities|Struct|BreakSplineConnectorMeshData (Utilities|Array|Get(acopy) (Variables|Default|GetMeshData) (LocalVariables|GetRelevantIndex))) (Utilities|Array|Get(acopy) (Utilities|Struct|BreakSplineConnectorMeshData (Utilities|Array|Get(acopy) (Variables|Default|GetMeshData) (+ (LocalVariables|GetRelevantIndex) 1)))))
      ;[1 1 1] Moves all indices in front forward by 1
      (for _index (range (+ (LocalVariables|GetRelevantIndex) 1) (Utilities|Array|LastIndex (Variables|Default|GetMeshData)))
        (for (_array_element _array_index) (Utilities|Struct|BreakSplineConnectorMeshData (Utilities|Array|Get(acopy) (Variables|Default|GetMeshData) _index))
          (Utilities|Array|SetArrayElem (Utilities|Struct|BreakSplineConnectorMeshData (Utilities|Array|Get(acopy) (Variables|Default|GetMeshData) _index)) _array_index (+ _array_element 1)))))))

(fn RemoveMesh
  (params (RandStream :type Random%20Stream%20Structure%20%28by%20ref%29))
  (bind _spawnedmeshcomponents (Variables|Default|GetSpawnedMeshComponents))
  (bind _returnvalue (Utilities|Array|LastIndex _spawnedmeshcomponents))
  (bind _outlargest (Class|ProceduralSplineConnector|GetLargestMeshTypeSectionIndices))
  (LocalVariables|SetRelevantIndex (Utilities|Array|Get(acopy) _outlargest (Math|Random|RandomIntegerinRangefromStream 0 (Utilities|Array|LastIndex _outlargest) RandStream)))
  (if (== (LocalVariables|GetRelevantIndex) (Utilities|Array|LastIndex (Variables|Default|GetMeshData)))
    ;[1 1 1] Early-Out in case largest index is the last one; No indices in front need to be updated.
    (LocalVariables|SetRelevantMesh (Utilities|Array|Get(acopy) _spawnedmeshcomponents _returnvalue))
    (Utilities|Array|RemoveIndex (Variables|Default|GetSpawnedMeshComponents) _returnvalue)
    (Components|DestroyComponent (LocalVariables|GetRelevantMesh))
    (else
      ;[1 1 1] Destroys the relevant component and removes the index it originally occupied.
      (LocalVariables|SetRelevantMesh (Utilities|Array|Get(acopy) (Variables|Default|GetSpawnedMeshComponents) (Utilities|Array|Get(acopy) (Utilities|Struct|BreakSplineConnectorMeshData (Utilities|Array|Get(acopy) (Variables|Default|GetMeshData) (LocalVariables|GetRelevantIndex))) (Utilities|Array|LastIndex (Utilities|Struct|BreakSplineConnectorMeshData (Utilities|Array|Get(acopy) (Variables|Default|GetMeshData) (LocalVariables|GetRelevantIndex)))))))
      (Utilities|Array|RemoveIndex (Variables|Default|GetSpawnedMeshComponents) (Utilities|Array|Get(acopy) (Utilities|Struct|BreakSplineConnectorMeshData (Utilities|Array|Get(acopy) (Variables|Default|GetMeshData) (LocalVariables|GetRelevantIndex))) (Utilities|Array|LastIndex (Utilities|Struct|BreakSplineConnectorMeshData (Utilities|Array|Get(acopy) (Variables|Default|GetMeshData) (LocalVariables|GetRelevantIndex))))))
      (Components|DestroyComponent (LocalVariables|GetRelevantMesh))
      (Utilities|Array|RemoveIndex (Utilities|Struct|BreakSplineConnectorMeshData (Utilities|Array|Get(acopy) (Variables|Default|GetMeshData) (LocalVariables|GetRelevantIndex))) (Utilities|Array|LastIndex (Utilities|Struct|BreakSplineConnectorMeshData (Utilities|Array|Get(acopy) (Variables|Default|GetMeshData) (LocalVariables|GetRelevantIndex)))))
      ;[1 1 1] Moves all indices in front backward by 1 to fill the space back in
      (for _index (range (+ (LocalVariables|GetRelevantIndex) 1) (Utilities|Array|LastIndex (Variables|Default|GetMeshData)))
        (for (_array_element _array_index) (Utilities|Struct|BreakSplineConnectorMeshData (Utilities|Array|Get(acopy) (Variables|Default|GetMeshData) _index))
          (Utilities|Array|SetArrayElem (Utilities|Struct|BreakSplineConnectorMeshData (Utilities|Array|Get(acopy) (Variables|Default|GetMeshData) _index)) _array_index (- _array_element 1)))))))