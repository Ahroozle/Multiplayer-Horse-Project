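; TestWorldGenerator is a test actor that generates a procedural world and previews the result on a plane.
; On BeginPlay it calls Build for the "Test" world type with a random seed, then finds the TestWorldContinent actors.
; If any exist, it feeds the first one's biome, elevation and moisture textures, plus the plane's world scale, into a dynamic material on that plane.
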(event EventBeginPlay
  (bind _plane (Variables|Default|GetPlane))
  (bind _returnvalue (Transformation|GetWorldScale _plane))
  (Class|WorldGenerator|Build "Test" (Math|Random|RandomInteger 2147483647))
  (bind _outactors (Actor|GetAllActorsOfClass "/Game/Blueprints/ProceduralMapGeneration/TestWorldContinent.TestWorldContinent_C"))
  (if (> (Utilities|Array|Length _outactors) 0)
    (bind _returnvalue_2 (Rendering|Material|CreateDynamicMaterialInstance (Variables|Default|GetPlane) 0 0 :!class /Script/Engine.PrimitiveComponent))
    (Rendering|Material|SetTextureParameterValue _returnvalue_2 "Color" (Variables|/Script/MPHorso.WorldContinent|GetBiomeTexture (Utilities|Array|Get(acopy) _outactors)))
    (Rendering|Material|SetTextureParameterValue _returnvalue_2 "Elevation" (Variables|/Script/MPHorso.WorldContinent|GetElevationTexture (Utilities|Array|Get(acopy) _outactors)))
    (Rendering|Material|SetTextureParameterValue _returnvalue_2 "Moisture" (Variables|/Script/MPHorso.WorldContinent|GetMoistureTexture (Utilities|Array|Get(acopy) _outactors)))
    (Rendering|Material|SetVectorParameterValue _returnvalue_2 "Scale" (Utilities|Struct|MakeLinearColor (.x _returnvalue) (.y _returnvalue) (.z _returnvalue) 0.0) :!class /Script/Engine.MaterialInstanceDynamic)))

(fn ConstructionScript)