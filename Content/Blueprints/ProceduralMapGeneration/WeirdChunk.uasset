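; WeirdChunk is a procedural map generation chunk that builds itself from instanced static meshes at the locations in its ResponsiblePieces array.
; Gen starts a very short looping timer that adds one unrotated, unit-scale instance per tick and removes that location from the front of the array, spreading the work over time.
; When the array is empty, it clears the timer and prints its name with "Done".
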(event Custom|CustomEvent_0
  (if (> (Utilities|Array|Length (Variables|Default|GetResponsiblePieces)) 0)
    (Components|InstancedStaticMesh|AddInstance (Variables|Default|GetInstancedStaticMesh) (Math|Transform|MakeTransform (Utilities|Array|Get(acopy) (Variables|Default|GetResponsiblePieces)) "0, 0, 0" "1,1,1"))
    (Utilities|Array|RemoveIndex (Variables|Default|GetResponsiblePieces))
    (else
      (Utilities|Time|ClearandInvalidateTimerbyHandle (stale Custom|Gen _returnvalue))
      (Development|PrintString (Utilities|String|Append (Utilities|GetDisplayName self) " Done")))))

(event Custom|Gen
  (bind _returnvalue (Utilities|Time|SetTimerbyEvent (delegate Custom|CustomEvent_0) 0.001 true)))

(fn ConstructionScript)