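; Winged physics roomba that wanders on the server, turning to random headings on timers and driving forward.
; LookAhead traces wall and pawn whisker rays; hits trigger a back-up and a new heading built from mirrored hit vectors.
; While falling it flaps its wings, and an airborne hit briefly pauses driving.
; Flipped over, it hops with escalating velocity impulses, ending in a spinning launch.
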(event OnComponentHit(Roomba)
  (params (HitComponent :type Primitive%20Component%20Object%20Reference) (OtherActor :type Actor%20Object%20Reference) (OtherComp :type Primitive%20Component%20Object%20Reference) (NormalImpulse :type Vector) (Hit :type Hit%20Result%20Structure%20%28by%20ref%29))
  (if (CallFunction|IsFalling)
    (CallFunction|DoAirBonk)))

(event Custom|NewDir
  (Variables|Default|SetDirection (Math|Rotator|MakeRotfromZX (Math|Vector|MakeVector 0.0 0.0 1.0) (Math|Random|RandomUnitVector)))
  (Utilities|Time|ClearandInvalidateTimerbyHandle (Variables|Default|GetDirTimer))
  (Variables|Default|SetDoneTurning false))

(event Custom|Flip
  (bind _returnvalue (Utilities|Time|SetTimerbyEvent (delegate Custom|FlopHop1) 1.0))
  (Variables|Default|SetFlipTimer _returnvalue))

(event Custom|FlopHop1
  (Physics|SetPhysicsLinearVelocity (Variables|Default|GetRoomba) (* (Class|KismetMathLibrary|RandomUnitVectorinCone "0, 0,1.000000" (Math|Trig|DegreesToRadians (Math|Float|MakeLiteralFloat 1e+01))) 1e+02) false "None")
  (bind _returnvalue (Utilities|Time|SetTimerbyEvent (delegate Custom|FlopHop2) 2.0))
  (Variables|Default|SetFlipTimer _returnvalue))

(event Custom|FlopHop2
  (Physics|SetPhysicsLinearVelocity (Variables|Default|GetRoomba) (* (Class|KismetMathLibrary|RandomUnitVectorinCone "0, 0,1.000000" (Math|Trig|DegreesToRadians (Math|Float|MakeLiteralFloat 1e+01))) 2.5e+02) false "None")
  (bind _returnvalue (Utilities|Time|SetTimerbyEvent (delegate Custom|FlopHop3) 3.0))
  (Variables|Default|SetFlipTimer _returnvalue))

(event Custom|FlopHop3
  (Physics|SetPhysicsLinearVelocity (Variables|Default|GetRoomba) (* (Class|KismetMathLibrary|RandomUnitVectorinCone "0, 0,1.000000" (Math|Trig|DegreesToRadians (Math|Float|MakeLiteralFloat 1e+01))) 5e+02) false "None")
  (bind _returnvalue (Utilities|Time|SetTimerbyEvent (delegate Custom|ULTIMAFLOP) 5.0))
  (Variables|Default|SetFlipTimer _returnvalue))

(event Custom|ULTIMAFLOP
  (bind _roomba (Variables|Default|GetRoomba))
  (Variables|Default|SetTickRoomba false)
  (Physics|SetPhysicsLinearVelocity _roomba (* (Class|KismetMathLibrary|RandomUnitVectorinCone "0, 0,1.000000" (Math|Trig|DegreesToRadians (Math|Float|MakeLiteralFloat 1e+01))) 2e+03) false "None")
  (Class|PrimitiveComponent|SetPhysicsAngularVelocity _roomba "0,10000.000000, 0" false "None")
  (Utilities|Time|ClearandInvalidateTimerbyHandle (Variables|Default|GetFlipTimer))
  (Utilities|FlowControl|Delay 4.0)
  (Variables|Default|SetTickRoomba true))

(event Custom|LookAhead
  (if (Math|Boolean|ANDBoolean (not (CallFunction|IsFalling)) (Variables|Default|GetTickRoomba) (not (Variables|Default|GetBackUp)))
    (bind (_anyobstructions _validhits) (CallFunction|CheckforObstructions))
    (if _anyobstructions
      (Variables|Default|SetBackUp true)
      (Utilities|FlowControl|Delay 0.25)
      (Utilities|Time|ClearandInvalidateTimerbyHandle (Variables|Default|GetDirTimer))
      (bind _returnvalue (CallFunction|MakeNewHeading _validhits))
      (Variables|Default|SetDirection (Math|Rotator|MakeRotfromZX (Math|Vector|MakeVector 0.0 0.0 1.0) _returnvalue))
      (Variables|Default|SetDoneTurning false))))

(event Custom|DoAirBonk
  (Variables|Default|SetTickRoomba false)
  (Utilities|Time|ClearandInvalidateTimerbyHandle (Variables|Default|GetDirTimer))
  (Utilities|FlowControl|Delay 5.0)
  (Variables|Default|SetTickRoomba true))

(event EventBeginPlay
  (if (Networking|IsServer)
    (CallFunction|InitWhiskers)
    (if (Math|Random|RandomBool)
      (CallFunction|NewDir)
      (else
        (bind _returnvalue (Utilities|Time|SetTimerbyFunctionName 0 "NewDir" (Math|Random|RandomFloatinRange 1e+01 2e+01)))
        (Variables|Default|SetDirTimer _returnvalue)))
    (Utilities|Time|SetTimerbyFunctionName 0 "LookAhead" 0.01 true)
    (else
      (Actor|Tick|SetActorTickEnabled false))))

(event EventTick
  (params (DeltaSeconds :type Float%20%28single-precision%29))
  (if (>= (Math|Vector|DotProduct (Math|Vector|GetUpVector (Variables|Default|GetRoomba)) "0, 0,1.000000") 0.0)
    (if (Utilities|Time|IsValidTimerHandle (Variables|Default|GetFlipTimer))
      (Utilities|Time|ClearandInvalidateTimerbyHandle (Variables|Default|GetFlipTimer)))
    (CallFunction|HandleFly)
    (if (Variables|Default|GetTickRoomba)
      (if (Variables|Default|GetDoneTurning)
        (CallFunction|Move)
        (if (not (Utilities|Time|IsValidTimerHandle (Variables|Default|GetDirTimer)))
          (bind _returnvalue (Utilities|Time|SetTimerbyFunctionName 0 "NewDir" (Math|Random|RandomFloatinRange 5.0 1e+01)))
          (Variables|Default|SetDirTimer _returnvalue))
        (else
          (CallFunction|Turn))))
    (elif (and (not (CallFunction|IsFalling)) (not (Utilities|Time|IsValidTimerHandle (Variables|Default|GetFlipTimer))))
      (CallFunction|Flip))))

(fn ConstructionScript)

(fn Turn
  (Transformation|SetActorRotation (Class|KismetMathLibrary|RInterptoConstant (Transformation|GetActorRotation) (Variables|Default|GetDirection) (Utilities|Time|GetWorldDeltaSeconds) (Math|Float|SelectFloat 2e+02 2e+01 (Variables|Default|GetBackUp))))
  (Physics|SetPhysicsLinearVelocity (Variables|Default|GetRoomba) (Math|Vector|MakeVector 0.0 0.0 0.0) false "None")
  (Variables|Default|SetCurrentSpeed 0.0)
  (bind _output_get (Variables|Default|SetDoneTurning (Math|Rotator|Equal(Rotator) (Transformation|GetActorRotation) (Variables|Default|GetDirection) 0.1)))
  (if (and _output_get (Variables|Default|GetBackUp))
    (Variables|Default|SetBackUp false)))

(fn Move
  (Variables|Default|SetCurrentSpeed (Math|Interpolation|FInterptoConstant (Variables|Default|GetCurrentSpeed) (Variables|Default|GetMaxSpeed) (Utilities|Time|GetWorldDeltaSeconds) 1e+02))
  (Physics|SetPhysicsLinearVelocity (Variables|Default|GetRoomba) (Math|Vector|MakeVector (.x (* (Transformation|GetActorForwardVector) (Math|Float|SelectFloat (* (Variables|Default|GetCurrentSpeed) -2.0) (Variables|Default|GetCurrentSpeed) (Variables|Default|GetBackUp)))) (.y (* (Transformation|GetActorForwardVector) (Math|Float|SelectFloat (* (Variables|Default|GetCurrentSpeed) -2.0) (Variables|Default|GetCurrentSpeed) (Variables|Default|GetBackUp)))) (.z (* (Transformation|GetActorForwardVector) (Math|Float|SelectFloat (* (Variables|Default|GetCurrentSpeed) -2.0) (Variables|Default|GetCurrentSpeed) (Variables|Default|GetBackUp))))) false "None"))

(fn HandleFly
  (if (CallFunction|IsFalling)
    (if (not (Utilities|Time|IsValidTimerHandle (Variables|Default|GetFlapTimer)))
      (bind _returnvalue (Utilities|Time|SetTimerbyFunctionName 0 "Flap" 0.01 true))
      (Variables|Default|SetFlapTimer _returnvalue))
    (else
      (Utilities|Time|ClearandInvalidateTimerbyHandle (Variables|Default|GetFlapTimer))
      (Transformation|SetRelativeRotation (Variables|Default|GetLeftWingRoot) "0, 0, 0" false false)
      (Variables|Default|SetFlapSeconds 0.0))))

(fn Flap
  (bind _leftwingroot (Variables|Default|GetLeftWingRoot))
  (bind _rightwingroot (Variables|Default|GetRightWingRoot))
  (bind _flaptime (LocalVariables|GetFlapTime))
  (bind _output_get (Variables|Default|SetFlapSeconds (+ (Variables|Default|GetFlapSeconds) (Utilities|Time|GetWorldDeltaSeconds))))
  (if (> (Math|Float|%(Float) _output_get _flaptime) (/ _flaptime 2.0))
    (LocalVariables|SetTargRotLeft "0.000000,90.000000, 0")
    (LocalVariables|SetTargRotRight "0,-90.000000, 0")
    (else
      (LocalVariables|SetTargRotLeft "0, 0, 0")
      (LocalVariables|SetTargRotRight "0, 0, 0")))
  (Transformation|SetRelativeRotation _leftwingroot (Math|Interpolation|RInterpTo (Variables|/Script/Engine.SceneComponent|GetRelativeRotation _leftwingroot) (LocalVariables|GetTargRotLeft) (Utilities|Time|GetWorldDeltaSeconds) (LocalVariables|GetWingInterpSpeed)) false false)
  (Transformation|SetRelativeRotation _rightwingroot (Math|Interpolation|RInterpTo (Variables|/Script/Engine.SceneComponent|GetRelativeRotation _rightwingroot) (LocalVariables|GetTargRotRight) (Utilities|Time|GetWorldDeltaSeconds) (LocalVariables|GetWingInterpSpeed)) false false))

(fn IsFalling
  (return (<= (.Z (Math|Vector|BreakVector (Transformation|GetVelocity))) -16.0)))

(fn CheckforObstructions
  (bind _roomba (Variables|Default|GetRoomba))
  (bind _roomba_2 (Variables|Default|GetRoomba))
  (bind _hits (LocalVariables|GetHits))
  (bind _returnvalue (Transformation|GetWorldLocation _roomba))
  (bind _returnvalue_2 (Transformation|GetWorldLocation _roomba_2))
  (bind _outactors (Actor|GetAllActorsOfClass "/Script/MPHorso.MPHorsoCameraGuideCluster"))
  (for _array_element (Variables|Default|GetWallWhiskers)
    (bind (_outhit _returnvalue_3) (Collision|LineTraceForObjects _returnvalue_2 (+ _returnvalue_2 (Math|Transform|TransformDirection (Transformation|GetWorldTransform _roomba_2) _array_element)) (Utilities|Array|MakeArray "ObjectTypeQuery1" "ObjectTypeQuery2") false _outactors "None"))
    (if _returnvalue_3
      (Utilities|Array|Add (LocalVariables|GetHits) _outhit)))
  (for _array_element_2 (Variables|Default|GetPlayerWhiskers)
    (bind (_outhit_2 _returnvalue_4) (Collision|LineTraceForObjects _returnvalue (+ _returnvalue (Math|Transform|TransformDirection (Transformation|GetWorldTransform _roomba) _array_element_2)) (Utilities|Array|MakeArray "ObjectTypeQuery3") false _outactors "None"))
    (if _returnvalue_4
      (Utilities|Array|Add (LocalVariables|GetHits) _outhit_2)))
  (return (> (Utilities|Array|Length _hits) 0) _hits))

(fn MakeNewHeading
  (params (ObstructionHits :type Array%20of%20Hit%20Result%20Structures))
  (for _array_element ObstructionHits
    (LocalVariables|SetTotalVec (+ (LocalVariables|GetTotalVec) (Math|Vector|Normalize (Math|Vector|MirrorVectorbyNormal (- (.ImpactPoint (Collision|BreakHitResult _array_element)) (Transformation|GetActorLocation)) (Math|Vector|GetRightVector (Variables|Default|GetRoomba)))))))
  (return (Math|Vector|Normalize (LocalVariables|GetTotalVec))))

(fn InitWhiskers
  (bind _returnvalue (Math|Vector|MakeVector 0.0 1.0 0.0))
  (bind _returnvalue_2 (Math|Vector|MakeVector 1.0 0.0 0.0))
  (bind _returnvalue_3 (Math|Vector|MakeVector 0.0 0.0 1.0))
  (bind _wallwhiskers (Variables|Default|GetWallWhiskers))
  (bind _playerwhiskers (Variables|Default|GetPlayerWhiskers))
  (bind _roomba (Variables|Default|GetRoomba))
  (bind _max (Components|StaticMesh|GetLocalBounds _roomba))
  (bind _x (Math|Vector|BreakVector _max))
  (bind _returnvalue_4 (* _x 1.5))
  (bind _returnvalue_5 (* _returnvalue_2 _returnvalue_4))
  (bind _returnvalue_6 (Math|Vector|RotateVectorAroundAxis _returnvalue_5 -15.0 _returnvalue))
  (Utilities|FlowControl|Sequence
    (:then_0
      (Utilities|Array|Add _wallwhiskers (Math|Vector|RotateVectorAroundAxis _returnvalue_5 1e+01 _returnvalue_3))
      (Utilities|Array|Add _wallwhiskers (Math|Vector|RotateVectorAroundAxis _returnvalue_5 4e+01 _returnvalue_3))
      (Utilities|Array|Add _wallwhiskers (Math|Vector|RotateVectorAroundAxis _returnvalue_5 7e+01 _returnvalue_3))
      (Utilities|Array|Add _wallwhiskers (Math|Vector|RotateVectorAroundAxis _returnvalue_5 -1e+01 _returnvalue_3))
      (Utilities|Array|Add _wallwhiskers (Math|Vector|RotateVectorAroundAxis _returnvalue_5 -4e+01 _returnvalue_3))
      (Utilities|Array|Add _wallwhiskers (Math|Vector|RotateVectorAroundAxis _returnvalue_5 -7e+01 _returnvalue_3)))
    (:then_1
      (Utilities|Array|Add _playerwhiskers (Math|Vector|RotateVectorAroundAxis _returnvalue_6 1e+01 _returnvalue_3))
      (Utilities|Array|Add _playerwhiskers (Math|Vector|RotateVectorAroundAxis _returnvalue_6 4e+01 _returnvalue_3))
      (Utilities|Array|Add _playerwhiskers (Math|Vector|RotateVectorAroundAxis _returnvalue_6 7e+01 _returnvalue_3))
      (Utilities|Array|Add _playerwhiskers (Math|Vector|RotateVectorAroundAxis _returnvalue_6 -1e+01 _returnvalue_3))
      (Utilities|Array|Add _playerwhiskers (Math|Vector|RotateVectorAroundAxis _returnvalue_6 -4e+01 _returnvalue_3))
      (Utilities|Array|Add _playerwhiskers (Math|Vector|RotateVectorAroundAxis _returnvalue_6 -7e+01 _returnvalue_3)))))

(fn IsCurrentlyManipulable
  (params (Querier :type Controller%20Object%20Reference))
  (return true))