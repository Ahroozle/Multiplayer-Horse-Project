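; MagicGrab is a telekinesis effect actor that scales to its target, holds it above and trailing its owner, or levitates the owner when self-targeted.
; Grabbed players lose gravity and other targets stop simulating physics until Die restores them.
; Looping 0.01s timers drive following, rise impulses, position snapping and a tinted camera-facing plane.
; Already-grabbed targets make the server recast telegrab for the prior grabber, and mutual grabs drift upward.
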(event Custom|Die
  (bind _target (Variables|Default|GetTarget))
  (if (!= _target (Components|GetOwner))
    (bind _asplayer_entity_base_bp (Utilities|Casting|CastToPlayerEntityBaseBP _target)
      (:then
        (CallFunction|RevertPlayer _asplayer_entity_base_bp))
      (:CastFailed
        (CallFunction|ReenableGravities)))
    (bind _target_2 (Variables|Default|GetTarget)
      (:then
        (Transformation|DetachFromActor _target_2 "KeepWorld" "KeepWorld" "KeepWorld"))
      (:else
        _)))
  (Actor|DestroyActor))

(event EventBeginPlay
  (bind _returnvalue (Components|GetOwner))
  (bind _target (Variables|Default|GetTarget)
    (:then
      (bind _asmagic_grab (Utilities|Casting|CastToMagicGrab (Actor|GetAttachParentActor _target))
        (:then
          (if (Networking|IsServer)
            (Default|CastMagic (.AsObserver%20BP (Utilities|Casting|CastToObserverBP (Components|GetOwner (Components|GetOwner _asmagic_grab)))) "/Game/Blueprints/Magic/TelegrabMagicUI.TelegrabMagicUI_C")))
        (:CastFailed
          _)))
    (:else
      _))
  (bind _returnvalue_2 (Rendering|Material|CreateDynamicMaterialInstance (Variables|Default|GetPlane) 0 0 :!class /Script/Engine.PrimitiveComponent))
  (Rendering|Material|SetVectorParameterValue _returnvalue_2 "MagicColor" (Variables|Default|GetColor) :!class /Script/Engine.MaterialInstanceDynamic)
  (bind _target_2 (Variables|Default|GetTarget)
    (:then
      (Transformation|SetActorScale3D (Math|Conversions|ToVector(Float) (/ (Math|Vector|GetMaxElement (.BoxExtent (Collision|GetActorBounds _target_2 false))) (Math|Vector|GetMaxElement (.BoxExtent (Collision|GetActorBounds false))))))
      (if (!= _target_2 (Components|GetOwner))
        (Transformation|AttachActorToActor _target_2 self "None" "SnapToTarget" "KeepWorld" "KeepWorld" true)
        (bind _asplayer_entity_base_bp (Utilities|Casting|CastToPlayerEntityBaseBP _target_2)
          (:then
            (CallFunction|PrepPlayer _asplayer_entity_base_bp)
            (Utilities|Time|SetTimerbyFunctionName 0 "SnapPlayer" 0.01 true))
          (:CastFailed
            (CallFunction|DisableGravities)
            (if (not (Class|KismetSystemLibrary|IsStandalone))
              (Utilities|Time|SetTimerbyFunctionName 0 "SnapObject" 0.01 true))
            (Transformation|AttachActorToActor _returnvalue "None" "KeepWorld" "KeepWorld" "KeepWorld" true)))
        (CallFunction|InitAnchorPos)
        (Utilities|Time|SetTimerbyFunctionName 0 "PositionGrabbed" 0.01 true)
        (else
          (Variables|Default|SetOwnerAsChar (.AsCharacter (Utilities|Casting|CastToCharacter (Components|GetOwner))))
          (Utilities|Time|SetTimerbyFunctionName 0 "Rise" 0.01 true)
          (Transformation|AttachActorToActor _returnvalue "None" "KeepWorld" "KeepWorld" "KeepWorld" true)))
      (Utilities|Time|SetTimerbyFunctionName 0 "BillboardPlane" 0.01 true))
    (:else
      (CallFunction|Die))))

(fn ConstructionScript)

(fn BillboardPlane
  (bind _returnvalue (Class|StaticFuncLib|RetrieveGameInstance))
  (bind _returnvalue_2 (Class|MPHorsoGameInstance|GetRelevantCamera _returnvalue))
  (Utilities|IsValid _returnvalue_2
    (:Is%20Valid
      (Transformation|SetWorldRotation (Variables|Default|GetPlane) (Math|Rotator|MakeRotfromZY (Math|Vector|NegateVector (Math|Vector|GetForwardVector _returnvalue_2)) (Math|Vector|MakeVector 0.0 0.0 1.0)) false false))))

(fn Rise
  (bind _owneraschar (Variables|Default|GetOwnerAsChar)
    (:then
      (Physics|AddImpulse (Variables|/Script/Engine.Character|GetCharacterMovement _owneraschar) "0, 0,19.500000" true))
    (:else)))

(fn PositionGrabbed
  (bind _returnvalue (Components|GetOwner))
  (bind _returnvalue_2 (Transformation|GetVelocity _returnvalue))
  (bind _boxextent (Collision|GetActorBounds _returnvalue false))
  (bind (_x _y _z) (Math|Vector|BreakVector _boxextent))
  (bind _asmagic_grab (Utilities|Casting|CastToMagicGrab (Actor|GetAttachParentActor _returnvalue))
    (:then
      (if (== (Components|GetOwner _asmagic_grab) (Variables|Default|GetTarget))
        (Transformation|AddActorWorldOffset (* (Math|Vector|MakeVector 0.0 0.0 5.0) (Utilities|Time|GetWorldDeltaSeconds)))
        (else
          (if (not (Math|Float|NearlyEqual(Float) (Math|Vector|VectorLength (Transformation|GetVelocity _returnvalue)) 0.0 0.1)) :!label _label
            (Variables|Default|SetLastAnchorPos (+ (Transformation|GetActorLocation _returnvalue) (Math|Vector|MakeVector 0.0 0.0 (* _z 1.0)) (* (Math|Vector|MakeVector _x _y 0.0) (Math|Vector|NegateVector (Math|Vector|Normalize (Math|Vector|MakeVector (.x _returnvalue_2) (.y _returnvalue_2) 0.0)))))))
          (Transformation|SetActorLocation (Math|Interpolation|VInterpTo (Transformation|GetActorLocation) (Variables|Default|GetLastAnchorPos) (Utilities|Time|GetWorldDeltaSeconds) 4.0) false false))))
    (:CastFailed
      (goto _label))))

(fn DisableGravities
  (for _array_element (Actor|GetComponentsByClass (Variables|Default|GetTarget) "/Script/Engine.PrimitiveComponent")
    (if (Physics|IsSimulatingPhysics _array_element "None")
      (Physics|SetSimulatePhysics _array_element false)
      (Utilities|Array|Add (Variables|Default|GetPhysicsPieces) _array_element))))

(fn ReenableGravities
  (for _array_element (Variables|Default|GetPhysicsPieces)
    (Physics|SetSimulatePhysics _array_element true)))

(fn InitAnchorPos
  (bind _returnvalue (Components|GetOwner))
  (Variables|Default|SetLastAnchorPos (+ (Transformation|GetActorLocation _returnvalue) (Math|Vector|MakeVector 0.0 0.0 (* (.Z (Math|Vector|BreakVector (.BoxExtent (Collision|GetActorBounds _returnvalue false)))) 1.0)))))

(fn SnapPlayer
  (Transformation|SetActorLocation (Variables|Default|GetTarget) (Transformation|GetActorLocation) false false))

(fn PrepPlayer
  (params (TargetAsPlayer :type Player%20Entity%20Base%20BP%20Object%20Reference))
  (bind _charactermovement (Variables|/Script/Engine.Character|GetCharacterMovement TargetAsPlayer))
  (Variables|Default|SetStoredGravScale (Variables|/Script/Engine.CharacterMovementComponent|GetGravityScale _charactermovement))
  (Variables|/Script/Engine.CharacterMovementComponent|SetGravityScale _charactermovement 0.0))

(fn RevertPlayer
  (params (TargetAsPlayer :type Player%20Entity%20Base%20BP%20Object%20Reference))
  (Variables|/Script/Engine.CharacterMovementComponent|SetGravityScale (Variables|/Script/Engine.Character|GetCharacterMovement TargetAsPlayer) (Variables|Default|GetStoredGravScale)))

(fn SnapObject
  (Transformation|SetActorLocation (Variables|Default|GetTarget) (Transformation|GetActorLocation) false false))