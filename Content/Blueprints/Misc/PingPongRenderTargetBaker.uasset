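; Editor-time baker that runs a material repeatedly over render targets to produce an iterated texture in FinalTarget.
; The construction script calls Bake when Refresh or BakeOnEdit is set, resetting Refresh each time.
; Bake alternates Ping and Pong targets, feeding each pass's output into a dynamic material's texture parameter for the next.
; The first pass keeps the material's own texture, and the last draws into FinalTarget.
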(fn ConstructionScript
  (if (or (Variables|Default|GetRefresh) (Variables|Default|GetBakeOnEdit))
    (Variables|Default|SetRefresh false)
    (if (> (Variables|Default|GetIterations) 0)
      (CallFunction|Bake))))

(fn Bake
  (bind _iterations (Variables|Default|GetIterations))
  (if (Math|Boolean|ANDBoolean (Utilities|IsValid (Variables|Default|GetPingTarget)) (Utilities|IsValid (Variables|Default|GetPongTarget)) (Utilities|IsValid (Variables|Default|GetFinalTarget)) (Utilities|IsValid (Variables|Default|GetMaterialToBake)))
    (bind _returnvalue (Rendering|Material|CreateDynamicMaterialInstance (Variables|Default|GetMaterialToBake) :!class /Script/Engine.KismetMaterialLibrary))
    (LocalVariables|SetDynMat _returnvalue)
    (for _index (range 1 _iterations)
      (if (!= _index 1)
        (Rendering|Material|SetTextureParameterValue (LocalVariables|GetDynMat) (Variables|Default|GetTexParamName) (.AsTexture%20Render%20Target%202D (Utilities|Casting|CastToTextureRenderTarget2D (Utilities|SelectObject (Variables|Default|GetPingTarget) (Variables|Default|GetPongTarget) (== (Math|Integer|%(Integer) _index 2) 0))))))
      (Rendering|ClearRenderTarget2D self (.AsTexture%20Render%20Target%202D (Utilities|Casting|CastToTextureRenderTarget2D (Utilities|SelectObject (Variables|Default|GetFinalTarget) (Utilities|SelectObject (Variables|Default|GetPongTarget) (Variables|Default|GetPingTarget) (== (Math|Integer|%(Integer) _index 2) 0)) (== _index _iterations)))))
      (Rendering|DrawMaterialtoRenderTarget (.AsTexture%20Render%20Target%202D (Utilities|Casting|CastToTextureRenderTarget2D (Utilities|SelectObject (Variables|Default|GetFinalTarget) (Utilities|SelectObject (Variables|Default|GetPongTarget) (Variables|Default|GetPingTarget) (== (Math|Integer|%(Integer) _index 2) 0)) (== _index _iterations)))) (LocalVariables|GetDynMat)))))