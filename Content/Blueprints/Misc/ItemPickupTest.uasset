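; Test pickup actor that gives an overlapping player one of two test items, chosen at random.
; On overlap it reaches the inventory widget through the PlayerEntityBaseBP's owning ObserverBP.
; If the inventory has room for the chosen MPHorsoItemBase class, it constructs the item object and adds it through the widget.
; The pickup is not destroyed, so each new overlap can grant another item.
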(event EventBeginPlay)

(event Collision|EventActorBeginOverlap
  (params (OtherActor :type Actor%20Object%20Reference))
  (bind _asplayer_entity_base_bp (Utilities|Casting|CastToPlayerEntityBaseBP OtherActor))
  (bind _asobserver_bp (Utilities|Casting|CastToObserverBP (Components|GetOwner _asplayer_entity_base_bp)))
  (bind _invwidg (Variables|/Game/Blueprints/ObserverBP.ObserverBP_C|GetInvWidg _asobserver_bp)
    (:then
      (bind _output_get (Variables|Default|SetItemClass (.AsMPHorso%20Item%20Base (Utilities|Casting|CastToMPHorsoItemBaseClass (Class|KismetMathLibrary|SelectClass "/Game/Blueprints/Items/TestItem.TestItem_C" "/Game/Blueprints/Items/TestItem2.TestItem2_C" (Math|Random|RandomBool))))))
      (if (Default|InventoryNotFull _invwidg _output_get)
        (bind _returnvalue (Game|ConstructObjectfromClass _output_get self))
        (Default|AddItemtoInventory _invwidg _returnvalue)))
    (:else)))

(event EventTick
  (params (DeltaSeconds :type Float%20%28single-precision%29)))

(fn ConstructionScript)