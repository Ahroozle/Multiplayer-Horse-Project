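; SmearFrameComponent is an actor component that drives smear-frame effects on dynamic materials from its owner's movement.
; Each tick, while SmearDyn holds materials, it shifts a short history of owner locations.
; With CurvySmear set it passes three past positions to the materials for a curved smear; otherwise it passes a per-frame Velocity offset.
; SmearDyn is only read here, never filled.
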(event EventTick
  (params (DeltaSeconds :type Float%20%28single-precision%29))
  (if (> (Utilities|Array|Length (Variables|Default|GetSmearDyn)) 0)
    (CallFunction|UpdateVelocities)))

(event EventBeginPlay
  (bind _output_get (Variables|Default|SetPrevPos (Transformation|GetActorLocation (Components|GetOwner))))
  (bind _output_get_2 (Variables|Default|SetLastPos _output_get))
  (bind _output_get_3 (Variables|Default|SetOldestPos _output_get_2))
  (Variables|Default|SetCurrPos _output_get_3))

(fn UpdateVelocities
  (if (Variables|Default|GetCurvySmear)
    (Variables|Default|SetOldestPos (Variables|Default|GetPrevPos))
    (Variables|Default|SetPrevPos (Variables|Default|GetLastPos))
    (Variables|Default|SetLastPos (Variables|Default|GetCurrPos))
    (Variables|Default|SetCurrPos (Transformation|GetActorLocation (Components|GetOwner)))
    (for _array_element (Variables|Default|GetSmearDyn)
      (Rendering|Material|SetVectorParameterValue _array_element "OldestPos" (Math|Conversions|ToLinearColor(Vector) (Variables|Default|GetOldestPos)) :!class /Script/Engine.MaterialInstanceDynamic)
      (Rendering|Material|SetVectorParameterValue _array_element "PrevPos" (Math|Conversions|ToLinearColor(Vector) (Variables|Default|GetPrevPos)) :!class /Script/Engine.MaterialInstanceDynamic)
      (Rendering|Material|SetVectorParameterValue _array_element "LastPos" (Math|Conversions|ToLinearColor(Vector) (Variables|Default|GetLastPos)) :!class /Script/Engine.MaterialInstanceDynamic))
    (else
      (Variables|Default|SetPrevPos (Variables|Default|GetLastPos))
      (Variables|Default|SetLastPos (Transformation|GetActorLocation (Components|GetOwner)))
      (LocalVariables|SetVeloc (Math|Conversions|ToLinearColor(Vector) (- (Variables|Default|GetLastPos) (Variables|Default|GetPrevPos))))
      (for _array_element_2 (Variables|Default|GetSmearDyn)
        (Rendering|Material|SetVectorParameterValue _array_element_2 "Velocity" (LocalVariables|GetVeloc) :!class /Script/Engine.MaterialInstanceDynamic)))))