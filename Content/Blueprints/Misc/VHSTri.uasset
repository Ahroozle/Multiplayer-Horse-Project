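; VHSTri is a decorative actor whose Edges component hovers back and forth around the actor's location.
; On BeginPlay it starts a fast looping timer that runs DoHover instead of using Tick.
; Each call sets the Edges world location to the actor location plus BobVector scaled by a sine of game time, tuned by a time multiplier and offset.
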(event Custom|DoHover
  (Transformation|SetWorldLocation (Variables|Default|GetEdges) (+ (* (Variables|Default|GetBobVector) (Math|Trig|Sin(Radians) (+ (* (Utilities|Time|GetTimeSeconds) (Variables|Default|GetTimeMultiplier)) (Variables|Default|GetTimeOffset)))) (Transformation|GetActorLocation)) false false))

(event EventBeginPlay
  (Utilities|Time|SetTimerbyEvent (delegate Custom|DoHover) 0.01 true))

(fn ConstructionScript)