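; RenderTargetBaker is an editor utility actor that bakes a material into a render target.
; The construction script calls Bake when the Refresh flag is toggled, which it then resets, or on every edit while BakeOnEdit is on.
; Bake checks that both the target and material are valid, clears the render target to black, then draws the material into it.
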(event EventBeginPlay)

(event Collision|EventActorBeginOverlap
  (params (OtherActor :type Actor%20Object%20Reference)))

(event EventTick
  (params (DeltaSeconds :type Float%20%28single-precision%29)))

(fn ConstructionScript
  (if (or (Variables|Default|GetRefresh) (Variables|Default|GetBakeOnEdit))
    (Variables|Default|SetRefresh false)
    (CallFunction|Bake)))

(fn Bake
  (bind _targettobaketo (Variables|Default|GetTargetToBakeTo)
    (:then
      (bind _materialtobake (Variables|Default|GetMaterialToBake)
        (:then
          (Rendering|ClearRenderTarget2D self (Variables|Default|GetTargetToBakeTo))
          (Rendering|DrawMaterialtoRenderTarget _targettobaketo _materialtobake))
        (:else)))
    (:else)))