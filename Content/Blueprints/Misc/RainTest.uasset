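; RainTest is a rain effect actor that follows the observer pawn's Body in X and Y while keeping its own height.
; On BeginPlay it attaches a spawned, rotated RainCaptureActor and derives the drop and splash radius and RainParameters area size from its ortho width.
; It also sets the rain amount on both particle components.
; A fast looping timer moves the actor and writes the player's Z to the parameter collection.
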(event EventBeginPlay
  (Variables|Default|SetFocusRef (Variables|/Game/Blueprints/ObserverBP.ObserverBP_C|GetBody (.AsObserver%20BP (Utilities|Casting|CastToObserverBP (Pawn|GetControlledPawn (Game|GetPlayerController 0))))))
  (Utilities|Time|SetTimerbyFunctionName 0 "TrackPlayer" 0.01 true)
  (bind _returnvalue (Game|SpawnActorfromClass "/Game/Blueprints/Misc/RainCaptureActor.RainCaptureActor_C" (Math|Transform|MakeTransform "0, 0, 0" "0.000000, 0,0.000000" "1,1,1") "Undefined" 0 0))
  (Transformation|AttachActorToActor _returnvalue self "None" "SnapToTarget" "SnapToTarget" "KeepWorld" false)
  (Transformation|SetActorRelativeRotation _returnvalue "-90.000000, 0,-90.000000")
  (Effects|Components|ParticleSystem|SetFloatParameter (Variables|Default|GetRain_Drops) "RainRadius" (/ (Variables|/Script/Engine.SceneCaptureComponent2D|GetOrthoWidth (Variables|/Script/Engine.SceneCapture2D|GetCaptureComponent2D _returnvalue)) 2.0))
  (Rendering|Material|SetScalarParameterValue "/Game/Assets/Mat/Rain/RainParameters.RainParameters" "RainAreaSize" (Variables|/Script/Engine.SceneCaptureComponent2D|GetOrthoWidth (Variables|/Script/Engine.SceneCapture2D|GetCaptureComponent2D _returnvalue)) :!class /Script/Engine.KismetMaterialLibrary)
  (Effects|Components|ParticleSystem|SetFloatParameter (Variables|Default|GetRain_Drops) "RainAmount" (Variables|Default|GetRainAmount)))

(fn ConstructionScript)

(fn TrackPlayer
  (bind _focusref (Variables|Default|GetFocusRef)
    (:then
      (Rendering|Material|SetScalarParameterValue "/Game/Assets/Mat/Rain/RainParameters.RainParameters" "PlayerZ" (.z (Transformation|GetActorLocation _focusref)) :!class /Script/Engine.KismetMaterialLibrary)
      (Transformation|SetActorLocation (Math|Vector|MakeVector (.x (Transformation|GetActorLocation _focusref)) (.y (Transformation|GetActorLocation _focusref)) (.z (Transformation|GetActorLocation))) false false))
    (:else)))