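; Base actor for a destructible energy barrier that fades in, tracks HP and expects derived classes to override overlap and call UpdateHP.
; Damage updates the sphere's dynamic material and curve-driven shake, with sparking hits also drawing cracks into a lazily created render target.
; At zero HP, Die picks a power-down fade, gradual shatter or delayed critical burst by final-hit damage ratio, using looping timers for animation.
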(event Custom|FinishCriticalDie
  (bind _maxhp (Variables|Default|GetMaxHP))
  (bind _lasthitdamage (Variables|Default|GetLastHitDamage))
  (bind _returnvalue (/ _lasthitdamage _maxhp))
  (Components|DestroyComponent (Variables|Default|GetBarrier))
  (Utilities|Time|ClearTimerbyFunctionName 0 "DoShake")
  (Components|Activation|Deactivate (Variables|Default|GetBarrierTwinkle))
  (bind _returnvalue_2 (Effects|SpawnEmitterAttached "/Game/Assets/VFX/BarrierFX/BarrierShatter_Critical.BarrierShatter_Critical" (Variables|Default|GetDefaultSceneRoot) "None" "0,0.000000, 0" "0, 0, 0" "SnapToTargetIncludingScale"))
  (Effects|Components|ParticleSystem|SetColorParameter _returnvalue_2 "MainColor" (Variables|Default|GetBarrierColor))
  (Effects|Components|ParticleSystem|SetFloatParameter _returnvalue_2 "SphereSize" (* (.Z (Math|Vector|BreakVector (Transformation|GetActorScale3D))) 1e+02))
  (Effects|Components|ParticleSystem|SetVectorParameter _returnvalue_2 "BlowVelocity" (+ (* (Variables|Default|GetLastHitDirection) (* _returnvalue 5e+03)) "0, 0,1960.000000"))
  (Effects|Components|ParticleSystem|SetFloatParameter _returnvalue_2 "BlowPower" (* _returnvalue 1e+02))
  (CallFunction|BeginWaitforDie _returnvalue_2)
  (bind _returnvalue_3 (Class|StaticFuncLib|PlaySound (Transformation|GetActorTransform) "/Game/Assets/Sound/SFX/Barrier/BarrierBreak.BarrierBreak" (Math|Random|RandomFloatinRange 0.9 1.1)))
  (Audio|Components|Audio|AdjustAttenuation (Variables|/Script/MPHorso.OneShotAudio|GetaudioComp _returnvalue_3) (Variables|Default|GetAtten))
  (Audio|Components|Audio|Play (Variables|/Script/MPHorso.OneShotAudio|GetaudioComp _returnvalue_3) 0.0))

(event Custom|BeginWaitForDie
  (params (PSys :type Particle%20System%20Component%20Object%20Reference))
  (EventDispatchers|AssignOnSystemFinished PSys (delegate Custom|CompletelyDie)))

(event Custom|CompletelyDie
  (params (PSystem :type Particle%20System%20Component%20Object%20Reference))
  (Actor|DestroyActor))

(event EventBeginPlay
  (Variables|Default|SetCurrentHP (Variables|Default|GetMaxHP))
  (bind _returnvalue (Rendering|Material|CreateDynamicMaterialInstance (Variables|Default|GetBarrier) 0 0 :!class /Script/Engine.PrimitiveComponent))
  (bind _output_get (Variables|Default|SetSphereDyn _returnvalue))
  (Rendering|Material|SetVectorParameterValue _output_get "BarrierColor" (Variables|Default|GetBarrierColor) :!class /Script/Engine.MaterialInstanceDynamic)
  (Rendering|Material|SetScalarParameterValue _output_get "VisibleAmount" 0.0 :!class /Script/Engine.MaterialInstanceDynamic)
  (Utilities|Time|SetTimerbyFunctionName 0 "DoShake" 0.01 true)
  (Utilities|Time|SetTimerbyFunctionName 0 "PlayCastAnim" 0.01 true))

(event Collision|EventActorBeginOverlap
  (params (OtherActor :type Actor%20Object%20Reference))
  ;[1 1 1] Remember to call UpdateHP from within and give it damage recieved as input
  (Development|PrintString "BarrierBase::ActorBeginOverlap: This isn't supposed to be used! Please overload if you are using this from a derived class."))

(event EventTick
  (params (DeltaSeconds :type Float%20%28single-precision%29))
  (bind _shineroot (Variables|Default|GetShineRoot)
    (:then
      (Transformation|SetWorldRotation _shineroot (Math|Rotator|FindLookatRotation (Transformation|GetWorldLocation _shineroot) (Transformation|GetWorldLocation (Variables|/Game/Blueprints/ObserverBP.ObserverBP_C|GetCamera (.AsObserver%20BP (Utilities|Casting|CastToObserverBP (Pawn|GetControlledPawn (Game|GetPlayerController 0))))))) false false))
    (:else)))

(fn ConstructionScript)

(fn ShuffleRot
  (Variables|Default|SetNextRot (Math|Random|RandomUnitVector)))

(fn UpdateHP
  (params (IncomingDamage :type Float%20%28single-precision%29) (AttackerLocation :type Vector) (ShouldSpark :type Boolean))
  (bind _returnvalue (Transformation|GetActorLocation))
  (bind _maxhp (Variables|Default|GetMaxHP))
  (Variables|Default|GetBarrier
    (:then
      (bind _output_get (Variables|Default|SetCurrentHP (- (Variables|Default|GetCurrentHP) IncomingDamage)))
      (LocalVariables|SetVHRat (/ _output_get _maxhp))
      (bind _output_get_2 (LocalVariables|SetHRat (/ _output_get _maxhp)))
      (if (> _output_get_2 0.0)
        (Rendering|Material|SetScalarParameterValue (Variables|Default|GetSphereDyn) "HealthRatio" (LocalVariables|GetVHRat) :!class /Script/Engine.MaterialInstanceDynamic)
        (if ShouldSpark
          (bind _returnvalue_2 (Effects|SpawnEmitterAttached "/Game/Assets/VFX/BarrierFX/BarrierSpark.BarrierSpark" (Variables|Default|GetDefaultSceneRoot) "None" "0, 0, 0" (Math|Conversions|RotationFromXVector (Math|Vector|Normalize (- AttackerLocation _returnvalue))) "SnapToTargetIncludingScale"))
          (Effects|Components|ParticleSystem|SetColorParameter _returnvalue_2 "SparkColor" (Variables|Default|GetBarrierColor))
          (CallFunction|AddCrack AttackerLocation IncomingDamage))
        (else
          (if ShouldSpark
            (Variables|Default|SetLastHitLocation AttackerLocation)
            (Variables|Default|SetLastHitDirection (Math|Vector|Normalize (- _returnvalue AttackerLocation)))
            (Variables|Default|SetLastHitDamage IncomingDamage))
          (CallFunction|Die (Math|Float|SelectFloat (/ IncomingDamage (Variables|Default|GetMaxHP)) 0.0 ShouldSpark)))))
    (:else)))

(fn DoShake
  (bind _behaviorcurve (LocalVariables|GetBehaviorCurve))
  (bind _currenthp (Variables|Default|GetCurrentHP))
  (bind _maxhp (Variables|Default|GetMaxHP))
  (bind _returnvalue (/ _currenthp _maxhp))
  (bind _returnvalue_2 (- 1.0 _returnvalue))
  (bind _returnvalue_3 (Math|Curves|GetFloatValue _behaviorcurve _returnvalue_2))
  (bind _barrier (Variables|Default|GetBarrier)
    (:then
      (Transformation|SetRelativeLocation _barrier (* (Math|Random|RandomUnitVector) (* (LocalVariables|GetMaxVib) _returnvalue_3)) false false)
      (Transformation|SetRelativeScale3D _barrier (+ (Math|Vector|MakeVector 2.0 2.0 2.0) (* (Math|Random|RandomUnitVector) (* _returnvalue_3 (LocalVariables|GetMaxFlub))))))
    (:else)))

(fn PlayCastAnim
  (bind _output_get (Variables|Default|SetVisibleAmount (Math|Float|Min(Float) (+ (Variables|Default|GetVisibleAmount) (* (Utilities|Time|GetWorldDeltaSeconds) 1.0)) 1.0)))
  (bind _spheredyn (Variables|Default|GetSphereDyn)
    (:then
      (Rendering|Material|SetScalarParameterValue _spheredyn "VisibleAmount" _output_get :!class /Script/Engine.MaterialInstanceDynamic))
    (:else
      _))
  (if (>= (Variables|Default|GetVisibleAmount) 1.0)
    (Utilities|Time|ClearTimerbyFunctionName 0 "PlayCastAnim")))

(fn AddCrack
  (params (Location :type Vector) (Damage :type Float%20%28single-precision%29))
  (bind _maxhp (Variables|Default|GetMaxHP))
  (bind _returnvalue (/ Damage _maxhp))
  (Variables|Default|GetCrackRT
    (:then
      _)
    (:else
      (bind _returnvalue_2 (Rendering|CreateRenderTarget2D 1024 1024))
      (bind _output_get (Variables|Default|SetCrackRT _returnvalue_2))
      (Variables|/Script/Engine.Texture|SetCompressionSettings _output_get "TC_HDR")
      (Variables|/Script/Engine.Texture|SetSRGB _output_get false)
      (Rendering|ClearRenderTarget2D _output_get)
      (bind _spheredyn (Variables|Default|GetSphereDyn)
        (:then
          (Rendering|Material|SetTextureParameterValue _spheredyn "CracksRT" _output_get))
        (:else))))
  (Variables|Default|GetCrackDrawDyn
    (:then
      _)
    (:else
      (bind _returnvalue_3 (Rendering|Material|CreateDynamicMaterialInstance (LocalVariables|GetCrackDrawMat) :!class /Script/Engine.KismetMaterialLibrary))
      (Variables|Default|SetCrackDrawDyn _returnvalue_3)))
  (Rendering|Material|SetVectorParameterValue (Variables|Default|GetCrackDrawDyn) "ImpactPointLS" (Math|Conversions|ToLinearColor(Vector) (Math|Transform|InverseTransformLocation (Transformation|GetWorldTransform (Variables|Default|GetBarrier)) Location)) :!class /Script/Engine.MaterialInstanceDynamic)
  (Rendering|Material|SetScalarParameterValue (Variables|Default|GetCrackDrawDyn) "CrackIntensity" (Math|Float|MapRangeClamped _returnvalue 0.0 0.3 0.0 1.0) :!class /Script/Engine.MaterialInstanceDynamic)
  (Rendering|Material|SetScalarParameterValue (Variables|Default|GetCrackDrawDyn) "ImpactSize" (Math|Float|MapRangeClamped _returnvalue 0.0 0.5 25.0 75.0) :!class /Script/Engine.MaterialInstanceDynamic)
  (Rendering|Material|SetScalarParameterValue (Variables|Default|GetCrackDrawDyn) "RotAngle" (Math|Random|RandomFloatinRange 0.0 1.0) :!class /Script/Engine.MaterialInstanceDynamic)
  (Rendering|Material|SetScalarParameterValue (Variables|Default|GetCrackDrawDyn) "FadeSeconds" (Math|Float|MapRangeClamped _returnvalue 0.0 0.2 3.0 1e+01) :!class /Script/Engine.MaterialInstanceDynamic)
  (Rendering|DrawMaterialtoRenderTarget (Variables|Default|GetCrackRT) (Variables|Default|GetCrackDrawDyn)))

(fn Die
  (params (HitHealthRatio :type Float%20%28single-precision%29))
  (Collision|SetCollisionEnabled (Variables|Default|GetBarrier) "NoCollision")
  (Rendering|SetVisibility (Variables|Default|GetShine) false false)
  (Components|Activation|Deactivate (Variables|Default|GetBarrierTwinkle))
  (if (<= HitHealthRatio 0.0)
    (Utilities|Time|SetTimerbyFunctionName 0 "PowerDownDie" 0.01 true)
    (elif (< HitHealthRatio 0.3)
      (bind _returnvalue (Effects|SpawnEmitterAttached "/Game/Assets/VFX/BarrierFX/BarrierShatter.BarrierShatter" (Variables|Default|GetDefaultSceneRoot) "None" "0,0.000000, 0" "0, 0, 0" "SnapToTargetIncludingScale"))
      (bind _output_get (Variables|Default|SetShatterSys _returnvalue))
      (Effects|Components|ParticleSystem|SetColorParameter _output_get "MainColor" (Variables|Default|GetBarrierColor))
      (Utilities|Time|SetTimerbyFunctionName 0 "ShatterDie" 0.01 true)
      (else
        (CallFunction|CriticalDie)))))

(fn PowerDownDie
  (bind _output_get (Variables|Default|SetVisibleAmount (Math|Float|Max(Float) (- (Variables|Default|GetVisibleAmount) (* (Utilities|Time|GetWorldDeltaSeconds) 1.0)) 0.0)))
  (bind _spheredyn (Variables|Default|GetSphereDyn)
    (:then
      (Rendering|Material|SetScalarParameterValue _spheredyn "VisibleAmount" _output_get :!class /Script/Engine.MaterialInstanceDynamic))
    (:else
      _))
  (if (<= (Variables|Default|GetVisibleAmount) 0.0)
    (Utilities|Time|ClearTimerbyFunctionName 0 "PowerDownDie")
    (CallFunction|CompletelyDie)))

(fn ShatterDie
  (bind _returnvalue (Transformation|GetActorScale3D))
  (bind _z (Math|Vector|BreakVector _returnvalue))
  (bind _output_get (Variables|Default|SetVisibleAmount (Math|Float|Max(Float) (- (Variables|Default|GetVisibleAmount) (* (Utilities|Time|GetWorldDeltaSeconds) 0.25)) 0.0)))
  (bind _spheredyn (Variables|Default|GetSphereDyn)
    (:then
      (Rendering|Material|SetScalarParameterValue _spheredyn "Shatter" _output_get :!class /Script/Engine.MaterialInstanceDynamic))
    (:else
      _))
  (bind _shattersys (Variables|Default|GetShatterSys)
    (:then
      (Effects|Components|ParticleSystem|SetFloatParameter _shattersys "ShatterRadius" (* (.Z (Math|Vector|BreakVector (Transformation|GetActorScale3D))) 1e+02 (Math|Trig|Sin(Radians) (Math|Float|MultiplybyPi (Variables|Default|GetVisibleAmount)))))
      (Effects|Components|ParticleSystem|SetVectorParameter _shattersys "ShatterOffset" (Math|Vector|Lerp(Vector) (Math|Vector|MakeVector 0.0 0.0 (* _z -1e+02)) (Math|Vector|MakeVector 0.0 0.0 (* _z 1e+02)) (Variables|Default|GetVisibleAmount))))
    (:else
      _))
  (if (<= (Variables|Default|GetVisibleAmount) 0.0)
    (Utilities|Time|ClearTimerbyFunctionName 0 "ShatterDie")
    (bind _shattersys_2 (Variables|Default|GetShatterSys)
      (:then
        (Components|Activation|Deactivate _shattersys_2)
        (CallFunction|BeginWaitforDie _shattersys_2))
      (:else
        (CallFunction|CompletelyDie)))))

(fn CriticalDie
  (Utilities|Time|ClearTimerbyFunctionName 0 "DoShake")
  (Effects|SpawnEmitteratLocation "/Game/Assets/VFX/BarrierFX/BarrierCritShine.BarrierCritShine" (Variables|Default|GetLastHitLocation))
  (bind _spheredyn (Variables|Default|GetSphereDyn)
    (:then
      (Rendering|Material|SetScalarParameterValue _spheredyn "CrackMask" 1.0 :!class /Script/Engine.MaterialInstanceDynamic))
    (:else
      _))
  (Utilities|Time|SetTimerbyFunctionName 0 "FinishCriticalDie" 0.25))