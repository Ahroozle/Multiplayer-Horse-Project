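; Magic arrow projectile actor that tints its materials, trail and effects with one color and flies forward by swept moves on Tick.
; It can home on a target point with steadily increasing rotation lerp, optionally holding collision and steering off for an initial wait.
; The first non-owner hit spawns impact effects and sound, then either dissolves immediately or lingers before fading out.
; A lifetime timer also triggers the burst and dissolve.
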(event Custom|StartDie
  (Utilities|Time|ClearTimerbyFunctionName 0 "EndLife")
  (Utilities|Time|SetTimerbyEvent (delegate Custom|FadeOut) 0.01 true)
  (bind _returnvalue (Effects|SpawnEmitteratLocation "/Game/Assets/VFX/Arrow/ArrowDissolve.ArrowDissolve" (Transformation|GetActorLocation) (Transformation|GetActorRotation)))
  (Transformation|SetWorldScale3D _returnvalue (Transformation|GetActorScale3D))
  (Effects|Components|ParticleSystem|SetColorParameter _returnvalue "MagicColor" (Variables|Default|GetColor)))

(event Custom|FadeOut
  (bind _output_get (Variables|Default|SetAlpha (Math|Interpolation|FInterptoConstant (Variables|Default|GetAlpha) 0.0 (Utilities|Time|GetWorldDeltaSeconds) 0.5)))
  (Rendering|Material|SetScalarParameterValue (Variables|Default|GetHeadDyn) "Alpha" _output_get :!class /Script/Engine.MaterialInstanceDynamic)
  (if (<= _output_get 0.0)
    (Actor|DestroyActor)))

(event Custom|EndLife
  (CallFunction|DieImmediate)
  (CallFunction|PlayDeathSound (Transformation|GetActorLocation))
  (Actor|Tick|SetActorTickEnabled false)
  (Effects|Components|ParticleSystem|SetFloatParameter (Variables|Default|GetHeadWave1) "SpawnRate" 0.0)
  (bind _returnvalue (Effects|SpawnEmitteratLocation (Variables|Default|GetHitEffect) (Transformation|GetActorLocation) (Transformation|GetActorRotation)))
  (Transformation|SetWorldScale3D _returnvalue (Transformation|GetActorScale3D))
  (Effects|Components|ParticleSystem|SetColorParameter _returnvalue "MagicColor" (Variables|Default|GetColor)))

(event Custom|PlayDeathSound
  (params (Loc :type Vector))
  (bind _returnvalue (Class|StaticFuncLib|PlaySound (Math|Transform|MakeTransform Loc "0, 0, 0" "1,1,1") (Variables|Default|GetHitSound) (Math|Random|RandomFloatinRange 0.8 1.2)))
  (Variables|/Script/Engine.AudioComponent|SetbOverrideAttenuation (Variables|/Script/MPHorso.OneShotAudio|GetaudioComp _returnvalue) true)
  (Variables|/Script/Engine.AudioComponent|SetAttenuationOverrides (Variables|/Script/MPHorso.OneShotAudio|GetaudioComp _returnvalue) (Variables|/Script/Engine.AudioComponent|GetAttenuationOverrides (Variables|Default|GetAudio)))
  (Audio|Components|Audio|Play (Variables|/Script/MPHorso.OneShotAudio|GetaudioComp _returnvalue) 0.0))

(event Custom|DieImmediate
  (bind _returnvalue (Effects|SpawnEmitteratLocation "/Game/Assets/VFX/Arrow/ArrowDissolve.ArrowDissolve" (Transformation|GetActorLocation) (Transformation|GetActorRotation)))
  (Transformation|SetWorldScale3D _returnvalue (Transformation|GetActorScale3D))
  (Rendering|SetVisibility (Variables|Default|GetBody) false false)
  (Actor|Tick|SetActorTickEnabled false)
  (Audio|Components|Audio|Stop (Variables|Default|GetAudio))
  (Effects|Components|ParticleSystem|SetColorParameter _returnvalue "MagicColor" (Variables|Default|GetColor))
  (Utilities|Time|SetTimerbyEvent (delegate Custom|FInishImmediateDie) 5.0)
  (Collision|SetCollisionEnabled (Variables|Default|GetBox) "NoCollision"))

(event Custom|WakeUpSteering
  (Variables|Default|SetMaySteer true)
  (Collision|SetCollisionEnabled (Variables|Default|GetBox) "QueryAndPhysics"))

(event Custom|FInishImmediateDie
  (Actor|DestroyActor))

(event EventBeginPlay
  (bind _audio (Variables|Default|GetAudio))
  (bind _returnvalue (Rendering|Material|CreateDynamicMaterialInstance (Variables|Default|GetBody) 0 0 :!class /Script/Engine.PrimitiveComponent))
  (Variables|Default|SetBodyDyn _returnvalue)
  (bind _returnvalue_2 (Rendering|Material|CreateDynamicMaterialInstance (Variables|Default|GetHead) 0 0 :!class /Script/Engine.PrimitiveComponent))
  (Variables|Default|SetHeadDyn _returnvalue_2)
  (Rendering|Material|SetVectorParameterValue (Variables|Default|GetHeadDyn) "MagicColor" (Variables|Default|GetColor) :!class /Script/Engine.MaterialInstanceDynamic)
  (Effects|Components|ParticleSystem|SetColorParameter (Variables|Default|GetTrail) "MagicColor" (Variables|Default|GetColor))
  (Variables|/Script/Engine.AudioComponent|SetSound _audio (Variables|Default|GetIdleCue))
  (Audio|Components|Audio|Play _audio 0.0)
  (if (Variables|Default|GetUseFrontVFX)
    (Components|Activation|Activate (Variables|Default|GetHeadWave2) true)
    (Effects|Components|ParticleSystem|SetColorParameter (Variables|Default|GetHeadWave2) "MagicColor" (Variables|Default|GetColor)))
  (Utilities|Time|SetTimerbyFunctionName 0 "EndLife" (Variables|Default|GetLifeSeconds))
  (if (> (Variables|Default|GetWaitTime) 0.0)
    (Collision|SetCollisionEnabled (Variables|Default|GetBox) "NoCollision")
    (Variables|Default|SetMaySteer false)
    (Utilities|Time|SetTimerbyEvent (delegate Custom|WakeUpSteering) (Variables|Default|GetWaitTime))))

(event EventTick
  (params (DeltaSeconds :type Float%20%28single-precision%29))
  (Transformation|SetActorLocation (+ (Transformation|GetActorLocation) (* (Transformation|GetActorForwardVector) (* DeltaSeconds (Variables|Default|GetSpeed)))) true false)
  (if (and (Variables|Default|GetSteerToTarget) (Variables|Default|GetMaySteer))
    (Transformation|SetActorRotation (Math|Rotator|Lerp(Rotator) (Transformation|GetActorRotation) (Math|Rotator|MakeRotfromXZ (- (Variables|Default|GetTarget) (Transformation|GetActorLocation)) (Math|Vector|MakeVector 0.0 0.0 1.0)) (Variables|Default|GetSteerAmount) true))
    (Variables|Default|SetSteerAmount (+ (Variables|Default|GetSteerAmount) (* (Utilities|Time|GetWorldDeltaSeconds) 0.01)))))

(event Collision|EventHit
  (params (MyComp :type Primitive%20Component%20Object%20Reference) (Other :type Actor%20Object%20Reference) (OtherComp :type Primitive%20Component%20Object%20Reference) (bSelfMoved :type Boolean) (HitLocation :type Vector) (HitNormal :type Vector) (NormalImpulse :type Vector :default "0, 0, 0") (Hit :type Hit%20Result%20Structure%20%28by%20ref%29))
  (bind _arrowhitscale (Variables|Default|GetArrowHitScale))
  (if (!= Other (Components|GetOwner))
    (Utilities|FlowControl|DoOnce false
      (:Completed
        (Actor|Tick|SetActorTickEnabled false)
        (Effects|Components|ParticleSystem|SetFloatParameter (Variables|Default|GetHeadWave1) "SpawnRate" 0.0)
        (bind _returnvalue (Effects|SpawnEmitteratLocation (Variables|Default|GetHitEffect) HitLocation (Math|Rotator|MakeRotfromXZ HitNormal (Math|Vector|MakeVector 0.0 0.0 1.0))))
        (Transformation|SetWorldScale3D _returnvalue (Math|Vector|SelectVector _arrowhitscale (Transformation|GetActorScale3D) (> (Math|Vector|VectorLength _arrowhitscale) 0.0)))
        (Effects|Components|ParticleSystem|SetColorParameter _returnvalue "MagicColor" (Variables|Default|GetColor))
        (Audio|Components|Audio|Stop (Variables|Default|GetAudio))
        (if (Variables|Default|GetLinger)
          (Utilities|Time|SetTimerbyEvent (delegate Custom|StartDie) 1e+01)
          (else
            (CallFunction|DieImmediate)))
        (CallFunction|PlayDeathSound HitLocation)))))

(fn ConstructionScript)