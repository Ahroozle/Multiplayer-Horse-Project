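; Magic spotlight actor that aims at the mouse cursor while attached to another actor.
; If player 0 controls the attach parent's owner, a looping timer deprojects the cursor onto the parent's ground plane or a camera-facing plane, favoring the nearer hit.
; It sends look-at rotation and distance-based scale to the owning ObserverBP's UpdateSpotlight.
; SetTransformForMouse applies a given rotation and scale, with no caller in this file.
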(event Custom|FinishBeginPlay
  (if (== (Pawn|GetController (.AsPawn (Utilities|Casting|CastToPawn (Components|GetOwner (Actor|GetAttachParentActor))))) (Game|GetPlayerController 0))
    (CallFunction|SetRequiredData)
    (Utilities|Time|SetTimerbyFunctionName 0 "TrackMouse" 0.01 true)
    (CallFunction|TrackMouse)))

(event EventBeginPlay
  (Utilities|Time|SetTimerbyEvent (delegate Custom|FinishBeginPlay) 0.01)
  (Variables|Default|SetStartingScale (Transformation|GetWorldScale (Variables|Default|GetScene))))

(fn ConstructionScript)

(fn TrackMouse
  (bind _returnvalue (Game|GetPlayerController 0))
  (bind _returnvalue_2 (Transformation|GetActorLocation))
  (bind _returnvalue_3 (Transformation|GetActorLocation))
  (bind _relevantcamera (Variables|Default|GetRelevantCamera))
  (bind _relevantcamera_2 (Variables|Default|GetRelevantCamera))
  (bind _groundplaneoffset (Variables|Default|GetGroundPlaneOffset))
  (bind _attachactor (Variables|Default|GetAttachActor))
  (bind (_worldlocation _worlddirection _returnvalue_4) (Game|Player|ConvertMouseLocationToWorldSpace _returnvalue))
  (bind _returnvalue_5 (Transformation|GetActorLocation _attachactor))
  (bind _returnvalue_6 (Transformation|GetWorldLocation _relevantcamera_2))
  (bind _returnvalue_7 (Math|Vector|GetForwardVector _relevantcamera))
  (bind _returnvalue_8 (Math|Vector|NegateVector _returnvalue_7))
  (bind _returnvalue_9 (* _worlddirection 1e+06))
  (bind _returnvalue_10 (- _returnvalue_5 _groundplaneoffset))
  (bind _returnvalue_11 (* _returnvalue_7 1e+03))
  (bind _returnvalue_12 (+ _worldlocation _returnvalue_9))
  (bind _returnvalue_13 (+ _returnvalue_3 _returnvalue_11))
  (bind (_t _intersection _returnvalue_14) (Class|KismetMathLibrary|LinePlaneIntersectionOriginNormal _worldlocation _returnvalue_12 _returnvalue_10 "0, 0,1.000000"))
  (bind _intersection_2 (Class|KismetMathLibrary|LinePlaneIntersectionOriginNormal _worldlocation _returnvalue_12 _returnvalue_13 _returnvalue_8))
  (if _returnvalue_4
    (LocalVariables|SetHitPos (Math|Vector|SelectVector _intersection_2 _intersection (or (not _returnvalue_14) (< (Math|Vector|VectorLength (- _intersection_2 _returnvalue_6)) (Math|Vector|VectorLength (- _intersection _returnvalue_6))))))
    (bind _obs (Variables|Default|GetObs)
      (:then
        (Default|UpdateSpotlight _obs (Math|Rotator|FindLookatRotation _returnvalue_2 (LocalVariables|GetHitPos)) (* (Variables|Default|GetStartingScale) (/ (Math|Vector|VectorLength (- _returnvalue_2 (LocalVariables|GetHitPos))) 5e+03))))
      (:else))))

(fn SetTransformforMouse
  (params (Rot :type Rotator) (Scale :type Vector))
  (Transformation|SetWorldRotation (Variables|Default|GetDefaultSceneRoot) Rot false false)
  (Transformation|SetWorldScale3D (Variables|Default|GetScene) Scale))

(fn SetRequiredData
  (Variables|Default|SetRelevantCamera (Class|MPHorsoGameInstance|GetRelevantCamera (Class|StaticFuncLib|RetrieveGameInstance)))
  (bind _output_get (Variables|Default|SetAttachActor (Actor|GetAttachParentActor)))
  (Variables|Default|SetObs (.AsObserver%20BP (Utilities|Casting|CastToObserverBP (Components|GetOwner _output_get))))
  (bind _output_get_2 (LocalVariables|SetCaps (Actor|GetComponentbyClass _output_get "/Script/Engine.CapsuleComponent")))
  (Utilities|IsValid _output_get_2
    (:Is%20Valid
      (Variables|Default|SetGroundPlaneOffset (Math|Vector|MakeVector 0.0 0.0 (Components|Capsule|GetUnscaledCapsuleHalfHeight (LocalVariables|GetCaps)))))))