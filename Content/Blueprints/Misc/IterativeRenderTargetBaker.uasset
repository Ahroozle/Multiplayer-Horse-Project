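; Blueprint utility that iteratively bakes a material into a pair of render targets from its Construction Script.
; A one-shot Refresh flag or the BakeOnEdit option runs one bake per construction, then increments the iteration counter.
; Each bake ping-pongs TargA and TargB by iteration parity, feeding one into a dynamic material's texture parameter and drawing into the cleared other, so each pass builds on the last.
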(fn ConstructionScript
  (if (or (Variables|Default|GetRefresh) (Variables|Default|GetBakeOnEdit))
    (Variables|Default|SetRefresh false)
    (CallFunction|Bake)
    (Math|Integer|IncrementInt (Variables|Default|GetCurrIteration))))

(fn Bake
  (bind _targa (Variables|Default|GetTargA))
  (bind _targb (Variables|Default|GetTargB))
  (bind _curriteration (Variables|Default|GetCurrIteration))
  (bind _returnvalue (Math|Integer|%(Integer) _curriteration 2))
  (bind _returnvalue_2 (== _returnvalue 0))
  (bind _returnvalue_3 (Utilities|SelectObject _targb _targa _returnvalue_2))
  (bind _astexture_render_target_2d (Utilities|Casting|CastToTextureRenderTarget2D _returnvalue_3))
  (if (Math|Boolean|ANDBoolean (Utilities|IsValid (Variables|Default|GetTargA)) (Utilities|IsValid (Variables|Default|GetTargB)) (Utilities|IsValid (Variables|Default|GetMaterialToBake)))
    (bind _returnvalue_4 (Rendering|Material|CreateDynamicMaterialInstance (Variables|Default|GetMaterialToBake) :!class /Script/Engine.KismetMaterialLibrary))
    (LocalVariables|SetDynMat _returnvalue_4)
    (if (>= (Variables|Default|GetCurrIteration) 0)
      (Rendering|Material|SetTextureParameterValue (LocalVariables|GetDynMat) (Variables|Default|GetTexParamName) (.AsTexture%20Render%20Target%202D (Utilities|Casting|CastToTextureRenderTarget2D (Utilities|SelectObject (Variables|Default|GetTargA) (Variables|Default|GetTargB) (== (Math|Integer|%(Integer) (Variables|Default|GetCurrIteration) 2) 0))))))
    (Rendering|ClearRenderTarget2D self _astexture_render_target_2d)
    (Rendering|DrawMaterialtoRenderTarget _astexture_render_target_2d (LocalVariables|GetDynMat))))