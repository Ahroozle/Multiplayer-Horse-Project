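; ColorSchemeDisplayer is a test-style actor that previews randomly generated horse color schemes on five components, P1 to P5.
; BeginPlay creates a dynamic material instance for each component and stores it in an array.
; Pressing F builds a separate random scheme per instance, with varying body and hair color counts and one eye color, converts it to a texture and assigns it to the Palette parameter.
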(event EventBeginPlay
  (for _array_element (Utilities|Array|MakeArray (Variables|Default|GetP1) (Variables|Default|GetP2) (Variables|Default|GetP3) (Variables|Default|GetP4) (Variables|Default|GetP5))
    (bind _returnvalue (Rendering|Material|CreateDynamicMaterialInstance _array_element 0 0 :!class /Script/Engine.PrimitiveComponent))
    (Utilities|Array|Add (Variables|Default|GetDyns) _returnvalue)))

(event Input|KeyboardEvents|F
  (params (Key :type Key%20Structure :default "AnyKey"))
  (:Pressed
    (for _array_element (Variables|Default|GetDyns)
      (bind _returnvalue (Class|StaticFuncLib|MakeTextureforColorScheme (Class|StaticFuncLib|MakeRandomHorseColorScheme (Math|Random|RandomIntegerinRange 1 2) (Math|Random|RandomIntegerinRange 1 3) 1)))
      (Rendering|Material|SetTextureParameterValue _array_element "Palette" _returnvalue))))

(fn ConstructionScript)