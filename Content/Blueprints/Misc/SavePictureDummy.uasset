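; Pony dummy actor that mirrors a character-creator dummy and renders a snapshot of itself, apparently for save pictures.
; It maps skeletal sprite flipbook parts by name to copy, apply, export or reset skins and colors, handling single-color and multi-region skins.
; Race switching toggles wing and horn visibility.
; Snap uses a self-only SceneCapture2D and a fresh render target to return a texture and its pixel colors.
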(event EventBeginPlay
  (CallFunction|PopulateMaps)
  (Components|Timeline|SetLooping (Variables|Default|GetRightLid) false)
  (Variables|/Script/Engine.SceneCaptureComponent|SetShowOnlyActors (Variables|Default|GetSceneCaptureComponent2D) (Utilities|Array|MakeArray self)))

(fn ConstructionScript)

(fn SwitchRace
  (params (NewRace :type ERaceType%20Enum))
  (bind _output_get (Variables|Default|SetCurrRace NewRace))
  (switch Utilities|FlowControl|Switch|SwitchonERaceType _output_get
    (:Race_EarthP
      (Rendering|SetVisibility (Variables|Default|GetWings) false true))
    (:Race_Pega
      (Rendering|SetVisibility (Variables|Default|GetWings) true true)
      (Rendering|SetVisibility (Variables|Default|GetHorn) false false))
    (:Race_Uni
      (Rendering|SetVisibility (Variables|Default|GetHorn) true false)
      (Rendering|SetVisibility (Variables|Default|GetWings) false true))))

(fn GetColorSchemeasString
  (LocalVariables|SetResStr (Utilities|String|EnumtoString (Variables|Default|GetCurrRace)))
  (for _array_element (Actor|GetComponentsByClass "/Script/MPHorso.SkeletalSpriteFlipbookComponent")
    (LocalVariables|SetResStr (Utilities|String|Append (LocalVariables|GetResStr) " 
" (Utilities|GetObjectName _array_element) "|" (Utilities|String|ToString(Integer) (Variables|/Script/Paper2D.PaperFlipbookComponent|GetSpriteColor _array_element)))))
  (return (LocalVariables|GetResStr)))

(fn PopulateMaps
  (for _array_element (Actor|GetComponentsByClass "/Script/MPHorso.SkeletalSpriteFlipbookComponent")
    (Utilities|Map|Add (Variables|Default|GetPartsByName) (Utilities|String|StringToName (Utilities|GetObjectName _array_element)) _array_element)
    (Utilities|Map|Add (Variables|Default|GetSkinsForParts) _array_element (Variables|/Script/MPHorso.SkeletalSpriteFlipbookComponent|GetSkinSet _array_element))))

(fn GetColorsasScheme
  (bind _scheme (LocalVariables|GetScheme))
  (bind _keys (Utilities|Map|Keys (Variables|Default|GetPartsByName)))
  (for _array_element _keys
    (if (> (Class|SkeletalSpriteSkinSetBase|GetSkinNumRegions (Variables|/Script/MPHorso.SkeletalSpriteFlipbookComponent|GetSkinSet (.Value (Utilities|Map|Find (Variables|Default|GetPartsByName) _array_element))) (Variables|/Script/MPHorso.SkeletalSpriteFlipbookComponent|GetCurrentRegionSet (.Value (Utilities|Map|Find (Variables|Default|GetPartsByName) _array_element)))) 1)
      (Utilities|Map|Add _scheme _array_element (Utilities|Struct|MakeCharColorSchemePart (Class|SkeletalSpriteSkinSetBase|GetSaveableSkinName (Variables|/Script/MPHorso.SkeletalSpriteFlipbookComponent|GetSkinSet (.Value (Utilities|Map|Find (Variables|Default|GetPartsByName) _array_element)))) (Variables|/Script/MPHorso.SkeletalSpriteFlipbookComponent|GetCurrentRegionSet (.Value (Utilities|Map|Find (Variables|Default|GetPartsByName) _array_element))) (Class|SkeletalSpriteFlipbookComponent|GetRegionColors (.Value (Utilities|Map|Find (Variables|Default|GetPartsByName) _array_element)))))
      (else
        (Utilities|Map|Add _scheme _array_element (Utilities|Struct|MakeCharColorSchemePart (Class|SkeletalSpriteSkinSetBase|GetSaveableSkinName (Variables|/Script/MPHorso.SkeletalSpriteFlipbookComponent|GetSkinSet (.Value (Utilities|Map|Find (Variables|Default|GetPartsByName) _array_element)))) (Variables|/Script/MPHorso.SkeletalSpriteFlipbookComponent|GetCurrentRegionSet (.Value (Utilities|Map|Find (Variables|Default|GetPartsByName) _array_element))) (Utilities|Array|MakeArray (Variables|/Script/Paper2D.PaperFlipbookComponent|GetSpriteColor (.Value (Utilities|Map|Find (Variables|Default|GetPartsByName) _array_element)))))))))
  (return (LocalVariables|GetScheme)))

(fn Reset
  (bind _values (Utilities|Map|Values (Variables|Default|GetPartsByName)))
  (for _array_element _values
    (Class|SkeletalSpriteFlipbookComponent|SetRegionColors _array_element (LocalVariables|GetOriginalRegions))
    (Sprite|SetSpriteColor _array_element "(R=1.000000,G=1.000000,B=1.000000,A=1.000000)")
    (if (.ReturnValue (Utilities|Map|Find (Variables|Default|GetSkinsForParts) _array_element))
      (Class|SkeletalSpriteFlipbookComponent|ChangeSkin _array_element (.Value (Utilities|Map|Find (Variables|Default|GetSkinsForParts) _array_element)))))
  (Rendering|SetVisibility (Variables|Default|GetMagic) false true)
  (Sprite|SetSpriteColor (Variables|Default|GetLeftPupil) "(R=0.150000,G=0.150000,B=0.150000,A=1.000000)")
  (Sprite|SetSpriteColor (Variables|Default|GetLowerMane_Front) "(R=1.000000,G=0.679543,B=0.000000,A=1.000000)"))

(fn SetColorScheme
  (params (ColorScheme :type Map%20of%20Names%20to%20Structs))
  (bind _keys (Utilities|Map|Keys ColorScheme))
  (for _array_element _keys
    (if (.ReturnValue (Utilities|Map|Find (Variables|Default|GetPartsByName) _array_element))
      (bind _returnvalue (Class|SkeletalSpriteSkinSetBase|LoadSkinSetfromName (.SkinSetName (Utilities|Struct|BreakCharColorSchemePart (.Value (Utilities|Map|Find ColorScheme _array_element))))))
      (Class|SkeletalSpriteFlipbookComponent|ChangeSkin (.Value (Utilities|Map|Find (Variables|Default|GetPartsByName) _array_element)) _returnvalue (.RegionSet (Utilities|Struct|BreakCharColorSchemePart (.Value (Utilities|Map|Find ColorScheme _array_element)))))
      (if (> (Class|SkeletalSpriteSkinSetBase|GetSkinNumRegions _returnvalue (.RegionSet (Utilities|Struct|BreakCharColorSchemePart (.Value (Utilities|Map|Find ColorScheme _array_element))))) 1)
        (Class|SkeletalSpriteFlipbookComponent|SetRegionColors (.Value (Utilities|Map|Find (Variables|Default|GetPartsByName) _array_element)) (.Colors (Utilities|Struct|BreakCharColorSchemePart (.Value (Utilities|Map|Find ColorScheme _array_element)))))
        (else
          (Sprite|SetSpriteColor (.Value (Utilities|Map|Find (Variables|Default|GetPartsByName) _array_element)) (Utilities|Array|Get(acopy) (.Colors (Utilities|Struct|BreakCharColorSchemePart (.Value (Utilities|Map|Find ColorScheme _array_element)))))))))))

(fn SetColorforParts
  (params (Parts :type Array%20of%20Names) (Color :type Linear%20Color%20Structure) (Region :type Integer))
  (for _array_element Parts
    (if (.ReturnValue (Utilities|Map|Find (Variables|Default|GetPartsByName) _array_element))
      (if (<= Region 0)
        (Sprite|SetSpriteColor (.Value (Utilities|Map|Find (Variables|Default|GetPartsByName) _array_element)) Color)
        (else
          (bind _output_get (LocalVariables|SetColsCopy (Class|SkeletalSpriteFlipbookComponent|GetRegionColors (.Value (Utilities|Map|Find (Variables|Default|GetPartsByName) _array_element)))))
          (Utilities|Array|SetArrayElem _output_get (- Region 1) Color)
          (Class|SkeletalSpriteFlipbookComponent|SetRegionColors (.Value (Utilities|Map|Find (Variables|Default|GetPartsByName) _array_element)) (LocalVariables|GetColsCopy)))))))

(fn Blink
  (bind _rightlid (Variables|Default|GetRightLid))
  (if (not (Audio|Components|Audio|IsPlaying _rightlid))
    (for _array_element (Utilities|Array|MakeArray _rightlid (Variables|Default|GetRightLidRim) (Variables|Default|GetLeftLid) (Variables|Default|GetLeftLidRim))
      (Sprite|SetFlipbook _array_element (.Value (Utilities|Map|Find (Variables|/Script/MPHorso.SkeletalSpriteFlipbookComponent|GetLocalSkins _array_element) "Blink")))
      (Components|Timeline|PlayfromStart _array_element))))

(fn SwitchSkinsforParts
  (params (Parts :type Array%20of%20Names) (NewSkins :type Array%20of%20Skeletal%20Sprite%20Skin%20Set%20Base%20Class%20References) (RegionSet :type Integer))
  (for (_array_element _array_index) Parts
    (if (Utilities|IsValidClass (Utilities|Array|Get(acopy) NewSkins _array_index))
      (if (.ReturnValue (Utilities|Map|Find (Variables|Default|GetPartsByName) _array_element))
        (if (and (Variables|/Script/MPHorso.SkeletalSpriteFlipbookComponent|GetUsesRegions (.Value (Utilities|Map|Find (Variables|Default|GetPartsByName) _array_element))) (<= (Class|SkeletalSpriteSkinSetBase|GetSkinNumRegions (Utilities|Array|Get(acopy) NewSkins _array_index) RegionSet) 1))
          (Sprite|SetSpriteColor (.Value (Utilities|Map|Find (Variables|Default|GetPartsByName) _array_element)) (Utilities|Array|Get(acopy) (Class|SkeletalSpriteFlipbookComponent|GetRegionColors (.Value (Utilities|Map|Find (Variables|Default|GetPartsByName) _array_element)))))
          (elif (and (not (Variables|/Script/MPHorso.SkeletalSpriteFlipbookComponent|GetUsesRegions (.Value (Utilities|Map|Find (Variables|Default|GetPartsByName) _array_element)))) (> (Class|SkeletalSpriteSkinSetBase|GetSkinNumRegions (Utilities|Array|Get(acopy) NewSkins _array_index) RegionSet) 1))
            (bind _output_get (LocalVariables|SetRegionColorsCopy (Class|SkeletalSpriteFlipbookComponent|GetRegionColors (.Value (Utilities|Map|Find (Variables|Default|GetPartsByName) _array_element)))))
            (Utilities|Array|SetArrayElem _output_get 0 (Variables|/Script/Paper2D.PaperFlipbookComponent|GetSpriteColor (.Value (Utilities|Map|Find (Variables|Default|GetPartsByName) _array_element))))
            (Class|SkeletalSpriteFlipbookComponent|SetRegionColors (.Value (Utilities|Map|Find (Variables|Default|GetPartsByName) _array_element)) (LocalVariables|GetRegionColorsCopy))
            (Sprite|SetSpriteColor (.Value (Utilities|Map|Find (Variables|Default|GetPartsByName) _array_element)) "(R=1.000000,G=1.000000,B=1.000000,A=1.000000)")))
        (Class|SkeletalSpriteFlipbookComponent|ChangeSkin (.Value (Utilities|Map|Find (Variables|Default|GetPartsByName) _array_element)) (Utilities|Array|Get(acopy) NewSkins _array_index) RegionSet)))))

(fn Snap
  (bind _scenecapturecomponent2d (Variables|Default|GetSceneCaptureComponent2D))
  (bind _returnvalue (Rendering|CreateRenderTarget2D 256 256))
  (bind _output_get (Variables|/Script/Engine.SceneCaptureComponent2D|SetTextureTarget _scenecapturecomponent2d _returnvalue))
  (Rendering|SceneCapture|CaptureScene _scenecapturecomponent2d :!class /Script/Engine.SceneCaptureComponent2D)
  (bind (_outcolors _returnvalue_2) (Class|StaticFuncLib|MakeTexturefromRenderTarget _output_get true))
  (return _outcolors _returnvalue_2))

(fn CopyfromCreatorDummy
  (params (CreatorDummy :type Character%20Creator%20Dummy%20Object%20Reference))
  (bind _partsbyname (Variables|/Game/Blueprints/Misc/CharacterCreatorDummy.CharacterCreatorDummy_C|GetPartsByName CreatorDummy))
  (CallFunction|SwitchRace (Variables|/Game/Blueprints/Misc/CharacterCreatorDummy.CharacterCreatorDummy_C|GetCurrRace CreatorDummy))
  (bind _keys (Utilities|Map|Keys _partsbyname))
  (for _array_element _keys
    (if (.ReturnValue (Utilities|Map|Find (Variables|Default|GetPartsByName) _array_element))
      (Class|SkeletalSpriteFlipbookComponent|ChangeSkin (.Value (Utilities|Map|Find (Variables|Default|GetPartsByName) _array_element)) (Variables|/Script/MPHorso.SkeletalSpriteFlipbookComponent|GetSkinSet (.Value (Utilities|Map|Find _partsbyname _array_element))) (Variables|/Script/MPHorso.SkeletalSpriteFlipbookComponent|GetCurrentRegionSet (.Value (Utilities|Map|Find _partsbyname _array_element))))
      (if (> (Class|SkeletalSpriteSkinSetBase|GetSkinNumRegions (Variables|/Script/MPHorso.SkeletalSpriteFlipbookComponent|GetSkinSet (.Value (Utilities|Map|Find _partsbyname _array_element))) (Variables|/Script/MPHorso.SkeletalSpriteFlipbookComponent|GetCurrentRegionSet (.Value (Utilities|Map|Find _partsbyname _array_element)))) 1)
        (Class|SkeletalSpriteFlipbookComponent|SetRegionColors (.Value (Utilities|Map|Find (Variables|Default|GetPartsByName) _array_element)) (Class|SkeletalSpriteFlipbookComponent|GetRegionColors (.Value (Utilities|Map|Find _partsbyname _array_element))))
        (else
          (Sprite|SetSpriteColor (.Value (Utilities|Map|Find (Variables|Default|GetPartsByName) _array_element)) (Variables|/Script/Paper2D.PaperFlipbookComponent|GetSpriteColor (.Value (Utilities|Map|Find _partsbyname _array_element)))))))))