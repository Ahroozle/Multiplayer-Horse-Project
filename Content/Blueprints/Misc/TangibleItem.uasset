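; TangibleItem is a physical, billboarded item pickup that gravitates to a player with inventory room, ignoring its owner for a short delay after reset.
; Pickup requests route through ObserverBP, and a timed lerp pulls it in before calling TakeItem.
; It toggles a replicated Alive state instead of being destroyed, parking below the world and releasing attached barriers.
; While alive it plays impact sounds, hops when resting, and stretches a raycast decal shadow.
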(event OnComponentHit(ItemCollision)
  (params (HitComponent :type Primitive%20Component%20Object%20Reference) (OtherActor :type Actor%20Object%20Reference) (OtherComp :type Primitive%20Component%20Object%20Reference) (NormalImpulse :type Vector) (Hit :type Hit%20Result%20Structure%20%28by%20ref%29))
  (bind _impactpoint (Collision|BreakHitResult Hit))
  (if (Math|Vector|NotEqual(Vector) (Variables|Default|GetLastHitLocation) _impactpoint 1e+02)
    (Variables|Default|SetLastHitLocation _impactpoint)
    (bind _returnvalue (Class|StaticFuncLib|PlaySound (Math|Transform|MakeTransform (Transformation|GetActorLocation) "0, 0, 0" "1,1,1") "/Game/Assets/Sound/SFX/ItemContact/ItemContact_Cue.ItemContact_Cue" 1.0))
    (Audio|Components|Audio|AdjustAttenuation (Variables|/Script/MPHorso.OneShotAudio|GetaudioComp _returnvalue) (Variables|Default|GetAtten))
    (Audio|Components|Audio|Play (Variables|/Script/MPHorso.OneShotAudio|GetaudioComp _returnvalue) 0.0)
    (else
      (Variables|Default|SetLastHitLocation _impactpoint)
      (if (<= (Math|Vector|VectorLengthSquared (Transformation|GetVelocity)) 1e+02)
        (if (not (Utilities|Time|IsTimerActivebyHandle (Variables|Default|GetHopTimer)))
          (bind _returnvalue_2 (Utilities|Time|SetTimerbyFunctionName 0 "Hop" (Variables|Default|GetHopDelay)))
          (Variables|Default|SetHopTimer _returnvalue_2))))))

(event Custom|Gravitate
  (bind _target (Variables|Default|GetTarget))
  (bind _returnvalue (Transformation|GetActorLocation _target))
  (bind _output_get (Variables|Default|SetCurrGravitateTime (+ (Variables|Default|GetCurrGravitateTime) (Utilities|Time|GetWorldDeltaSeconds))))
  (if (Math|Vector|Equal(Vector) (Math|Vector|Lerp(Vector) (Transformation|GetActorLocation) _returnvalue (/ _output_get (Variables|Default|GetMaxGravitateTime))) _returnvalue 5e+01)
    (Utilities|Time|ClearandInvalidateTimerbyHandle (stale Custom|StartGravitate _returnvalue))
    (Utilities|Time|ClearandInvalidateTimerbyHandle (Variables|Default|GetHopTimer))
    (Variables|Default|GetHeldClass
      (:then
        (Default|TakeItem (.AsObserver%20BP (Utilities|Casting|CastToObserverBP (Components|GetOwner (Variables|Default|GetTarget)))) (Variables|Default|GetHeldPrefixes) (Variables|Default|GetHeldClass) (Variables|Default|GetHeldStack)))
      (:else
        _))
    (Default|SetItemAlive (.AsObserver%20BP (Utilities|Casting|CastToObserverBP (Pawn|GetControlledPawn (Game|GetPlayerController 0)))) self false)
    (else
      (Transformation|SetActorLocation (Math|Vector|Lerp(Vector) (Transformation|GetActorLocation) _returnvalue (/ _output_get (Variables|Default|GetMaxGravitateTime))) false false))))

(event Custom|SetAliveMulticast
  (params (NewAlive :type Boolean))
  (CallFunction|SetAliveInternal NewAlive))

(event Custom|StartGravitate
  (params (Targ :type Actor%20Object%20Reference))
  (Variables|Default|SetTarget Targ)
  (Variables|Default|SetCurrGravitateTime 0.0)
  (bind _returnvalue (Utilities|Time|SetTimerbyEvent (delegate Custom|Gravitate) 0.01 true)))

(event Custom|ResetActor
  (Variables|Default|SetLastHitLocation (Transformation|GetActorLocation))
  (Variables|Default|SetGravToOwner false)
  (Default|SetItemAlive (.AsObserver%20BP (Utilities|Casting|CastToObserverBP (Pawn|GetControlledPawn (Game|GetPlayerController 0)))) self true)
  (bind _heldclass (Variables|Default|GetHeldClass)
    (:then
      (Rendering|Components|Sprite|SetSprite (Variables|Default|GetBillboard) (.AsTexture%202D (Utilities|Casting|CastToTexture2D (Class|MPHorsoItemHelperLibrary|GetDefaultItemImage _heldclass)))))
    (:else
      _))
  (Utilities|Time|SetTimerbyEvent (delegate Custom|TimeUp) 2.0))

(event Custom|TimeUp
  (bind _returnvalue (Components|GetOwner))
  (Variables|Default|SetGravToOwner true)
  (if (Collision|IsOverlappingActor _returnvalue :!class /Script/Engine.Actor)
    (Default|MakeItemGravto (.AsObserver%20BP (Utilities|Casting|CastToObserverBP (Pawn|GetControlledPawn (Game|GetPlayerController 0)))) self _returnvalue)))

(event Custom|SetAlive
  (params (NewAlive :type Boolean))
  (CallFunction|SetAliveProxy NewAlive))

(event Custom|SetAliveProxy
  (params (NewAlive :type Boolean))
  (CallFunction|SetAliveMulticast NewAlive))

(event EventBeginPlay
  (CallFunction|ResetActor))

(event Collision|EventActorBeginOverlap
  (params (OtherActor :type Actor%20Object%20Reference))
  (if (or (!= OtherActor (Components|GetOwner)) (Variables|Default|GetGravToOwner))
    (bind _asplayer_entity_base_bp (Utilities|Casting|CastToPlayerEntityBaseBP OtherActor))
    (bind _asobserver_bp (Utilities|Casting|CastToObserverBP (Components|GetOwner _asplayer_entity_base_bp)))
    (bind _invwidg (Variables|/Game/Blueprints/ObserverBP.ObserverBP_C|GetInvWidg _asobserver_bp)
      (:then
        (if (Default|InventoryNotFull _invwidg (Variables|Default|GetHeldClass))
          (Default|MakeItemGravto (.AsObserver%20BP (Utilities|Casting|CastToObserverBP (Pawn|GetControlledPawn (Game|GetPlayerController 0)))) self _asplayer_entity_base_bp)))
      (:else))))

(fn ConstructionScript)

(fn RaycastShadow
  (bind _returnvalue (Transformation|GetActorLocation))
  (bind _decal (Variables|Default|GetDecal))
  (bind (_outhit _returnvalue_2) (Collision|LineTraceByChannel _returnvalue (- _returnvalue "0, 0,100000.000000") "TraceTypeQuery1" false 0 "None"))
  (if _returnvalue_2
    (Transformation|SetRelativeScale3D _decal (Math|Vector|MakeVector (/ (Math|Float|Absolute(Float) (.z (- (Transformation|GetActorLocation) (- (.ImpactPoint (Collision|BreakHitResult _outhit)) "0, 0,100.000000")))) 32.0) 1.0 1.0))
    (Transformation|SetRelativeLocation _decal (Math|Vector|MakeVector 0.0 0.0 (* (/ (Math|Float|Absolute(Float) (.z (- (Transformation|GetActorLocation) (- (.ImpactPoint (Collision|BreakHitResult _outhit)) "0, 0,100.000000")))) 2.0) -1.0)) false false)))

(fn SetAliveInternal
  (params (NewAlive :type Boolean))
  (bind _output_get (Variables|Default|SetAlive NewAlive))
  (Rendering|SetActorHiddenInGame (not _output_get))
  (Collision|SetActorEnableCollision _output_get)
  (Actor|Tick|SetActorTickEnabled _output_get)
  (Physics|SetSimulatePhysics (Variables|Default|GetItemCollision) _output_get)
  (if _output_get
    (Utilities|Time|SetTimerbyFunctionName 0 "RaycastShadow" 0.01 true)
    (else
      (Utilities|Time|ClearTimerbyFunctionName 0 "RaycastShadow")
      (for _array_element (Actor|GetAttachedActors)
        (bind _asbarrier_base (Utilities|Casting|CastToBarrierBase _array_element))
        (Transformation|DetachFromActor _asbarrier_base "KeepWorld" "KeepRelative" "KeepRelative")
        (bind _asobserver_bp (Utilities|Casting|CastToObserverBP (Components|GetOwner (Components|GetOwner _asbarrier_base))))
        (Default|CastMagic _asobserver_bp "/Game/Blueprints/Magic/BarrierMagicUI.BarrierMagicUI_C"))
      (Utilities|Time|SetTimerbyFunctionName 0 "FinishSetAlive" 0.01))))

(fn OnRepHeldClass
  (bind _heldclass (Variables|Default|GetHeldClass)
    (:then
      (Rendering|Components|Sprite|SetSprite (Variables|Default|GetBillboard) (.AsTexture%202D (Utilities|Casting|CastToTexture2D (Class|MPHorsoItemHelperLibrary|GetDefaultItemImage _heldclass)))))
    (:else)))

(fn OnRepAlive
  (bind _alive (Variables|Default|GetAlive))
  (Rendering|SetActorHiddenInGame (not _alive))
  (Collision|SetActorEnableCollision _alive)
  (Actor|Tick|SetActorTickEnabled _alive)
  (Physics|SetSimulatePhysics (Variables|Default|GetItemCollision) _alive)
  (if _alive
    (Utilities|Time|SetTimerbyFunctionName 0 "RaycastShadow" 0.01 true)
    (else
      (Utilities|Time|ClearTimerbyFunctionName 0 "RaycastShadow")
      (for _array_element (Actor|GetAttachedActors)
        (bind _asbarrier_base (Utilities|Casting|CastToBarrierBase _array_element))
        (Transformation|DetachFromActor _asbarrier_base "KeepWorld" "KeepRelative" "KeepRelative")
        (bind _asobserver_bp (Utilities|Casting|CastToObserverBP (Components|GetOwner (Components|GetOwner _asbarrier_base))))
        (if (and (Networking|IsServer) (Default|SustainedSpellsContains (.AsPlayer%20Entity%20Base%20BP (Utilities|Casting|CastToPlayerEntityBaseBP (Components|GetOwner _asbarrier_base))) "Barrier"))
          (Default|CastMagic _asobserver_bp "/Game/Blueprints/Magic/BarrierMagicUI.BarrierMagicUI_C")))
      (bind _asmagic_grab (Utilities|Casting|CastToMagicGrab (Actor|GetAttachParentActor))
        (:then
          (bind _asobserver_bp_2 (Utilities|Casting|CastToObserverBP (Components|GetOwner (Components|GetOwner _asmagic_grab)))
            (:then
              (if (and (Networking|IsServer) (Default|SustainedSpellsContains (.AsPlayer%20Entity%20Base%20BP (Utilities|Casting|CastToPlayerEntityBaseBP (Components|GetOwner _asmagic_grab))) "Telegrab"))
                (Default|CastMagic _asobserver_bp_2 "/Game/Blueprints/Magic/TelegrabMagicUI.TelegrabMagicUI_C")))
            (:CastFailed
              _)))
        (:CastFailed
          _))
      (Utilities|Time|SetTimerbyFunctionName 0 "FinishSetAlive" 0.01))))

(fn Hop
  (bind _itemcollision (Variables|Default|GetItemCollision))
  (if (Physics|IsSimulatingPhysics _itemcollision "None")
    (Physics|AddImpulse _itemcollision "0, 0,250.000000" "None" true)
    (bind _returnvalue (Class|StaticFuncLib|PlaySound (Math|Transform|MakeTransform (Transformation|GetActorLocation) "0, 0, 0" "1,1,1") "/Game/Assets/Sound/SFX/ItemContact/ItemContact_Cue.ItemContact_Cue" 1.0))
    (Audio|Components|Audio|AdjustAttenuation (Variables|/Script/MPHorso.OneShotAudio|GetaudioComp _returnvalue) (Variables|Default|GetAtten))
    (Audio|Components|Audio|Play (Variables|/Script/MPHorso.OneShotAudio|GetaudioComp _returnvalue) 0.0)))

(fn FinishSetAlive
  (Transformation|SetActorLocation "0, 0,-100000.000000" false false))

(fn IsCurrentlyManipulable
  (params (Querier :type Controller%20Object%20Reference))
  (return true))