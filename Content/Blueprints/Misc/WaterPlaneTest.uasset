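; Test water plane actor that makes overlapping characters and primitive components float on its displaced wave surface.
; Reads displacement parameters from the plane's dynamic material and computes surface height at each object's location with CalcWaterSurface.
; Looping timers ease vertical velocity toward that surface over RiseSeconds, nudging deeply submerged walking characters with LaunchCharacter.
; Friction and damping are overridden near or below the surface, then restored from cached values above it or on exit.
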(event Collision|EventActorBeginOverlap
  (params (OtherActor :type Actor%20Object%20Reference))
  (bind _returnvalue (Actor|GetComponentbyClass OtherActor "/Script/Engine.PrimitiveComponent"))
  (bind _ascharacter (Utilities|Casting|CastToCharacter OtherActor)
    (:then
      (Utilities|Map|Add (Variables|Default|GetMonitoredCharacters) _ascharacter 0.0)
      (Utilities|Map|Add (Variables|Default|GetHeldFrictions) (Variables|/Script/Engine.Character|GetCharacterMovement _ascharacter) (Variables|/Script/Engine.CharacterMovementComponent|GetFallingLateralFriction (Variables|/Script/Engine.Character|GetCharacterMovement _ascharacter))))
    (:CastFailed
      (Utilities|IsValid _returnvalue
        (:Is%20Valid
          (Utilities|Map|Add (Variables|Default|GetMonitoredPrims) _returnvalue 0.0)
          (Utilities|Map|Add (Variables|Default|GetHeldFrictions) _returnvalue (Class|PrimitiveComponent|GetLinearDamping _returnvalue)))))))

(event EventBeginPlay
  (Utilities|Time|SetTimerbyFunctionName 0 "TickCharacterBuoyancy" 0.01 true)
  (Utilities|Time|SetTimerbyFunctionName 0 "TickPrimitiveBuoyancy" 0.01 true)
  (bind _returnvalue (Rendering|Material|CreateDynamicMaterialInstance (Variables|Default|GetPlane) 0 0 :!class /Script/Engine.PrimitiveComponent))
  (bind _output_get (Variables|Default|SetDynMat _returnvalue))
  (bind _returnvalue_2 (Rendering|Material|GetScalarParameterValue _output_get "DisplacementScale" :!class /Script/Engine.MaterialInstanceDynamic))
  (Variables|Default|SetDispScale _returnvalue_2)
  (bind _returnvalue_3 (Rendering|Material|GetScalarParameterValue _output_get "DisplacementStrength" :!class /Script/Engine.MaterialInstanceDynamic))
  (Variables|Default|SetDispStrength _returnvalue_3))

(event Collision|EventActorEndOverlap
  (params (OtherActor :type Actor%20Object%20Reference))
  (CallFunction|SafeRemove OtherActor))

(fn ConstructionScript)

(fn TickCharacterBuoyancy
  (bind _keys (Utilities|Map|Keys (Variables|Default|GetMonitoredCharacters)))
  (for _array_element _keys
    (Utilities|IsValid _array_element
      (:Is%20Valid
        (if (> (.Z (Math|Vector|BreakVector (- (CallFunction|CalcBuoyPoint (Transformation|GetActorLocation _array_element)) (Transformation|GetActorLocation _array_element)))) -1e+02)
          (bind _output_get (LocalVariables|SetCurrSeconds (Math|Float|Clamp(Float) (+ (.Value (Utilities|Map|Find (Variables|Default|GetMonitoredCharacters) _array_element)) (Utilities|Time|GetWorldDeltaSeconds)) 0.0 (Variables|Buoyancy|GetRiseSeconds))))
          (Utilities|Map|Add (Variables|Default|GetMonitoredCharacters) _array_element _output_get)
          (Variables|/Script/Engine.CharacterMovementComponent|SetFallingLateralFriction (Variables|/Script/Engine.Character|GetCharacterMovement _array_element) 1.0)
          (if (and (> (.Z (Math|Vector|BreakVector (- (CallFunction|CalcBuoyPoint (Transformation|GetActorLocation _array_element)) (Transformation|GetActorLocation _array_element)))) (/ (Components|Capsule|GetScaledCapsuleHalfHeight (Variables|/Script/Engine.Character|GetCapsuleComponent _array_element)) 2.0)) (Utilities|Enum|Equal(Enum) (Variables|/Script/Engine.CharacterMovementComponent|GetMovementMode (Variables|/Script/Engine.Character|GetCharacterMovement _array_element)) "MOVE_Walking"))
            (Character|LaunchCharacter _array_element "0, 0,1.000000" false true))
          (Variables|/Script/Engine.MovementComponent|SetVelocity (Variables|/Script/Engine.Character|GetCharacterMovement _array_element) (Math|Vector|Lerp(Vector) (Variables|/Script/Engine.MovementComponent|GetVelocity (Variables|/Script/Engine.Character|GetCharacterMovement _array_element)) (Math|Vector|MakeVector (.X (Math|Vector|BreakVector (Variables|/Script/Engine.MovementComponent|GetVelocity (Variables|/Script/Engine.Character|GetCharacterMovement _array_element)))) (.Y (Math|Vector|BreakVector (Variables|/Script/Engine.MovementComponent|GetVelocity (Variables|/Script/Engine.Character|GetCharacterMovement _array_element)))) (Math|Float|Lerp 1e+02 (* (.Z (Math|Vector|BreakVector (- (CallFunction|CalcBuoyPoint (Transformation|GetActorLocation _array_element)) (Transformation|GetActorLocation _array_element)))) (* (/ (Variables|Default|GetDispStrength) (Variables|Buoyancy|GetDisplacementDivisor)) 2.0)) (/ (LocalVariables|GetCurrSeconds) (Variables|Buoyancy|GetRiseSeconds)))) (/ (LocalVariables|GetCurrSeconds) (Variables|Buoyancy|GetRiseSeconds))))
          (else
            (Utilities|Map|Add (Variables|Default|GetMonitoredCharacters) _array_element 0.0)
            (Variables|/Script/Engine.CharacterMovementComponent|SetFallingLateralFriction (Variables|/Script/Engine.Character|GetCharacterMovement _array_element) (.Value (Utilities|Map|Find (Variables|Default|GetHeldFrictions) (Variables|/Script/Engine.Character|GetCharacterMovement _array_element))))))))))

(fn CalcBuoyPoint
  (params (TargetLoc :type Vector))
  (bind (_x _y) (Math|Vector|BreakVector TargetLoc))
  (bind _returnvalue (Utilities|Time|GetTimeSeconds))
  (bind _dispscale (Variables|Default|GetDispScale))
  (return (Math|Vector|MakeVector _x _y (+ (.z (Transformation|GetWorldLocation (Variables|Default|GetPlane))) (* (- (Class|StaticFuncLib|CalcWaterSurface TargetLoc _dispscale _returnvalue) (Class|StaticFuncLib|CalcWaterSurface "0, 0, 0" _dispscale _returnvalue)) (Variables|Default|GetDispStrength))))))

(fn TickPrimitiveBuoyancy
  (bind _keys (Utilities|Map|Keys (Variables|Default|GetMonitoredPrims)))
  (for _array_element _keys
    (Utilities|IsValid _array_element
      (:Is%20Valid
        (if (> (.Z (Math|Vector|BreakVector (- (CallFunction|CalcBuoyPoint (Transformation|GetWorldLocation _array_element)) (Transformation|GetWorldLocation _array_element)))) -1e+02)
          (bind _output_get (LocalVariables|SetCurrSeconds (Math|Float|Clamp(Float) (+ (.Value (Utilities|Map|Find (Variables|Default|GetMonitoredPrims) _array_element)) (Utilities|Time|GetWorldDeltaSeconds)) 0.0 (Variables|Buoyancy|GetRiseSeconds))))
          (Utilities|Map|Add (Variables|Default|GetMonitoredPrims) _array_element _output_get)
          (Class|PrimitiveComponent|SetLinearDamping _array_element 1.0)
          (bind _returnvalue (Physics|GetPhysicsLinearVelocity _array_element "None"))
          (Class|PrimitiveComponent|SetAllPhysicsLinearVelocity _array_element (Math|Vector|Lerp(Vector) _returnvalue (Math|Vector|MakeVector (.X (Math|Vector|BreakVector _returnvalue)) (.Y (Math|Vector|BreakVector _returnvalue)) (Math|Float|Lerp 1e+02 (* (.Z (Math|Vector|BreakVector (- (CallFunction|CalcBuoyPoint (Transformation|GetWorldLocation _array_element)) (Transformation|GetWorldLocation _array_element)))) (* (/ (Variables|Default|GetDispStrength) (Variables|Buoyancy|GetDisplacementDivisor)) 2.0)) (/ (LocalVariables|GetCurrSeconds) (Variables|Buoyancy|GetRiseSeconds)))) (/ (LocalVariables|GetCurrSeconds) (Variables|Buoyancy|GetRiseSeconds))) false)
          (else
            (Utilities|Map|Add (Variables|Default|GetMonitoredPrims) _array_element 0.0)
            (Class|PrimitiveComponent|SetLinearDamping _array_element (.Value (Utilities|Map|Find (Variables|Default|GetHeldFrictions) _array_element)))))))))

(fn SafeRemove
  (params (Actor :type Actor%20Object%20Reference))
  (bind _returnvalue (Actor|GetComponentbyClass Actor "/Script/Engine.PrimitiveComponent"))
  (bind _ascharacter (Utilities|Casting|CastToCharacter Actor)
    (:then
      (if (.ReturnValue (Utilities|Map|Find (Variables|Default|GetMonitoredCharacters) _ascharacter))
        (bind _keys (Utilities|Map|Keys (Variables|Default|GetMonitoredCharacters)))
        (bind _output_get (LocalVariables|SetCharKeys _keys))
        (bind _values (Utilities|Map|Values (Variables|Default|GetMonitoredCharacters)))
        (bind _output_get_2 (LocalVariables|SetCharValues _values))
        (Utilities|Array|RemoveIndex _output_get_2 (Utilities|Array|FindItem _output_get _ascharacter))
        (Utilities|Array|RemoveIndex (LocalVariables|GetCharKeys) (Utilities|Array|FindItem _output_get _ascharacter))
        (Utilities|Map|Clear (Variables|Default|GetMonitoredCharacters))
        (for (_array_element _array_index) (LocalVariables|GetCharKeys)
          (Utilities|Map|Add (Variables|Default|GetMonitoredCharacters) _array_element (Utilities|Array|Get(acopy) (LocalVariables|GetCharValues) _array_index)))
        (Variables|/Script/Engine.CharacterMovementComponent|SetFallingLateralFriction (Variables|/Script/Engine.Character|GetCharacterMovement _ascharacter) (.Value (Utilities|Map|Find (Variables|Default|GetHeldFrictions) (Variables|/Script/Engine.Character|GetCharacterMovement _ascharacter))))))
    (:CastFailed
      (Utilities|IsValid _returnvalue
        (:Is%20Valid
          (if (.ReturnValue (Utilities|Map|Find (Variables|Default|GetMonitoredPrims) _returnvalue))
            (bind _keys_2 (Utilities|Map|Keys (Variables|Default|GetMonitoredPrims)))
            (bind _output_get_3 (LocalVariables|SetPrimKeys _keys_2))
            (bind _values_2 (Utilities|Map|Values (Variables|Default|GetMonitoredPrims)))
            (bind _output_get_4 (LocalVariables|SetCharValues _values_2))
            (Utilities|Array|RemoveIndex _output_get_4 (Utilities|Array|FindItem _output_get_3 _returnvalue))
            (Utilities|Array|RemoveIndex (LocalVariables|GetPrimKeys) (Utilities|Array|FindItem _output_get_3 _returnvalue))
            (Utilities|Map|Clear (Variables|Default|GetMonitoredPrims))
            (for (_array_element_2 _array_index_2) (LocalVariables|GetPrimKeys)
              (Utilities|Map|Add (Variables|Default|GetMonitoredPrims) _array_element_2 (Utilities|Array|Get(acopy) (LocalVariables|GetCharValues) _array_index_2)))
            (Class|PrimitiveComponent|SetLinearDamping _returnvalue (.Value (Utilities|Map|Find (Variables|Default|GetHeldFrictions) _returnvalue)))))))))