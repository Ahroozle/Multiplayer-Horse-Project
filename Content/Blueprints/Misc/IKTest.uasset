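; Test actor for inverse kinematics on a chain of scene components.
; BeginPlay points IKRoot at Targ, which Tick moves to the observer body of the relevant camera while drawing debug spheres on each segment.
; A hand-written follow-the-leader solver, DoIK, drags segments from the tip and optionally re-anchors the chain.
; Its mouse-driven call, segment-length setup and other debug drawing are disconnected.
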(event EventBeginPlay
  (Variables|/Script/MPHorso.MPHorsoIKRoot|SetTarget (Variables|Default|GetIK_Root) (Variables|Default|GetTarg))
  (bind _output_get (Variables|Default|SetSegs (Utilities|Array|MakeArray (Variables|Default|GetIK_Root) (Variables|Default|GetScene1) (Variables|Default|GetScene2) (Variables|Default|GetScene3) (Variables|Default|GetScene4) (Variables|Default|GetScene5)))))

(event EventTick
  (params (DeltaSeconds :type Float%20%28single-precision%29))
  (bind _segs (Variables|Default|GetSegs))
  (Transformation|SetWorldLocation (Variables|Default|GetTarg) (Transformation|GetActorLocation (Variables|/Game/Blueprints/ObserverBP.ObserverBP_C|GetBody (.AsObserver%20BP (Utilities|Casting|CastToObserverBP (Components|GetOwner (Class|MPHorsoGameInstance|GetRelevantCamera (Class|StaticFuncLib|RetrieveGameInstance))))))) false false)
  (for _index (range 0 (- (Utilities|Array|Length _segs) 1))
    (Rendering|Debug|DrawDebugSphere (Transformation|GetWorldLocation (Utilities|Array|Get(acopy) _segs _index)) 1.0 4 "(R=1.000000,G=0.000000,B=0.000000,A=1.000000)" 0.0)))

(fn ConstructionScript)

(fn DoIK
  (params (Targ :type Vector))
  (bind _segs (Variables|Default|GetSegs))
  (LocalVariables|SetCurrTarg Targ)
  (bind (_arrayindex _arrayelement) (Utilities|Array|ReverseforEachLoop (Variables|Default|GetSegLens))
    (:LoopBody
      (bind _nexttarg (CallFunction|Follow (LocalVariables|GetCurrTarg) _arrayelement (Utilities|Array|Get(acopy) _segs (+ _arrayindex 1)) (Utilities|Array|Get(acopy) _segs _arrayindex)))
      (LocalVariables|SetCurrTarg _nexttarg))
    (:Completed
      (if (Variables|Default|GetAnchored)
        (LocalVariables|SetCurrTarg (- (Variables|Default|GetStartPos) (Transformation|GetWorldLocation (Utilities|Array|Get(acopy) (Variables|Default|GetSegs))))) ; Now used for storing the offset for all scenecomps
        (for _array_element (Variables|Default|GetSegs)
          (Transformation|SetWorldLocation _array_element (+ (Transformation|GetWorldLocation _array_element) (LocalVariables|GetCurrTarg)) false false))))))

(fn Follow
  (params (Target :type Vector) (Length :type Float%20%28single-precision%29) (End :type Scene%20Component%20Object%20Reference) (Start :type Scene%20Component%20Object%20Reference))
  (Transformation|SetWorldLocation End Target false false)
  (bind _output_get (LocalVariables|Setvec (+ (* (Math|Vector|Normalize (- (Transformation|GetWorldLocation Start) Target)) Length) Target)))
  (Transformation|SetWorldLocation Start _output_get false false)
  (return _output_get))