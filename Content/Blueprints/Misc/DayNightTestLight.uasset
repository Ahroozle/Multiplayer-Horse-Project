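; Test directional light actor that animates a day-night cycle from game time sped up tenfold.
; Tick converts that time to a 24-hour value and samples two color curves.
; BehaviorCurve's red channel sets rotation around an axis computed at BeginPlay and its blue channel sets intensity, while LightColorCurve sets color.
; Tick also fetches all PostProcessVolumes but leaves the result unused.
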(event EventBeginPlay
  (Variables|Default|SetRotAxis (Math|Vector|RotateVectorAroundAxis (Transformation|GetActorForwardVector) 9e+01 (Transformation|GetActorUpVector))))

(event EventTick
  (params (DeltaSeconds :type Float%20%28single-precision%29))
  (bind _returnvalue (Utilities|Time|GetTimeSeconds))
  (bind _behaviorcurve (Variables|Default|GetBehaviorCurve))
  (bind _directionallight (Variables|Default|GetDirectionalLight))
  (bind _returnvalue_2 (* _returnvalue 1e+01))
  (bind _returnvalue_3 (Class|NPCDateFuncLib|GetEqMinfromRLSecs _returnvalue_2))
  (bind _returnvalue_4 (/ _returnvalue_3 6e+01))
  (bind _returnvalue_5 (Math|Float|%(Float) _returnvalue_4 24.0))
  (bind _returnvalue_6 (Math|Curves|GetLinearColorValue _behaviorcurve _returnvalue_5))
  (Transformation|SetActorRotation (Math|Vector|RotatorfromAxisandAngle (Variables|Default|GetRotAxis) (* (.r _returnvalue_6) 1.8e+02)))
  (Rendering|Components|Light|SetLightColor _directionallight (Math|Curves|GetLinearColorValue (Variables|Default|GetLightColorCurve) _returnvalue_5) true)
  (Rendering|Components|Light|SetIntensity _directionallight (* (.b _returnvalue_6) 3.0))
  (bind _outactors (Actor|GetAllActorsOfClass "/Script/Engine.PostProcessVolume")))

(fn ConstructionScript)