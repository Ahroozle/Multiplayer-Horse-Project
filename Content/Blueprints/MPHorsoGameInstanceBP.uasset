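; Game instance for MPHorso that runs host-side join screening and moderation, and returns to MainMenu on network errors.
; When hosting, it loads IP access and moderator lists from files, then spawns a UDP receiver and sender to answer join requests with whitelist/blacklist and password checks.
; Kick, ban and op functions act by IP or player and update those files.
; Server and volume settings persist through a GeneralSettingsSaveGame slot.
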(event Custom|OnReceiverInitSucceed
  (bind _returnvalue (Game|SpawnActorfromClass "/Script/MPHorso.MPHorsoUDPSender" (Math|Transform|MakeTransform "0, 0, 0" "0, 0, 0" "1,1,1") "Undefined" 0 0))
  (bind _output_get (Variables|Default|SetSender _returnvalue))
  (EventDispatchers|AssignSocketInitFailedDelegate _output_get (delegate Custom|OnSenderInitFail))
  (EventDispatchers|AssignSocketInitSucceededDelegate _output_get (delegate Custom|OnSenderInitSucceed))
  (Class|MPHorsoUDPSender|InitializeSender (Variables|Default|GetSender) "MPHorso_ServerSender" "127.0.0.1" (Class|MPHorsoNetLibrary|GetDefaultPort)))

(event Custom|OnDataReceived
  (params (ReceivedData :type Horse%20Net%20Data%20Structure%20%28by%20ref%29) (FromIP :type String))
  (bind (_datatype _data) (Utilities|Struct|BreakHorseNetData ReceivedData))
  (if (CallFunction|IPAuthorized FromIP)
    (switch Utilities|FlowControl|Switch|SwitchonEHorseDataType _datatype
      (:HorseData_RawData
        (Development|PrintString (Utilities|String|Append "Unexpected data <" (Utilities|String|EnumtoString _datatype) " | \"" (Class|MPHorsoNetLibrary|StringfromBytes _data) "\"> encountered. Nothing will be done.") :!label _label))
      (:HorseData_JoinRequest
        (if (> (Utilities|String|Len (Variables|Default|GetPassword)) 0)
          (Class|MPHorsoUDPSender|SendDatato (Variables|Default|GetSender) (Utilities|Struct|MakeHorseNetData "HorseData_PassRequest" (Class|MPHorsoNetLibrary|StringtoBytes "Requesting Password")) FromIP)
          (else
            (Class|MPHorsoUDPSender|SendDatato (Variables|Default|GetSender) (Utilities|Struct|MakeHorseNetData "HorseData_ConnectionAccepted" (Class|MPHorsoNetLibrary|StringtoBytes "Join Accepted")) FromIP))))
      (:HorseData_PassRequest
        (goto _label))
      (:HorseData_PassData
        (if (Utilities|Enum|Equal(Enum) (Class|MPHorsoNetLibrary|StringfromBytes _data) (Variables|Default|GetPassword))
          (Class|MPHorsoUDPSender|SendDatato (Variables|Default|GetSender) (Utilities|Struct|MakeHorseNetData "HorseData_ConnectionAccepted" (Class|MPHorsoNetLibrary|StringtoBytes "Join Accepted")) FromIP)
          (else
            (Class|MPHorsoUDPSender|SendDatato (Variables|Default|GetSender) (Utilities|Struct|MakeHorseNetData "HorseData_ConnectionRejected" (Class|MPHorsoNetLibrary|StringtoBytes "Incorrect Password.")) FromIP))))
      (:HorseData_ConnectionRejected
        (goto _label))
      (:HorseData_ConnectionAccepted
        (goto _label)))
    (else
      (Class|MPHorsoUDPSender|SendDatato (Variables|Default|GetSender) (Utilities|Struct|MakeHorseNetData "HorseData_ConnectionRejected" (Class|MPHorsoNetLibrary|StringtoBytes (Utilities|String|SelectString "You are banned." "You aren't on the whitelist." (Utilities|Enum|Equal(Enum) (Variables|Default|GetAccessControlType) "AC_Blacklist")))) FromIP))))

(event Custom|OnSenderInitFail
  (params (ErrorString :type String))
  ;[1 1 1] TODO HOW TO HANDLE?
)

(event Custom|OnSenderInitSucceed
  (EventDispatchers|AssignDataReceivedDelegate (Variables|Default|GetReceiver) (delegate Custom|OnDataReceived)))

(event Custom|SetUpComms
  (bind _returnvalue (Game|SpawnActorfromClass "/Script/MPHorso.MPHorsoUDPReceiver" (Math|Transform|MakeTransform "0, 0, 0" "0, 0, 0" "1,1,1") "Undefined" 0 0))
  (bind _output_get (Variables|Default|SetReceiver _returnvalue))
  (EventDispatchers|AssignSocketInitFailedDelegate _output_get (delegate Custom|OnReceiverInitFail))
  (EventDispatchers|AssignSocketInitSucceededDelegate _output_get (delegate Custom|OnReceiverInitSucceed))
  (Class|MPHorsoUDPReceiver|InitializeReceiver _output_get "MPHorso_ServerReceiver" "127.0.0.1" (Variables|Default|GetServerPort)))

(event Custom|AskForOp
  (params (Asker :type Observer%20BP%20Object%20Reference))
  (if (not (Variables|/Game/Blueprints/ObserverBP.ObserverBP_C|GetIsOp Asker))
    (if (Utilities|Array|ContainsItem (Variables|Default|GetModList) (Utilities|TrimPort (Class|MPHorsoNetLibrary|GetPlayerIP (.AsPlayer%20Controller (Utilities|Casting|CastToPlayerController (Pawn|GetController Asker))))))
      (Variables|/Game/Blueprints/ObserverBP.ObserverBP_C|SetIsOp Asker true))))

(event Custom|OnReceiverInitFail
  (params (ErrorString :type String))
  ;[1 1 1] TODO HOW TO HANDLE?
)

(event EventBanIP
  (params (IP :type String))
  (bind _outip (Utilities|TrimPort IP))
  (bind _aclist (Variables|Default|GetACList))
  (switch Utilities|FlowControl|Switch|SwitchonEAccessControlType (Variables|Default|GetAccessControlType)
    (:AC_None
      _)
    (:AC_Blacklist
      (Utilities|Array|AddUnique _aclist _outip)
      (CallFunction|UpdateACFile :!label _label))
    (:AC_Whitelist
      (Utilities|Array|RemoveItem _aclist _outip)
      (goto _label)))
  (CallFunction|PerformKick IP "\"You Have Been Banned.\""))

(event EventReadyforPlay
  (|CallParentFunction)
  (if (Variables|Default|GetIsHosting)
    (Variables|/Game/Blueprints/ObserverBP.ObserverBP_C|SetIsOp (.AsObserver%20BP (Utilities|Casting|CastToObserverBP (Pawn|GetControlledPawn (Game|GetPlayerController 0)))) true)
    (CallFunction|PopLists)
    (CallFunction|SetUpComms)))

(event EventUnbanIP
  (params (IP :type String))
  (bind _outip (Utilities|TrimPort IP))
  (bind _aclist (Variables|Default|GetACList))
  (switch Utilities|FlowControl|Switch|SwitchonEAccessControlType (Variables|Default|GetAccessControlType)
    (:AC_Blacklist
      (Utilities|Array|RemoveItem _aclist _outip))
    (:AC_Whitelist
      (Utilities|Array|AddUnique _aclist _outip)))
  (CallFunction|UpdateACFile))

(event EventOpIP
  (params (IP :type String))
  (Utilities|Array|AddUnique (Variables|Default|GetModList) (Utilities|TrimPort IP))
  (CallFunction|UpdateModFile))

(event EventKickPlayer
  (params (Player :type Player%20Controller%20Object%20Reference))
  (bind _asmphorso_player_controller_bp (Utilities|Casting|CastToMPHorsoPlayerControllerBP Player))
  (Default|KickSelf _asmphorso_player_controller_bp "You Have Been Kicked."))

(event EventUnopIP
  (params (IP :type String))
  (Utilities|Array|RemoveItem (Variables|Default|GetModList) (Utilities|TrimPort IP))
  (CallFunction|UpdateModFile))

(event EventBanPlayer
  (params (Player :type Player%20Controller%20Object%20Reference))
  (bind _returnvalue (Class|MPHorsoNetLibrary|GetPlayerIP Player))
  (bind _aclist (Variables|Default|GetACList))
  (bind _outip (Utilities|TrimPort _returnvalue))
  (switch Utilities|FlowControl|Switch|SwitchonEAccessControlType (Variables|Default|GetAccessControlType)
    (:AC_None
      _)
    (:AC_Blacklist
      (Utilities|Array|AddUnique _aclist _outip)
      (CallFunction|UpdateACFile :!label _label))
    (:AC_Whitelist
      (Utilities|Array|RemoveItem _aclist _outip)
      (goto _label)))
  (bind _asmphorso_player_controller_bp (Utilities|Casting|CastToMPHorsoPlayerControllerBP Player))
  (Default|KickSelf _asmphorso_player_controller_bp "You Have Been Banned."))

(event EventOpPlayer
  (params (Player :type Player%20Controller%20Object%20Reference))
  (Utilities|Array|AddUnique (Variables|Default|GetModList) (Utilities|TrimPort (Class|MPHorsoNetLibrary|GetPlayerIP Player)))
  (CallFunction|UpdateModFile)
  (Variables|/Game/Blueprints/ObserverBP.ObserverBP_C|SetIsOp (.AsObserver%20BP (Utilities|Casting|CastToObserverBP (Pawn|GetControlledPawn Player))) true))

(event EventUnopPlayer
  (params (Player :type Player%20Controller%20Object%20Reference))
  (Utilities|Array|RemoveItem (Variables|Default|GetModList) (Utilities|TrimPort (Class|MPHorsoNetLibrary|GetPlayerIP Player)))
  (CallFunction|UpdateModFile)
  (Variables|/Game/Blueprints/ObserverBP.ObserverBP_C|SetIsOp (.AsObserver%20BP (Utilities|Casting|CastToObserverBP (Pawn|GetControlledPawn Player))) false))

(event EventHandleNetworkError
  (params (FailureType :type ENetworkFailure%20Enum :default "NetDriverAlreadyExists") (bIsServer :type Boolean))
  (Game|OpenLevel(byName) "MainMenu"))

(event EventKickIP
  (params (IP :type String))
  (CallFunction|PerformKick IP "\"You Have Been Kicked.\""))

(fn SaveSettings
  (bind _generalsave (Variables|Default|GetGeneralSave))
  (Variables|Default|GetGeneralSave
    (:then
      _)
    (:else
      (CallFunction|LoadSettings)))
  (Variables|/Game/Blueprints/Misc/GeneralSettingsSaveGame.GeneralSettingsSaveGame_C|SetAccessControlMethod _generalsave (Variables|Default|GetAccessControlType))
  (Variables|/Game/Blueprints/Misc/GeneralSettingsSaveGame.GeneralSettingsSaveGame_C|SetAccessListPath _generalsave (Variables|Default|GetAccessControlListPath))
  (Variables|/Game/Blueprints/Misc/GeneralSettingsSaveGame.GeneralSettingsSaveGame_C|SetServerPort _generalsave (Variables|Default|GetServerPort))
  (Variables|/Game/Blueprints/Misc/GeneralSettingsSaveGame.GeneralSettingsSaveGame_C|SetModListPath _generalsave (Variables|Default|GetModListPath))
  (Variables|/Game/Blueprints/Misc/GeneralSettingsSaveGame.GeneralSettingsSaveGame_C|SetMasterVolume _generalsave (Variables|Default|GetMasterVolume))
  (Variables|/Game/Blueprints/Misc/GeneralSettingsSaveGame.GeneralSettingsSaveGame_C|SetBGMVolume _generalsave (Variables|Default|GetBGMVolume))
  (Variables|/Game/Blueprints/Misc/GeneralSettingsSaveGame.GeneralSettingsSaveGame_C|SetAmbiVolume _generalsave (Variables|Default|GetAmbiVolume))
  (Variables|/Game/Blueprints/Misc/GeneralSettingsSaveGame.GeneralSettingsSaveGame_C|SetSFXVolume _generalsave (Variables|Default|GetSFXVolume))
  (SaveGame|SaveGametoSlot (Variables|Default|GetGeneralSave) (Variables|Default|GetGeneralSaveSlotName)))

(fn LoadSettings
  (bind _returnvalue (SaveGame|LoadGamefromSlot (Variables|Default|GetGeneralSaveSlotName)))
  (Utilities|IsValid _returnvalue
    (:Is%20Valid
      (bind _asgeneral_settings_save_game (Utilities|Casting|CastToGeneralSettingsSaveGame _returnvalue)
        (:then
          (Variables|Default|SetGeneralSave _asgeneral_settings_save_game))
        (:CastFailed
          (bind _returnvalue_2 (SaveGame|CreateSaveGameObject "/Game/Blueprints/Misc/GeneralSettingsSaveGame.GeneralSettingsSaveGame_C" :!label _label))
          (bind _output_get (Variables|Default|SetGeneralSave _returnvalue_2))
          (SaveGame|SaveGametoSlot _output_get (Variables|Default|GetGeneralSaveSlotName)))))
    (:Is%20Not%20Valid
      (goto _label)))
  (Variables|Default|SetServerPort (Variables|/Game/Blueprints/Misc/GeneralSettingsSaveGame.GeneralSettingsSaveGame_C|GetServerPort (Variables|Default|GetGeneralSave)))
  (Variables|Default|SetAccessControlType (Variables|/Game/Blueprints/Misc/GeneralSettingsSaveGame.GeneralSettingsSaveGame_C|GetAccessControlMethod (Variables|Default|GetGeneralSave)))
  (Variables|Default|SetAccessControlListPath (Variables|/Game/Blueprints/Misc/GeneralSettingsSaveGame.GeneralSettingsSaveGame_C|GetAccessListPath (Variables|Default|GetGeneralSave)))
  (Variables|Default|SetModListPath (Variables|/Game/Blueprints/Misc/GeneralSettingsSaveGame.GeneralSettingsSaveGame_C|GetModListPath (Variables|Default|GetGeneralSave)))
  (Variables|Default|SetMasterVolume (Variables|/Game/Blueprints/Misc/GeneralSettingsSaveGame.GeneralSettingsSaveGame_C|GetMasterVolume (Variables|Default|GetGeneralSave)))
  (Variables|Default|SetBGMVolume (Variables|/Game/Blueprints/Misc/GeneralSettingsSaveGame.GeneralSettingsSaveGame_C|GetBGMVolume (Variables|Default|GetGeneralSave)))
  (Variables|Default|SetAmbiVolume (Variables|/Game/Blueprints/Misc/GeneralSettingsSaveGame.GeneralSettingsSaveGame_C|GetAmbiVolume (Variables|Default|GetGeneralSave)))
  (Variables|Default|SetSFXVolume (Variables|/Game/Blueprints/Misc/GeneralSettingsSaveGame.GeneralSettingsSaveGame_C|GetSFXVolume (Variables|Default|GetGeneralSave))))

(fn PopLists
  (Utilities|FlowControl|Sequence
    (:then_0
      (bind (_outstring _returnvalue) (Class|StaticFuncLib|GetStringfromFile (Variables|Default|GetAccessControlListPath)))
      (if _returnvalue
        (Variables|Default|SetACList (Utilities|String|ParseIntoArray _outstring " 
"))))
    (:then_1
      (bind (_outstring_2 _returnvalue_2) (Class|StaticFuncLib|GetStringfromFile (Variables|Default|GetModListPath)))
      (if _returnvalue_2
        (Variables|Default|SetModList (Utilities|String|ParseIntoArray _outstring_2 " 
"))))))

(fn IPAuthorized
  (params (IP :type String))
  (bind (_lefts _rights _returnvalue) (Utilities|String|Split IP ":"))
  (bind _aclist (Variables|Default|GetACList))
  (bind _returnvalue_2 (Utilities|String|SelectString _lefts IP _returnvalue))
  (bind _returnvalue_3 (Utilities|Array|ContainsItem _aclist _returnvalue_2))
  (switch Utilities|FlowControl|Switch|SwitchonEAccessControlType (Variables|Default|GetAccessControlType)
    (:AC_None
      (return true))
    (:AC_Blacklist
      (return (not _returnvalue_3)))
    (:AC_Whitelist
      (return _returnvalue_3))))

(fn PerformKick
  (params (IP :type String) (Message :type String))
  (bind _output_get (LocalVariables|SetFound (Class|MPHorsoNetLibrary|GetPlayerbyIP self IP)))
  (Utilities|IsValid _output_get
    (:Is%20Valid
      (Default|KickSelf (.AsMPHorso%20Player%20Controller%20BP (Utilities|Casting|CastToMPHorsoPlayerControllerBP _output_get)) Message))))

(fn UpdateACFile
  (for _array_element (Variables|Default|GetACList)
    (LocalVariables|SetConstructedString (Utilities|String|Append (LocalVariables|GetConstructedString) _array_element " 
")))
  (Class|StaticFuncLib|SaveStringtoFile (LocalVariables|GetConstructedString) (Variables|Default|GetAccessControlListPath)))

(fn UpdateModFile
  (for _array_element (Variables|Default|GetModList)
    (LocalVariables|SetConstructedString (Utilities|String|Append (LocalVariables|GetConstructedString) _array_element " 
")))
  (Class|StaticFuncLib|SaveStringtoFile (LocalVariables|GetConstructedString) (Variables|Default|GetModListPath)))