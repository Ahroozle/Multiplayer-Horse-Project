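; Barrier spell controller that toggles a sustained, stamina-draining MagicBarrier on a chosen actor.
; If no barrier is sustained, the local player's instance requests a target and relays it to its Paired instance, which casts; otherwise it relays an immediate finish.
; Casting spawns and attaches a barrier with stamina-based HP, color-scheme tint and bounds-derived scale using a hard-coded size.
; Recasting breaks the caster's barriers with overkill damage and stops the drain.
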(event Custom|OnReceiveArg1
  (params (ActorArg :type Actor%20Object%20Reference))
  (EventDispatchers|UnbindEventfromOnReceiveActorArg (delegate Custom|OnReceiveArg1))
  (bind _paired (Variables|Default|GetPaired)
    (:then
      (CallFunction|TransmitArg1 _paired ActorArg (Variables|Default|GetObsRef))
      (Class|MagicUI|Die))
    (:else)))

(event Custom|TransmitMagicOn
  (params (Obs :type Observer%20BP%20Object%20Reference))
  (CallFunction|FinishTransmitMagicon Obs))

(event Custom|FinishTransmitMagicOn
  (params (Obs :type Observer%20BP%20Object%20Reference))
  (CallFunction|SetObs Obs)
  (CallFunction|SetBodyMagic true false))

(event Custom|FinishTransmitFinish
  (params (Obs :type Observer%20BP%20Object%20Reference))
  (CallFunction|CastSpell Obs)
  (Default|CallOnSpellFinished)
  (Class|MagicUI|Die))

(event Custom|TransmitFinish
  (params (Obs :type Observer%20BP%20Object%20Reference))
  (CallFunction|FinishTransmitFinish Obs))

(event Custom|FinishTransmitArg1
  (params (Arg1 :type Actor%20Object%20Reference) (Obs :type Observer%20BP%20Object%20Reference))
  (Variables|Default|SetTarget Arg1)
  (CallFunction|CastSpell Obs)
  (Default|CallOnSpellFinished)
  (Class|MagicUI|Die))

(event Custom|TransmitArg1
  (params (Arg1 :type Actor%20Object%20Reference) (Obs :type Observer%20BP%20Object%20Reference))
  (CallFunction|FinishTransmitArg1 Arg1 Obs))

(event Custom|ServerDie
  (CallFunction|MulticastServerDie))

(event Custom|MulticastServerDie
  (|CallParentFunction))

(event EventInit
  (|CallParentFunction)
  (bind _bodyref (Variables|Default|GetBodyRef)
    (:then
      (if (Default|SustainedSpellsContains _bodyref "Barrier")
        (bind _paired (Variables|Default|GetPaired)
          (:then
            (CallFunction|TransmitFinish _paired (Variables|Default|GetObsRef))
            (Class|MagicUI|Die))
          (:else))
        (else
          (if (== (Game|GetPlayerController 0) (Components|GetOwner))
            (EventDispatchers|AssignOnReceiveActorArg (delegate Custom|OnReceiveArg1))
            (Class|MagicUI|RequestArg "Actor"))
          (bind _paired_2 (Variables|Default|GetPaired)
            (:then
              (CallFunction|TransmitMagicon _paired_2 (Variables|Default|GetObsRef)))
            (:else)))))
    (:else)))

(event EventCancelSpell
  (Class|MagicUI|Die)
  (bind _paired (Variables|Default|GetPaired)
    (:then
      (CallFunction|ServerDie _paired))
    (:else)))

(fn ConstructionScript
  (|CallParentFunction))

(fn CastSpell
  (params (Caster :type Actor%20Object%20Reference))
  (bind _asobserver_bp (Utilities|Casting|CastToObserverBP Caster)
    (:then
      (bind _output_get (Variables|Default|SetObsRef _asobserver_bp))
      (bind _body (Variables|/Game/Blueprints/ObserverBP.ObserverBP_C|GetBody _output_get)
        (:then
          (Variables|Default|SetBodyRef _body)
          (if (Default|SustainedSpellsContains _body "Barrier")
            (Default|UpdateSustainedSpells _body "Barrier" false)
            (bind _outactors (Actor|GetAllActorsOfClass "/Game/Blueprints/Misc/MagicBarrier.MagicBarrier_C"))
            (for _array_element _outactors
              (if (== _body (Variables|/Game/Blueprints/Misc/MagicBarrier.MagicBarrier_C|GetOwningBody _array_element))
                (Default|UpdateHP _array_element (+ (Variables|/Game/Blueprints/Misc/BarrierBase.BarrierBase_C|GetCurrentHP _array_element) 1.0) (Transformation|GetActorLocation _body) true)))
            (CallFunction|SetBodyMagic false false)
            (bind _stamwidgref (Variables|/Game/Blueprints/Entities/PlayerEntityTypes/PlayerEntityBaseBP.PlayerEntityBaseBP_C|GetStamWidgRef _body)
              (:then
                (Default|StopContinuousDepletion _stamwidgref "Barrier"))
              (:else
                _))
            (return false)
            (else
              (Default|UpdateSustainedSpells _body "Barrier" true)
              (if (>= (Utilities|Array|FindItem (Variables|/Game/Blueprints/Entities/PlayerEntityTypes/PlayerEntityBaseBP.PlayerEntityBaseBP_C|GetColorSchemeNames _body) "Magic") 0)
                (Variables|Default|SetChosenColor (Utilities|Array|Get(acopy) (Variables|/Game/Blueprints/Entities/PlayerEntityTypes/PlayerEntityBaseBP.PlayerEntityBaseBP_C|GetColorSchemeColors _body) (Utilities|Array|FindItem (Variables|/Game/Blueprints/Entities/PlayerEntityTypes/PlayerEntityBaseBP.PlayerEntityBaseBP_C|GetColorSchemeNames _body) "Magic")))
                (else
                  (Variables|Default|SetChosenColor (CallFunction|GetMaterialColor))))
              (bind _returnvalue (Game|SpawnActorfromClass "/Game/Blueprints/Misc/MagicBarrier.MagicBarrier_C" (Math|Transform|MakeTransform "0, 0, 0" "0, 0, 0" (CallFunction|GetBarrierScale)) "Undefined" _body (Variables|Default|GetChosenColor) (Variables|/Game/Blueprints/Entities/PlayerEntityTypes/PlayerEntityBaseBP.PlayerEntityBaseBP_C|GetStaminaMax _body)))
              (Variables|/Game/Blueprints/Misc/MagicBarrier.MagicBarrier_C|SetOwningBody _returnvalue _body)
              (Variables|/Game/Blueprints/Misc/BarrierBase.BarrierBase_C|SetCurrentHP _returnvalue (Variables|/Game/Blueprints/Entities/PlayerEntityTypes/PlayerEntityBaseBP.PlayerEntityBaseBP_C|GetStaminaCurrent _body))
              (Rendering|Material|SetVectorParameterValue (Variables|/Game/Blueprints/Misc/BarrierBase.BarrierBase_C|GetWireDyn _returnvalue) "BarrierColor" (Variables|Default|GetChosenColor) :!class /Script/Engine.MaterialInstanceDynamic)
              (Transformation|AttachActorToActor _returnvalue (Variables|Default|GetTarget) "None" "SnapToTarget" "KeepRelative" "KeepRelative" false)
              (bind _stamwidgref_2 (Variables|/Game/Blueprints/Entities/PlayerEntityTypes/PlayerEntityBaseBP.PlayerEntityBaseBP_C|GetStamWidgRef _body)
                (:then
                  (Default|DepleteStamina _stamwidgref_2 "Barrier" (Utilities|Struct|MakeStaminaCost (* (Variables|/Game/Blueprints/Entities/PlayerEntityTypes/PlayerEntityBaseBP.PlayerEntityBaseBP_C|GetMagicCostMultiplier _body) (Variables|Default|GetContinuousCost)) true)))
                (:else
                  _))
              (return false))))
        (:else
          _)))
    (:CastFailed
      _))
  (return false))

(fn GetBarrierScale
  (bind _target (Variables|Default|GetTarget)
    (:then
      (return (Math|Conversions|ToVector(Float) (/ (Math|Vector|VectorLength (* (Math|Vector|MakeVector 128.0 128.0 128.0) 2.0)) (Math|Vector|VectorLength (.BoxExtent (Collision|GetActorBounds _target false)))))))
    (:else
      (return "1.000000,1.000000,1.000000"))))

(fn SetPaired
  (params (Paired :type Magic%20UI%20Object%20Reference))
  (bind _asbarrier_magic_ui (Utilities|Casting|CastToBarrierMagicUI Paired)
    (:then
      (Variables|Default|SetPaired _asbarrier_magic_ui))
    (:CastFailed
      _))
  (return false))