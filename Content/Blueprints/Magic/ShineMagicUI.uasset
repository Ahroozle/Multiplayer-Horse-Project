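; Spell UI Blueprint for Shine, a sustained spell that toggles a MagicShine actor on the caster's magic tip.
; On Init it hands the observer to its paired instance and dies; that instance casts, signals completion and dies.
; CastSpell spawns and attaches the effect with continuous stamina drain, or removes both if Shine is already sustained.
; Cancelling kills this instance and cancels the paired one through a server-to-multicast chain.
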(event Custom|FinishTransmitFinish
  (params (Obs :type Observer%20BP%20Object%20Reference))
  (CallFunction|CastSpell Obs)
  (Default|CallOnSpellFinished)
  (Class|MagicUI|Die))

(event Custom|TransmitFinish
  (params (Obs :type Observer%20BP%20Object%20Reference))
  (CallFunction|FinishTransmitFinish Obs))

(event Custom|ServerDie
  (CallFunction|MulticastServerDie))

(event Custom|MulticastServerDie
  (|CallParentFunction))

(event EventInit
  (|CallParentFunction)
  (bind _paired (Variables|Default|GetPaired)
    (:then
      (CallFunction|TransmitFinish _paired (Variables|Default|GetObsRef))
      (Class|MagicUI|Die))
    (:else)))

(event EventCancelSpell
  (Class|MagicUI|Die)
  (bind _paired (Variables|Default|GetPaired)
    (:then
      (CallFunction|ServerDie _paired))
    (:else)))

(fn ConstructionScript
  (|CallParentFunction))

(fn CastSpell
  (params (Caster :type Actor%20Object%20Reference))
  (bind _asobserver_bp (Utilities|Casting|CastToObserverBP Caster)
    (:then
      (bind _output_get (Variables|Default|SetObsRef _asobserver_bp))
      (bind _body (Variables|/Game/Blueprints/ObserverBP.ObserverBP_C|GetBody _output_get)
        (:then
          (Variables|Default|SetBodyRef _body)
          (Utilities|IsValid (Default|GetMagicTip _body)
            (:Is%20Valid
              (if (Default|SustainedSpellsContains _body "Shine")
                (Default|UpdateSustainedSpells _body "Shine" false)
                (for _array_element (Actor|GetAttachedActors _body)
                  (if (Utilities|ClassIsChildOf (Utilities|GetClass _array_element) "/Game/Blueprints/Misc/MagicShine.MagicShine_C")
                    (Actor|DestroyActor _array_element)))
                (CallFunction|SetBodyMagic false false)
                (bind _stamwidgref (Variables|/Game/Blueprints/Entities/PlayerEntityTypes/PlayerEntityBaseBP.PlayerEntityBaseBP_C|GetStamWidgRef _body)
                  (:then
                    (Default|StopContinuousDepletion _stamwidgref "Shine"))
                  (:else
                    _))
                (return false)
                (else
                  (CallFunction|SetBodyMagic true false)
                  (bind _returnvalue (Game|SpawnActorfromClass "/Game/Blueprints/Misc/MagicShine.MagicShine_C" (Math|Transform|MakeTransform "0, 0, 0" "0, 0, 0" "1,1,1") "Undefined" _body (LocalVariables|GetAttenuationRadius) 0))
                  (Transformation|AttachComponentToComponent _returnvalue (Default|GetMagicTip _body) "None" "KeepRelative" "KeepRelative" "KeepRelative" true)
                  (Default|UpdateSustainedSpells _body "Shine" true)
                  (bind _stamwidgref_2 (Variables|/Game/Blueprints/Entities/PlayerEntityTypes/PlayerEntityBaseBP.PlayerEntityBaseBP_C|GetStamWidgRef _body)
                    (:then
                      (Default|DepleteStamina _stamwidgref_2 "Shine" (Utilities|Struct|MakeStaminaCost (* (Variables|/Game/Blueprints/Entities/PlayerEntityTypes/PlayerEntityBaseBP.PlayerEntityBaseBP_C|GetMagicCostMultiplier _body) (LocalVariables|GetContinuousCost)) true)))
                    (:else
                      _))
                  (return false))))
            (:Is%20Not%20Valid
              _)))
        (:else
          _)))
    (:CastFailed
      _))
  (return false))

(fn SetPaired
  (params (Paired :type Magic%20UI%20Object%20Reference))
  (bind _asshine_magic_ui (Utilities|Casting|CastToShineMagicUI Paired)
    (:then
      (Variables|Default|SetPaired _asshine_magic_ui))
    (:CastFailed
      _))
  (return false))