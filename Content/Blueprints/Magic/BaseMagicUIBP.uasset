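; Base spell-targeting UI that gathers actor, location and height arguments from the player's cursor.
; Each request starts a looping timer that moves sprite markers, tinted by the emblem's SpellColor, and checks validity until a left click finalizes it.
; Finalized arguments accumulate, anchoring later actor range checks and height picks.
; It previews stamina cost on the body's widget, charges it on finish, and cancels on right click or stamina-out.
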(event Custom|RequestActorArg
  (Variables|CurrentArgs|SetCurrentActorArg 0)
  (CallFunction|GetNewestActorArgComponents)
  (bind _obsref (Variables|OwnerRefs|GetObsRef)
    (:then
      (Utilities|Time|SetTimerbyFunctionName 0 "TickActorArg" 0.01 true)
      (EventDispatchers|AssignLClickInput _obsref (delegate Custom|FinalizeActorArg))
      (bind _outactors (Actor|GetAllActorswithInterface "/Script/MPHorso.MagicManipulableInterface"))
      (Utilities|Set|AddItems (Variables|Default|GetCurrentValidActorTargets) _outactors)
      (Class|MagicUI|MarkTargets (Variables|Default|GetTargetIndicator) _outactors)
      (CallFunction|ColorMarks (Variables|Default|GetTargetMarkers)))
    (:else)))

(event Custom|FinalizeActorArg
  (if (CallFunction|WithinCurrentStamRange)
    (bind _currentactorarg (Variables|CurrentArgs|GetCurrentActorArg)
      (:then
        (bind _obsref (Variables|OwnerRefs|GetObsRef)
          (:then
            (EventDispatchers|UnbindEventfromLClickInput _obsref (delegate Custom|FinalizeActorArg))
            (CallFunction|PlayArgFinalizedSound)
            (Utilities|Array|Add (Variables|Default|GetPreviousArgs) (Variables|Default|GetNewestArg))
            (Utilities|Time|ClearTimerbyFunctionName 0 "TickActorArg")
            (Class|MagicUI|RegisterMovingArg (Variables|Default|GetNewestArg) _currentactorarg)
            (Default|CallOnReceiveActorArg _currentactorarg)
            (Class|MagicUI|HideMarks))
          (:else)))
      (:else
        (CallFunction|PlayArgRejectedSound :!label _label)))
    (else
      (goto _label))))

(event Custom|FinalizeHeightArg
  (if (CallFunction|WithinCurrentStamRange)
    (bind _obsref (Variables|OwnerRefs|GetObsRef)
      (:then
        (EventDispatchers|UnbindEventfromLClickInput _obsref (delegate Custom|FinalizeHeightArg))
        (CallFunction|PlayArgFinalizedSound)
        (Utilities|Array|Add (Variables|Default|GetPreviousArgs) (Variables|Default|GetNewestArg))
        (Utilities|Time|ClearTimerbyFunctionName 0 "TickHeightArg")
        (Default|CallOnReceiveHeightArg (Variables|CurrentArgs|GetCurrentHeightArg)))
      (:else))
    (else
      (CallFunction|PlayArgRejectedSound))))

(event Custom|FinalizeLocationArg
  (if (Variables|CurrentArgs|GetCurrentLocationValid)
    (bind _obsref (Variables|OwnerRefs|GetObsRef)
      (:then
        (EventDispatchers|UnbindEventfromLClickInput _obsref (delegate Custom|FinalizeLocationArg))
        (CallFunction|PlayArgFinalizedSound)
        (Utilities|Array|Add (Variables|Default|GetPreviousArgs) (Variables|Default|GetNewestArg))
        (Utilities|Time|ClearTimerbyFunctionName 0 "TickLocationArg")
        (Default|CallOnReceiveLocationArg (Variables|CurrentArgs|GetCurrentLocationArg)))
      (:else))
    (else
      (CallFunction|PlayArgRejectedSound))))

(event Custom|PlayArgRejectedSound
  (bind _obsref (Variables|OwnerRefs|GetObsRef)
    (:then
      (Class|StaticFuncLib|PlaySound (Math|Transform|MakeTransform (Transformation|GetActorLocation _obsref) "0, 0, 0" "1,1.000000,1") "/Game/Assets/Sound/SFX/MagicSounds/Magic_InvalidArg_Cue.Magic_InvalidArg_Cue" 1.0))
    (:else)))

(event Custom|PlayArgFinalizedSound
  (bind _obsref (Variables|OwnerRefs|GetObsRef)
    (:then
      (Class|StaticFuncLib|PlaySound (Math|Transform|MakeTransform (Transformation|GetActorLocation _obsref) "0, 0, 0" "1,1,1") "/Game/Assets/Sound/SFX/MagicSounds/Magic_Arg_Cue.Magic_Arg_Cue" (+ 1.0 (* (Math|Conversions|ToFloat(Integer) (Utilities|Array|Length (Variables|Default|GetPreviousArgs))) 0.5))))
    (:else)))

(event Custom|RequestLocationArg
  (CallFunction|GetNewestLocationArgComponents)
  (bind _obsref (Variables|OwnerRefs|GetObsRef)
    (:then
      (Utilities|Time|SetTimerbyFunctionName 0 "TickLocationArg" 0.01 true)
      (EventDispatchers|AssignLClickInput _obsref (delegate Custom|FinalizeLocationArg)))
    (:else)))

(event Custom|CancelSpell
  (bind _obsref (Variables|OwnerRefs|GetObsRef)
    (:then
      (EventDispatchers|UnbindEventfromRClickInput _obsref (delegate Custom|CancelSpell)))
    (:else
      _))
  (Default|CallOnSpellCancelled)
  (CallFunction|SetBodyMagic false true)
  (Class|MagicUI|Die))

(event Custom|RequestHeightArg
  (CallFunction|GetNewestHeightArgComponents)
  (bind _obsref (Variables|OwnerRefs|GetObsRef)
    (:then
      (Utilities|Time|SetTimerbyFunctionName 0 "TickHeightArg" 0.01 true)
      (EventDispatchers|AssignLClickInput _obsref (delegate Custom|FinalizeHeightArg)))
    (:else)))

(event Custom|OnSpellCancelled_Event_0
  (bind _bodyref (Variables|OwnerRefs|GetBodyRef)
    (:then
      (bind _stamwidgref (Variables|/Game/Blueprints/Entities/PlayerEntityTypes/PlayerEntityBaseBP.PlayerEntityBaseBP_C|GetStamWidgRef _bodyref)
        (:then
          (Default|ClearShownCost _stamwidgref))
        (:else)))
    (:else)))

(event Custom|OnSpellFinished_Event_0
  (bind _bodyref (Variables|OwnerRefs|GetBodyRef)
    (:then
      (bind _stamwidgref (Variables|/Game/Blueprints/Entities/PlayerEntityTypes/PlayerEntityBaseBP.PlayerEntityBaseBP_C|GetStamWidgRef _bodyref)
        (:then
          (Default|InflictShownCost _stamwidgref))
        (:else)))
    (:else)))

(event EventInit
  (bind _returnvalue (Components|GetOwner))
  (EventDispatchers|AssignOnSpellCancelled (delegate Custom|OnSpellCancelled_Event_0))
  (EventDispatchers|AssignOnSpellFinished (delegate Custom|OnSpellFinished_Event_0))
  (bind _asplayer_controller (Utilities|Casting|CastToPlayerController _returnvalue)
    (:then
      (bind _asobserver_bp (Utilities|Casting|CastToObserverBP (Pawn|GetControlledPawn _asplayer_controller)))
      (Variables|OwnerRefs|SetObsRef _asobserver_bp))
    (:CastFailed
      (bind _asobserver_bp_2 (Utilities|Casting|CastToObserverBP _returnvalue))
      (Variables|OwnerRefs|SetObsRef _asobserver_bp_2)))
  (EventDispatchers|BindEventtoRClickInput (Variables|OwnerRefs|GetObsRef) (delegate Custom|CancelSpell))
  (bind _output_get (Variables|OwnerRefs|SetBodyRef (Variables|/Game/Blueprints/ObserverBP.ObserverBP_C|GetBody (Variables|OwnerRefs|GetObsRef))))
  (bind _stamwidgref (Variables|/Game/Blueprints/Entities/PlayerEntityTypes/PlayerEntityBaseBP.PlayerEntityBaseBP_C|GetStamWidgRef _output_get)
    (:then
      (EventDispatchers|BindEventtoStamOut _stamwidgref (delegate Custom|CancelSpell))
      (Utilities|Time|SetTimerbyFunctionName 0 "TickStaminaCost" 0.01 true))
    (:else)))

(fn ConstructionScript)

(fn TickStaminaCost
  (bind _bodyref (Variables|OwnerRefs|GetBodyRef)
    (:then
      (bind _stamwidgref (Variables|/Game/Blueprints/Entities/PlayerEntityTypes/PlayerEntityBaseBP.PlayerEntityBaseBP_C|GetStamWidgRef _bodyref)
        (:then
          (Default|ShowCost _stamwidgref (Class|MagicUI|GetCurrentStaminaCost)))
        (:else)))
    (:else)))

(fn TickActorArg
  (bind _returnvalue (Game|GetPlayerController 0))
  (bind _newestarg (Variables|Default|GetNewestArg))
  (bind (_hitresult _returnvalue_2) (Game|Player|GetHitResultUnderCursorbyChannel _returnvalue "TraceTypeQuery1" true))
  (bind (_bblockinghit _binitialoverlap _time _location _impactpoint _normal _impactnormal _physmat _hitactor) (Collision|BreakHitResult _hitresult))
  (if _returnvalue_2
    (if (< (Math|Vector|VectorLength (- (CallFunction|GetReferenceLocation) _impactpoint)) (LocalVariables|GetDistanceThreshold))
      (if (Utilities|Set|Contains (Variables|Default|GetCurrentValidActorTargets) _hitactor)
        (bind _returnvalue_3 (Class|MagicManipulableInterface|IsCurrentlyManipulable(Message) _hitactor (Game|GetPlayerController 0)))
        (if _returnvalue_3
          (Transformation|SetWorldLocation _newestarg (Transformation|GetActorLocation _hitactor) false false)
          (Variables|CurrentArgs|SetCurrentActorArg _hitactor)
          (else
            (Transformation|SetWorldLocation _newestarg _impactpoint false false :!label _label)
            (Variables|CurrentArgs|SetCurrentActorArg 0)))
        (else
          (goto _label)))
      (else
        (goto _label)))
    (else
      (goto _label)))
  (CallFunction|UpdateValidFeedbackActorArg (and (Utilities|IsValid (Variables|CurrentArgs|GetCurrentActorArg)) (CallFunction|WithinCurrentStamRange))))

(fn GetReferenceLocation
  (bind _previousargs (Variables|Default|GetPreviousArgs))
  (if (< (Utilities|Array|Length _previousargs) 1)
    (bind _bodyref (Variables|OwnerRefs|GetBodyRef)
      (:then
        (return (Transformation|GetActorLocation _bodyref)))
      (:else
        (return "0, 0, 0")))
    (else
      (return (Transformation|GetWorldLocation (Utilities|Array|Get(acopy) _previousargs (Utilities|Array|LastIndex _previousargs)))))))

(fn WithinCurrentStamRange
  (bind _bodyref (Variables|OwnerRefs|GetBodyRef)
    (:then
      (return (>= (- (+ (Variables|/Game/Blueprints/Entities/PlayerEntityTypes/PlayerEntityBaseBP.PlayerEntityBaseBP_C|GetStaminaCurrent _bodyref) (Variables|/Game/Blueprints/Entities/PlayerEntityTypes/PlayerEntityBaseBP.PlayerEntityBaseBP_C|GetTempStamina _bodyref)) (Class|MagicUI|GetCurrentStaminaCost)) 0.0)))
    (:else
      (return false))))

(fn UpdateValidFeedbackActorArg
  (params (NewValid :type Boolean))
  (bind _currentactortarg (Variables|CurrentArgs|GetCurrentActorTarg))
  (bind _currentactorarg (Variables|CurrentArgs|GetCurrentActorArg))
  (bind _currentactorpole (Variables|CurrentArgs|GetCurrentActorPole))
  (bind _currentactortarg_2 (Variables|CurrentArgs|GetCurrentActorTarg))
  (bind _currentactorpole_2 (Variables|CurrentArgs|GetCurrentActorPole))
  (bind _returnvalue (Transformation|GetWorldLocation _currentactortarg))
  (bind _boxextent (Collision|GetActorBounds _currentactorarg false))
  (bind _relativescale3d (Variables|/Script/Engine.SceneComponent|GetRelativeScale3D _currentactorpole))
  (bind _returnvalue_2 (- _returnvalue "0, 0,45.000000"))
  (if NewValid
    (Rendering|Components|Sprite|SetSprite _currentactortarg_2 "/Game/Assets/Tex/Magic/Casting/MagicUI_ValidTarget_Sprite.MagicUI_ValidTarget_Sprite")
    (Rendering|SetVisibility _currentactorpole_2 true true)
    (Utilities|FlowControl|Sequence
      (:then_0
        (bind (_groundfound _success) (CallFunction|FindGround (Variables|CurrentArgs|GetCurrentActorTarg)))
        (if _success
          (Transformation|SetWorldLocation (Variables|CurrentArgs|GetCurrentActorBottomRing) (+ _groundfound "0, 0,10.000000") false false)
          (Transformation|SetWorldLocation _currentactorpole (+ (* (- _groundfound _returnvalue_2) 0.5) _returnvalue_2) false false)
          (Transformation|SetRelativeScale3D _currentactorpole (Math|Vector|MakeVector (.x _relativescale3d) (.y _relativescale3d) (/ (Math|Vector|VectorLength (- _groundfound _returnvalue_2)) 13.0)))))
      (:then_1
        (Transformation|SetWorldScale3D (Variables|CurrentArgs|GetCurrentActorBottomRing) (/ (Math|Vector|ClampVectorSize (* _boxextent 0.5) 25.0 (Math|Vector|GetMaxElement _boxextent)) 25.0))))
    (else
      (Rendering|Components|Sprite|SetSprite _currentactortarg_2 "/Game/Assets/Tex/Magic/Casting/MagicUI_InvalidTarget_Sprite.MagicUI_InvalidTarget_Sprite")
      (Rendering|SetVisibility _currentactorpole_2 false true))))

(fn GetNewestActorArgComponents
  (for _array_element (Components|GetChildrenComponents (Variables|Default|GetNewestArg) false)
    (if (Utilities|String|Contains (Utilities|GetObjectName _array_element) (Utilities|GetObjectName (Variables|Default|GetActorTarg)))
      (bind _aspaper_sprite_component (Utilities|Casting|CastToPaperSpriteComponent _array_element))
      (bind _output_get (Variables|CurrentArgs|SetCurrentActorTarg _aspaper_sprite_component))
      (Sprite|SetSpriteColor _output_get (CallFunction|GetMaterialColor))
      (elif (Utilities|String|Contains (Utilities|GetObjectName _array_element) (Utilities|GetObjectName (Variables|Default|GetActorPole)))
        (bind _aspaper_sprite_component_2 (Utilities|Casting|CastToPaperSpriteComponent _array_element))
        (bind _output_get_2 (Variables|CurrentArgs|SetCurrentActorPole _aspaper_sprite_component_2))
        (Sprite|SetSpriteColor _output_get_2 (CallFunction|GetMaterialColor))
        (elif (Utilities|String|Contains (Utilities|GetObjectName _array_element) (Utilities|GetObjectName (Variables|Default|GetActorBottomRing)))
          (bind _output_get_3 (Variables|CurrentArgs|SetCurrentActorBottomRing _array_element))
          (for _array_element_2 (Components|GetChildrenComponents _output_get_3 false)
            (Variables|/Script/Engine.SceneComponent|SetbAbsoluteScale _array_element_2 true)
            (bind _aspaper_sprite_component_3 (Utilities|Casting|CastToPaperSpriteComponent _array_element_2))
            (Sprite|SetSpriteColor _aspaper_sprite_component_3 (CallFunction|GetMaterialColor))))))))

(fn FindGround
  (params (FocusComponent :type Scene%20Component%20Object%20Reference))
  (bind _returnvalue (Transformation|GetWorldLocation FocusComponent))
  (bind (_outhit _returnvalue_2) (Collision|LineTraceForObjects _returnvalue (- _returnvalue "0, 0,10000.000000") (Utilities|Array|MakeArray "ObjectTypeQuery1") false 0 "None"))
  (return (.ImpactPoint (Collision|BreakHitResult _outhit)) _returnvalue_2))

(fn GetNewestLocationArgComponents
  (for _array_element (Components|GetChildrenComponents (Variables|Default|GetNewestArg) true)
    (if (Utilities|String|Contains (Utilities|GetObjectName _array_element) (Utilities|GetObjectName (Variables|Default|GetLocationTarget)))
      (bind _aspaper_sprite_component (Utilities|Casting|CastToPaperSpriteComponent _array_element))
      (bind _output_get (Variables|CurrentArgs|SetCurrentLocationTarget _aspaper_sprite_component))
      (Sprite|SetSpriteColor _output_get (CallFunction|GetMaterialColor))
      (elif (Utilities|String|Contains (Utilities|GetObjectName _array_element) (Utilities|GetObjectName (Variables|Default|GetLocationContact)))
        (bind _aspaper_sprite_component_2 (Utilities|Casting|CastToPaperSpriteComponent _array_element))
        (bind _output_get_2 (Variables|CurrentArgs|SetCurrentLocationContact _aspaper_sprite_component_2))
        (Sprite|SetSpriteColor _output_get_2 (CallFunction|GetMaterialColor))
        (else
          (bind _aspaper_sprite_component_3 (Utilities|Casting|CastToPaperSpriteComponent _array_element))
          (Sprite|SetSpriteColor _aspaper_sprite_component_3 (CallFunction|GetMaterialColor)))))))

(fn TickLocationArg
  (bind _returnvalue (Game|GetPlayerController 0))
  (bind _newestarg (Variables|Default|GetNewestArg))
  (bind (_hitresult _returnvalue_2) (Game|Player|GetHitResultUnderCursorbyChannel _returnvalue "TraceTypeQuery1" true))
  (bind (_bblockinghit _binitialoverlap _time _location _impactpoint _normal _impactnormal) (Collision|BreakHitResult _hitresult))
  (if _returnvalue_2
    (Transformation|SetWorldLocation _newestarg _impactpoint false false)
    (Variables|CurrentArgs|SetCurrentLocationArg _impactpoint)
    (CallFunction|UpdateValidFeedbackLocationArg (and (CallFunction|WithinCurrentStamRange) (>= (Math|Vector|DotProduct _impactnormal "0, 0,1.000000") (LocalVariables|GetNormalThreshold))) _impactnormal)
    (else
      (Transformation|SetWorldLocation _newestarg (CallFunction|GetMousePointonPlayerPlane (Transformation|GetActorLocation (Variables|OwnerRefs|GetObsRef))) false false)
      (CallFunction|UpdateValidFeedbackLocationArg false "0, 0, 0"))))

(fn UpdateValidFeedbackLocationArg
  (params (NewValid :type Boolean) (NormalIfValid :type Vector))
  (bind _currentlocationtarget (Variables|CurrentArgs|GetCurrentLocationTarget))
  (bind _currentlocationcontact (Variables|CurrentArgs|GetCurrentLocationContact))
  (bind _currentlocationcontact_2 (Variables|CurrentArgs|GetCurrentLocationContact))
  (bind _output_get (Variables|CurrentArgs|SetCurrentLocationValid NewValid))
  (if _output_get
    (Rendering|Components|Sprite|SetSprite _currentlocationtarget "/Game/Assets/Tex/Magic/Casting/MagicUI_ValidTarget_Sprite.MagicUI_ValidTarget_Sprite")
    (Rendering|SetVisibility _currentlocationcontact_2 true true)
    (Transformation|SetWorldRotation _currentlocationcontact (Class|KismetMathLibrary|MakeRotfromYX NormalIfValid (Math|Vector|GetForwardVector _currentlocationcontact)) false false)
    (else
      (Rendering|Components|Sprite|SetSprite _currentlocationtarget "/Game/Assets/Tex/Magic/Casting/MagicUI_InvalidTarget_Sprite.MagicUI_InvalidTarget_Sprite")
      (Rendering|SetVisibility _currentlocationcontact_2 false true))))

(fn GetMousePointonPlayerPlane
  (params (PlaneOrigin :type Vector))
  (bind _returnvalue (Game|GetPlayerController 0))
  (bind (_worldlocation _worlddirection) (Game|Player|ConvertMouseLocationToWorldSpace _returnvalue))
  (bind _obsref (Variables|OwnerRefs|GetObsRef)
    (:then
      (if (.ReturnValue (Class|KismetMathLibrary|LinePlaneIntersectionOriginNormal _worldlocation (+ _worldlocation (* _worlddirection 1e+08)) PlaneOrigin (Math|Vector|Normalize (Math|Vector|ProjectVectorontoPlane (Math|Vector|NegateVector (Math|Vector|GetForwardVector (Variables|/Game/Blueprints/ObserverBP.ObserverBP_C|GetCamera _obsref))) "0, 0,1.000000"))))
        (return (.Intersection (Class|KismetMathLibrary|LinePlaneIntersectionOriginNormal _worldlocation (+ _worldlocation (* _worlddirection 1e+08)) PlaneOrigin (Math|Vector|Normalize (Math|Vector|ProjectVectorontoPlane (Math|Vector|NegateVector (Math|Vector|GetForwardVector (Variables|/Game/Blueprints/ObserverBP.ObserverBP_C|GetCamera _obsref))) "0, 0,1.000000")))))
        (else
          (return "0, 0, 0"))))
    (:else
      (return "0, 0, 0"))))

(fn GetNewestHeightArgComponents
  (for _array_element (Components|GetChildrenComponents (Variables|Default|GetNewestArg) false)
    (if (Utilities|String|Contains (Utilities|GetObjectName _array_element) (Utilities|GetObjectName (Variables|Default|GetHeightPole)))
      (bind _aspaper_sprite_component (Utilities|Casting|CastToPaperSpriteComponent _array_element))
      (bind _output_get (Variables|CurrentArgs|SetCurrentHeightPole _aspaper_sprite_component))
      (Sprite|SetSpriteColor _output_get (CallFunction|GetMaterialColor))
      (elif (Utilities|String|Contains (Utilities|GetObjectName _array_element) (Utilities|GetObjectName (Variables|Default|GetHeightFocus)))
        (bind _aspaper_sprite_component_2 (Utilities|Casting|CastToPaperSpriteComponent _array_element))
        (bind _output_get_2 (Variables|CurrentArgs|SetCurrentHeightFocus _aspaper_sprite_component_2))
        (Sprite|SetSpriteColor _output_get_2 (CallFunction|GetMaterialColor))
        (elif (Utilities|String|Contains (Utilities|GetObjectName _array_element) (Utilities|GetObjectName (Variables|Default|GetHeightGroundIntersections)))
          (Variables|CurrentArgs|SetCurrentHeightGroundIntersects _array_element))))))

(fn TickHeightArg
  (bind _returnvalue (Math|Vector|MakeVector 0.0 0.0 45.0))
  (bind _currentheightfocus (Variables|CurrentArgs|GetCurrentHeightFocus))
  (bind _currentheightfocus_2 (Variables|CurrentArgs|GetCurrentHeightFocus))
  (bind _currentlocationarg (Variables|CurrentArgs|GetCurrentLocationArg))
  (bind _currentconstructedintersects (Variables|CurrentArgs|GetCurrentConstructedIntersects))
  (bind _currentheightpole (Variables|CurrentArgs|GetCurrentHeightPole))
  (bind _previousargs (Variables|Default|GetPreviousArgs))
  (bind _previousargs_2 (Variables|Default|GetPreviousArgs))
  (bind _newestarg (Variables|Default|GetNewestArg))
  (bind _returnvalue_2 (Utilities|Array|LastIndex _previousargs_2))
  (bind _returnvalue_3 (Transformation|GetWorldLocation _currentheightfocus))
  (bind _relativescale3d (Variables|/Script/Engine.SceneComponent|GetRelativeScale3D _currentheightpole))
  (bind _item (Utilities|Array|Get(acopy) _previousargs_2 _returnvalue_2))
  (bind _returnvalue_4 (- _returnvalue_3 _returnvalue))
  (bind _returnvalue_5 (- _currentlocationarg _returnvalue_4))
  (bind _returnvalue_6 (Transformation|GetWorldLocation _item))
  (bind _output_get (Variables|CurrentArgs|SetCurrentHeightArg (Math|Vector|MakeVector (.x _returnvalue_6) (.y _returnvalue_6) (.Z (Math|Vector|BreakVector (CallFunction|GetMousePointonPlayerPlane (Transformation|GetWorldLocation _newestarg)))))))
  (Transformation|SetWorldLocation _newestarg _output_get false false)
  (Utilities|FlowControl|Sequence
    (:then_0
      (Transformation|SetWorldLocation _currentheightpole (+ (* _returnvalue_5 0.5) _returnvalue_4) false false)
      (Transformation|SetRelativeScale3D _currentheightpole (Math|Vector|MakeVector (.x _relativescale3d) (.y _relativescale3d) (/ (Math|Vector|VectorLength _returnvalue_5) 13.0))))
    (:then_1
      (bind _currentheightgroundintersects (Variables|CurrentArgs|GetCurrentHeightGroundIntersects)
        (:then
          (bind (_outhits _returnvalue_7) (Class|KismetSystemLibrary|LineTraceMultiforObjects (Transformation|GetWorldLocation (Utilities|Array|Get(acopy) _previousargs (Utilities|Array|LastIndex _previousargs))) (Variables|CurrentArgs|GetCurrentHeightArg) (Utilities|Array|MakeArray "ObjectTypeQuery1") false 0 "None" true))
          (if _returnvalue_7
            (Rendering|SetVisibility _currentheightgroundintersects false true)
            (for (_array_element _array_index) _outhits
              (if (>= _array_index (Utilities|Array|Length _currentconstructedintersects))
                (bind _returnvalue_8 (AddComponent|AddPaperSpriteComponent true (Math|Transform|MakeTransform "0, 0, 0" "0, 0,-90.000000" "5.000000,5.000000,5.000000")))
                (Transformation|AttachComponentToComponent _returnvalue_8 (Variables|CurrentArgs|GetCurrentHeightGroundIntersects) "None" "KeepRelative" "KeepWorld" "KeepWorld" true)
                (Sprite|SetSpriteColor _returnvalue_8 (CallFunction|GetMaterialColor))
                (bind _output_get_2 (LocalVariables|SetCurrentIntersect _returnvalue_8))
                (Utilities|Array|Add (Variables|CurrentArgs|GetCurrentConstructedIntersects) _output_get_2)
                (else
                  (LocalVariables|SetCurrentIntersect (Utilities|Array|Get(acopy) _currentconstructedintersects _array_index))))
              (Rendering|SetVisibility (LocalVariables|GetCurrentIntersect) true false)
              (Transformation|SetWorldLocation (LocalVariables|GetCurrentIntersect) (.ImpactPoint (Collision|BreakHitResult _array_element)) false false))))
        (:else)))
    (:then_2
      (if (CallFunction|WithinCurrentStamRange)
        (Rendering|Components|Sprite|SetSprite _currentheightfocus_2 "/Game/Assets/Tex/Magic/Casting/MagicUI_FilledPoint_Sprite.MagicUI_FilledPoint_Sprite")
        (else
          (Rendering|Components|Sprite|SetSprite _currentheightfocus_2 "/Game/Assets/Tex/Magic/Casting/MagicUI_InvalidTarget_Sprite.MagicUI_InvalidTarget_Sprite"))))))

(fn GetMaterialColor
  (bind _asmaterial_instance (Utilities|Casting|CastToMaterialInstance (Variables|Default|GetSpellEmblem))
    (:then
      (for _array_element (Variables|/Script/Engine.MaterialInstance|GetVectorParameterValues _asmaterial_instance)
        (if (Utilities|Name|Equal(Name) (.ParameterName (Utilities|Struct|BreakVectorParameterValue _array_element)) "SpellColor")
          (return (.ParameterValue (Utilities|Struct|BreakVectorParameterValue _array_element)))))
      (return ""))
    (:CastFailed
      (return ""))))

(fn SetBodyMagic
  (params (On :type Boolean) (Cancelled :type Boolean))
  (bind _obsref (Variables|OwnerRefs|GetObsRef)
    (:then
      (bind _bodyref (Variables|OwnerRefs|GetBodyRef)
        (:then
          (if On
            (bind _returnvalue (Class|StaticFuncLib|PlaySound (Math|Transform|MakeTransform (Transformation|GetActorLocation _bodyref) "0, 0, 0" "1,1,1") "/Game/Assets/Sound/SFX/MagicSounds/MagicCycle_Cue.MagicCycle_Cue" 1.0))
            (Utilities|Map|Add (Variables|/Game/Blueprints/ObserverBP.ObserverBP_C|GetSpellSounds _obsref) (Variables|Default|GetSpellName) _returnvalue)
            (if (!= (Components|GetOwner) (Game|GetPlayerController 0))
              (Audio|Components|Audio|AdjustAttenuation (Variables|/Script/MPHorso.OneShotAudio|GetaudioComp _returnvalue) (LocalVariables|GetAtten)))
            (Audio|Components|Audio|Play (Variables|/Script/MPHorso.OneShotAudio|GetaudioComp _returnvalue) 0.0)
            (Transformation|AttachActorToActor _returnvalue _bodyref "None" "SnapToTarget" "KeepRelative" "KeepRelative" true)
            (Default|TurnMagicon _bodyref)
            (else
              (if Cancelled
                (Utilities|IsValid (.Value (Utilities|Map|Find (Variables|/Game/Blueprints/ObserverBP.ObserverBP_C|GetSpellSounds _obsref) (Variables|Default|GetSpellName)))
                  (:Is%20Valid
                    (Actor|DestroyActor))
                  (:Is%20Not%20Valid
                    _))
                (bind _returnvalue_2 (Class|StaticFuncLib|PlaySound (Math|Transform|MakeTransform (Transformation|GetActorLocation _bodyref) "0, 0, 0" "1,1,1") "/Game/Assets/Sound/SFX/MagicSounds/Magic_Cancel_Cue.Magic_Cancel_Cue" 1.0))
                (if (!= (Components|GetOwner) (Game|GetPlayerController 0))
                  (Audio|Components|Audio|AdjustAttenuation (Variables|/Script/MPHorso.OneShotAudio|GetaudioComp _returnvalue_2) (LocalVariables|GetAtten)))
                (Audio|Components|Audio|Play (Variables|/Script/MPHorso.OneShotAudio|GetaudioComp _returnvalue_2) 0.0)
                (Transformation|AttachActorToActor _returnvalue_2 _bodyref "None" "SnapToTarget" "KeepRelative" "KeepRelative" true)
                (else
                  (Utilities|IsValid (.Value (Utilities|Map|Find (Variables|/Game/Blueprints/ObserverBP.ObserverBP_C|GetSpellSounds _obsref) (Variables|Default|GetSpellName)))
                    (:Is%20Valid
                      (Effects|Components|ParticleSystem|SetBoolParameter (Variables|/Script/MPHorso.OneShotAudio|GetaudioComp (.Value (Utilities|Map|Find (Variables|/Game/Blueprints/ObserverBP.ObserverBP_C|GetSpellSounds _obsref) (Variables|Default|GetSpellName)))) "MagicDone" true))
                    (:Is%20Not%20Valid
                      _))))
              (Utilities|Map|Add (Variables|/Game/Blueprints/ObserverBP.ObserverBP_C|GetSpellSounds _obsref) (Variables|Default|GetSpellName) 0)
              (Default|TurnMagicOff _bodyref))))
        (:else)))
    (:else)))

(fn SetObs
  (params (Obs :type Observer%20BP%20Object%20Reference))
  (bind _output_get (Variables|OwnerRefs|SetObsRef Obs))
  (Utilities|IsValid _output_get
    (:Is%20Valid
      (Variables|OwnerRefs|SetBodyRef (Variables|/Game/Blueprints/ObserverBP.ObserverBP_C|GetBody _output_get)))))

(fn ColorMarks
  (params (MarkRoots :type Array%20of%20Scene%20Component%20Object%20References))
  (for _array_element MarkRoots
    (bind _aspaper_sprite_component (Utilities|Casting|CastToPaperSpriteComponent _array_element)
      (:then
        (Sprite|SetSpriteColor _aspaper_sprite_component (CallFunction|GetMaterialColor)))
      (:CastFailed
        (CallFunction|ColorMarks (Components|GetChildrenComponents _array_element false))))))