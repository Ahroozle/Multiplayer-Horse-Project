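; TelegrabMagicUI is the spell actor that toggles a sustained Telegrab on the caster's body.
; On init, the owning player picks an actor target, or an active Telegrab ends immediately.
; A paired instance receives these results through Transmit events and runs CastSpell.
; CastSpell spawns a colored MagicGrab with continuous stamina drain, ten times higher when self-targeted, or destroys the caster's grabs and stops the drain.
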(event Custom|OnReceiveArg1
  (params (ActorArg :type Actor%20Object%20Reference))
  (EventDispatchers|UnbindEventfromOnReceiveActorArg (delegate Custom|OnReceiveArg1))
  (bind _paired (Variables|Default|GetPaired)
    (:then
      (CallFunction|TransmitArg1 _paired ActorArg (Variables|Default|GetObsRef))
      (Class|MagicUI|Die))
    (:else)))

(event Custom|TransmitMagicOn
  (params (Obs :type Observer%20BP%20Object%20Reference))
  (CallFunction|FinishTransmitMagicon Obs))

(event Custom|FinishTransmitMagicOn
  (params (Obs :type Observer%20BP%20Object%20Reference))
  (CallFunction|SetObs Obs)
  (CallFunction|SetBodyMagic true false))

(event Custom|FinishTransmitFinish
  (params (Obs :type Observer%20BP%20Object%20Reference))
  (CallFunction|CastSpell Obs)
  (Default|CallOnSpellFinished)
  (Class|MagicUI|Die))

(event Custom|TransmitFinish
  (params (Obs :type Observer%20BP%20Object%20Reference))
  (CallFunction|FinishTransmitFinish Obs))

(event Custom|FinishTransmitArg1
  (params (Arg1 :type Actor%20Object%20Reference) (Obs :type Observer%20BP%20Object%20Reference))
  (Variables|Default|SetTarget Arg1)
  (CallFunction|CastSpell Obs)
  (Default|CallOnSpellFinished)
  (Class|MagicUI|Die))

(event Custom|TransmitArg1
  (params (Arg1 :type Actor%20Object%20Reference) (Obs :type Observer%20BP%20Object%20Reference))
  (CallFunction|FinishTransmitArg1 Arg1 Obs))

(event Custom|ServerDie
  (CallFunction|MulticastServerDie))

(event Custom|MulticastServerDie
  (|CallParentFunction))

(event EventInit
  (|CallParentFunction)
  (bind _bodyref (Variables|Default|GetBodyRef)
    (:then
      (if (Default|SustainedSpellsContains _bodyref "Telegrab")
        (bind _paired (Variables|Default|GetPaired)
          (:then
            (CallFunction|TransmitFinish _paired (Variables|Default|GetObsRef))
            (Class|MagicUI|Die))
          (:else))
        (else
          (if (== (Game|GetPlayerController 0) (Components|GetOwner))
            (EventDispatchers|AssignOnReceiveActorArg (delegate Custom|OnReceiveArg1))
            (Class|MagicUI|RequestArg "Actor"))
          (bind _paired_2 (Variables|Default|GetPaired)
            (:then
              (CallFunction|TransmitMagicon _paired_2 (Variables|Default|GetObsRef)))
            (:else)))))
    (:else)))

(event EventCancelSpell
  (Class|MagicUI|Die)
  (bind _paired (Variables|Default|GetPaired)
    (:then
      (CallFunction|ServerDie _paired))
    (:else)))

(fn ConstructionScript
  (|CallParentFunction))

(fn SetPaired
  (params (Paired :type Magic%20UI%20Object%20Reference))
  (bind _astelegrab_magic_ui (Utilities|Casting|CastToTelegrabMagicUI Paired)
    (:then
      (Variables|Default|SetPaired _astelegrab_magic_ui))
    (:CastFailed
      _))
  (return false))

(fn CastSpell
  (params (Caster :type Actor%20Object%20Reference))
  (bind _target (Variables|Default|GetTarget))
  (bind _asobserver_bp (Utilities|Casting|CastToObserverBP Caster)
    (:then
      (bind _output_get (Variables|Default|SetObsRef _asobserver_bp))
      (bind _body (Variables|/Game/Blueprints/ObserverBP.ObserverBP_C|GetBody _output_get)
        (:then
          (Variables|Default|SetBodyRef _body)
          (if (Default|SustainedSpellsContains _body "Telegrab")
            (Default|UpdateSustainedSpells _body "Telegrab" false)
            (bind _outactors (Actor|GetAllActorsOfClass "/Game/Blueprints/Misc/MagicGrab.MagicGrab_C"))
            (for _array_element _outactors
              (if (== _body (Components|GetOwner _array_element))
                (Default|Die _array_element)))
            (CallFunction|SetBodyMagic false false)
            (bind _stamwidgref (Variables|/Game/Blueprints/Entities/PlayerEntityTypes/PlayerEntityBaseBP.PlayerEntityBaseBP_C|GetStamWidgRef _body)
              (:then
                (Default|StopContinuousDepletion _stamwidgref "Telegrab"))
              (:else
                _))
            (return false)
            (else
              (Default|UpdateSustainedSpells _body "Telegrab" true)
              (if (>= (Utilities|Array|FindItem (Variables|/Game/Blueprints/Entities/PlayerEntityTypes/PlayerEntityBaseBP.PlayerEntityBaseBP_C|GetColorSchemeNames _body) "Magic") 0)
                (Variables|Default|SetChosenColor (Utilities|Array|Get(acopy) (Variables|/Game/Blueprints/Entities/PlayerEntityTypes/PlayerEntityBaseBP.PlayerEntityBaseBP_C|GetColorSchemeColors _body) (Utilities|Array|FindItem (Variables|/Game/Blueprints/Entities/PlayerEntityTypes/PlayerEntityBaseBP.PlayerEntityBaseBP_C|GetColorSchemeNames _body) "Magic")))
                (else
                  (Variables|Default|SetChosenColor (CallFunction|GetMaterialColor))))
              (Game|SpawnActorfromClass "/Game/Blueprints/Misc/MagicGrab.MagicGrab_C" (Math|Transform|MakeTransform (Transformation|GetActorLocation _target) "0, 0, 0" "1,1,1") "Undefined" _body _target (Variables|Default|GetChosenColor))
              (bind _stamwidgref_2 (Variables|/Game/Blueprints/Entities/PlayerEntityTypes/PlayerEntityBaseBP.PlayerEntityBaseBP_C|GetStamWidgRef _body)
                (:then
                  (Default|DepleteStamina _stamwidgref_2 "Telegrab" (Utilities|Struct|MakeStaminaCost (* (Variables|/Game/Blueprints/Entities/PlayerEntityTypes/PlayerEntityBaseBP.PlayerEntityBaseBP_C|GetMagicCostMultiplier _body) (* (Variables|Default|GetContinuousCost) (Math|Float|SelectFloat 1e+01 1.0 (== _body _target)))) true)))
                (:else
                  _))
              (return false))))
        (:else
          _)))
    (:CastFailed
      _))
  (return false))