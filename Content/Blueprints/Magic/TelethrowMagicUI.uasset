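; Spell UI for Telethrow, a magic that hurls a chosen actor toward a chosen location.
; The owning player picks actor, location and height in sequence, while a Bezier arrow previews throw power by flattening and thickening.
; Each choice is relayed to a Paired instance, which casts with distance-based stamina cost and colored teleport particles.
; Higher power means a faster, flatter velocity launch, with separate handling for characters, ChangelingRoombas and physics bodies.
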(event Custom|OnReceiveArg1
  (params (ActorArg :type Actor%20Object%20Reference))
  (EventDispatchers|UnbindEventfromOnReceiveActorArg (delegate Custom|OnReceiveArg1))
  (Variables|Default|SetTarget ActorArg)
  (bind _paired (Variables|Default|GetPaired)
    (:then
      (CallFunction|TransmitArg1 _paired ActorArg))
    (:else
      _))
  (EventDispatchers|BindEventtoOnReceiveLocationArg (delegate Custom|OnReceiveArg2))
  (Class|MagicUI|RequestArg "Location_Any")
  (CallFunction|MakeHelperArrow))

(event Custom|TransmitMagicOn
  (params (Obs :type Observer%20BP%20Object%20Reference))
  (CallFunction|FinishTransmitMagicon Obs))

(event Custom|FinishTransmitMagicOn
  (params (Obs :type Observer%20BP%20Object%20Reference))
  (CallFunction|SetObs Obs)
  (CallFunction|SetBodyMagic true false))

(event Custom|OnReceiveArg2
  (params (LocationArg :type Vector))
  (EventDispatchers|UnbindEventfromOnReceiveLocationArg (delegate Custom|OnReceiveArg2))
  (Variables|Default|SetTowardLoc LocationArg)
  (bind _paired (Variables|Default|GetPaired)
    (:then
      (CallFunction|TransmitArg2 _paired LocationArg))
    (:else
      _))
  (EventDispatchers|BindEventtoOnReceiveHeightArg (delegate Custom|OnReceiveArg3))
  (Class|MagicUI|RequestArg "Height")
  (Utilities|Time|SetTimerbyFunctionName 0 "ResizeArrow" 0.01 true))

(event Custom|FinishTransmitArg3
  (params (Arg3 :type Float%20%28single-precision%29) (Obs :type Observer%20BP%20Object%20Reference) (StamCost :type Float%20%28single-precision%29))
  (Variables|Default|SetThrowPower Arg3)
  (bind _bodyref (Variables|Default|GetBodyRef)
    (:then
      (bind _stamwidgref (Variables|/Game/Blueprints/Entities/PlayerEntityTypes/PlayerEntityBaseBP.PlayerEntityBaseBP_C|GetStamWidgRef _bodyref)
        (:then
          (Default|ShowCost _stamwidgref StamCost))
        (:else
          _)))
    (:else
      _))
  (CallFunction|CastSpell Obs)
  (Default|CallOnSpellFinished)
  (CallFunction|SetBodyMagic false false)
  (Class|MagicUI|Die))

(event Custom|FinishTransmitArg1
  (params (Arg1 :type Actor%20Object%20Reference))
  (Variables|Default|SetTarget Arg1))

(event Custom|FinishTransmitArg2
  (params (Arg2 :type Vector))
  (Variables|Default|SetTowardLoc Arg2))

(event Custom|TransmitArg1
  (params (Arg1 :type Actor%20Object%20Reference))
  (CallFunction|FinishTransmitArg1 Arg1))

(event Custom|OnReceiveArg3
  (params (HeightArg :type Vector))
  (EventDispatchers|UnbindEventfromOnReceiveHeightArg (delegate Custom|OnReceiveArg3))
  (bind _paired (Variables|Default|GetPaired)
    (:then
      (CallFunction|TransmitArg3 _paired (Variables|Default|GetThrowPower) (Variables|Default|GetObsRef) (CallFunction|GetCurrentStaminaCost)))
    (:else
      _))
  (bind _bezarrow (Variables|Default|GetBezArrow)
    (:then
      (Actor|DestroyActor _bezarrow)
      (Class|MagicUI|Die))
    (:else)))

(event Custom|TransmitArg3
  (params (Arg3 :type Float%20%28single-precision%29) (Obs :type Observer%20BP%20Object%20Reference) (StamCost :type Float%20%28single-precision%29))
  (CallFunction|FinishTransmitArg3 Arg3 Obs StamCost))

(event Custom|TransmitArg2
  (params (Arg2 :type Vector))
  (CallFunction|FinishTransmitArg2 Arg2))

(event Custom|ServerDie
  (CallFunction|MulticastServerDie))

(event Custom|MulticastServerDie
  (|CallParentFunction))

(event EventInit
  (|CallParentFunction)
  (if (== (Game|GetPlayerController 0) (Components|GetOwner))
    (EventDispatchers|AssignOnReceiveActorArg (delegate Custom|OnReceiveArg1))
    (Class|MagicUI|RequestArg "Actor")
    (bind _paired (Variables|Default|GetPaired)
      (:then
        (CallFunction|TransmitMagicon _paired (Variables|Default|GetObsRef)))
      (:else))))

(event EventCancelSpell
  (bind _bezarrow (Variables|Default|GetBezArrow)
    (:then
      (Actor|DestroyActor _bezarrow))
    (:else
      _))
  (Class|MagicUI|Die)
  (bind _bodyref (Variables|Default|GetBodyRef)
    (:then
      (bind _stamwidgref (Variables|/Game/Blueprints/Entities/PlayerEntityTypes/PlayerEntityBaseBP.PlayerEntityBaseBP_C|GetStamWidgRef _bodyref)
        (:then
          (Default|ClearShownCost _stamwidgref))
        (:else
          _)))
    (:else
      _))
  (bind _paired (Variables|Default|GetPaired)
    (:then
      (CallFunction|ServerDie _paired))
    (:else)))

(fn ConstructionScript
  (|CallParentFunction))

(fn SetPaired
  (params (Paired :type Magic%20UI%20Object%20Reference))
  (bind _astelethrow_magic_ui (Utilities|Casting|CastToTelethrowMagicUI Paired)
    (:then
      (Variables|Default|SetPaired _astelethrow_magic_ui))
    (:CastFailed
      _))
  (return false))

(fn CastSpell
  (params (Caster :type Actor%20Object%20Reference))
  (bind _asobserver_bp (Utilities|Casting|CastToObserverBP Caster)
    (:then
      (if (>= (Utilities|Array|FindItem (Variables|/Game/Blueprints/Entities/PlayerEntityTypes/PlayerEntityBaseBP.PlayerEntityBaseBP_C|GetColorSchemeNames (Variables|/Game/Blueprints/ObserverBP.ObserverBP_C|GetBody _asobserver_bp)) "Magic") 0)
        (LocalVariables|SetChosenColor (Utilities|Array|Get(acopy) (Variables|/Game/Blueprints/Entities/PlayerEntityTypes/PlayerEntityBaseBP.PlayerEntityBaseBP_C|GetColorSchemeColors (Variables|/Game/Blueprints/ObserverBP.ObserverBP_C|GetBody _asobserver_bp)) (Utilities|Array|FindItem (Variables|/Game/Blueprints/Entities/PlayerEntityTypes/PlayerEntityBaseBP.PlayerEntityBaseBP_C|GetColorSchemeNames (Variables|/Game/Blueprints/ObserverBP.ObserverBP_C|GetBody _asobserver_bp)) "Magic")))
        (else
          (LocalVariables|SetChosenColor (CallFunction|GetMaterialColor) :!label _label))))
    (:CastFailed
      (goto _label)))
  (bind _target (Variables|Default|GetTarget)
    (:then
      (bind _asmagic_grab (Utilities|Casting|CastToMagicGrab (Actor|GetAttachParentActor _target))
        (:then
          (if (Networking|IsServer)
            (Default|CastMagic (.AsObserver%20BP (Utilities|Casting|CastToObserverBP (Components|GetOwner (Components|GetOwner _asmagic_grab)))) "/Game/Blueprints/Magic/TelegrabMagicUI.TelegrabMagicUI_C")))
        (:CastFailed
          _))
      (bind _returnvalue (Effects|SpawnEmitteratLocation "/Game/Assets/VFX/MagicFX/Teleport/Teleport_StartPoint.Teleport_StartPoint" (Transformation|GetActorLocation _target)))
      (CallFunction|Launch _target (+ (* (- (Variables|Default|GetTowardLoc) (Transformation|GetActorLocation (Variables|Default|GetTarget))) (Math|Float|Lerp 1.0 3.0 (Variables|Default|GetThrowPower))) (* "0, 0,980.000000" (- 1.0 (Variables|Default|GetThrowPower)))))
      (bind _returnvalue_2 (Effects|SpawnEmitteratLocation "/Game/Assets/VFX/MagicFX/Teleport/Teleport_EndPoint.Teleport_EndPoint" (Variables|Default|GetTowardLoc)))
      (bind _returnvalue_3 (Effects|SpawnEmitteratLocation "/Game/Assets/VFX/MagicFX/Teleport/Teleport_Line.Teleport_Line" (Transformation|GetActorLocation _target)))
      (Effects|Components|ParticleSystem|SetColorParameter _returnvalue_3 "MagicColor" (LocalVariables|GetChosenColor))
      (for _array_element (Variables|Default|GetBezPieces)
        (Class|ParticleSystemComponent|GenerateParticleEvent _returnvalue_3 "LineBurst" 0.0 _array_element "0, 0, 0" "0, 0, 0"))
      (Utilities|IsValid (Variables|/Game/Blueprints/ObserverBP.ObserverBP_C|GetBody _asobserver_bp)
        (:Is%20Valid
          (Components|Activation|Deactivate (Variables|/Game/Blueprints/Entities/PlayerEntityTypes/PlayerEntityBaseBP.PlayerEntityBaseBP_C|GetDust (Variables|/Game/Blueprints/ObserverBP.ObserverBP_C|GetBody _asobserver_bp)))
          (bind _stamwidgref (Variables|/Game/Blueprints/Entities/PlayerEntityTypes/PlayerEntityBaseBP.PlayerEntityBaseBP_C|GetStamWidgRef (Variables|/Game/Blueprints/ObserverBP.ObserverBP_C|GetBody _asobserver_bp))
            (:then
              (Default|InflictShownCost _stamwidgref))
            (:else
              _)))
        (:Is%20Not%20Valid
          _))
      (return false))
    (:else
      (return false))))

(fn MakeHelperArrow
  (bind _previousargs (Variables|Default|GetPreviousArgs))
  (bind _returnvalue (Game|SpawnActorfromClass "/Game/Blueprints/Magic/UniversalSpellUIHelpers/SpellHelper_BezArrow.SpellHelper_BezArrow_C" (Math|Transform|MakeTransform "0, 0, 0" "0, 0, 0" "1,1,1") "Undefined" (Variables|Default|GetObsRef) (Utilities|Array|Get(acopy) _previousargs (Utilities|Array|LastIndex _previousargs)) (Variables|Default|GetNewestArg) 5e+02 "0.000000,0.000000,1.000000" 5 true))
  (bind _output_get (Variables|Default|SetBezArrow _returnvalue))
  (Variables|/Game/Blueprints/Magic/UniversalSpellUIHelpers/SpellHelper_BezArrow.SpellHelper_BezArrow_C|SetColor _output_get (CallFunction|GetMaterialColor)))

(fn GetArrowLocs
  (for _array_element (Variables|/Game/Blueprints/Magic/UniversalSpellUIHelpers/SpellHelper_BezArrow.SpellHelper_BezArrow_C|GetSegSprites (Variables|Default|GetBezArrow))
    (Utilities|Array|Add (LocalVariables|GetBezLocs) (Transformation|GetWorldLocation _array_element)))
  (return (LocalVariables|GetBezLocs)))

(fn GetCurrentStaminaCost
  (bind _target (Variables|Default|GetTarget)
    (:then
      (bind _bodyref (Variables|Default|GetBodyRef)
        (:then
          (bind _newestarg (Variables|Default|GetNewestArg)
            (:then
              (LocalVariables|SetOtherLoc (Transformation|GetWorldLocation _newestarg)))
            (:else
              (LocalVariables|SetOtherLoc (Variables|Default|GetTowardLoc))))
          (return (* (Variables|/Game/Blueprints/Entities/PlayerEntityTypes/PlayerEntityBaseBP.PlayerEntityBaseBP_C|GetMagicCostMultiplier _bodyref) (/ (Math|Vector|VectorLength (- (LocalVariables|GetOtherLoc) (Transformation|GetActorLocation _target))) (LocalVariables|GetStamRatioDist)))))
        (:else
          _)))
    (:else
      _))
  (return 0.0))

(fn ResizeArrow
  (bind _bezarrow (Variables|Default|GetBezArrow)
    (:then
      (bind _output_get (Variables|Default|SetThrowPower (Math|Float|Clamp(Float) (/ (Math|Vector|VectorLength (- (Variables|Default|GetTowardLoc) (Transformation|GetWorldLocation (Variables|Default|GetNewestArg)))) 1.25e+03))))
      (Variables|/Game/Blueprints/Magic/UniversalSpellUIHelpers/SpellHelper_BezArrow.SpellHelper_BezArrow_C|SetCurveGrade _bezarrow (Math|Float|Lerp 5e+02 1e+02 _output_get))
      (LocalVariables|SetArrowSize (Math|Float|Lerp 1.0 1e+01 _output_get))
      (for _array_element (Variables|/Game/Blueprints/Magic/UniversalSpellUIHelpers/SpellHelper_BezArrow.SpellHelper_BezArrow_C|GetSegSprites _bezarrow)
        (Transformation|SetWorldScale3D _array_element (Math|Vector|MakeVector (LocalVariables|GetArrowSize) (LocalVariables|GetArrowSize) (.z (Transformation|GetWorldScale _array_element)))))
      (Transformation|SetWorldScale3D (Variables|/Game/Blueprints/Magic/UniversalSpellUIHelpers/SpellHelper_BezArrow.SpellHelper_BezArrow_C|GetArrowSprite _bezarrow) (Math|Conversions|ToVector(Float) (LocalVariables|GetArrowSize))))
    (:else)))

(fn Launch
  (params (Target :type Actor%20Object%20Reference) (Velocity :type Vector))
  (bind _ascharacter (Utilities|Casting|CastToCharacter Target)
    (:then
      (Character|LaunchCharacter _ascharacter Velocity true true))
    (:CastFailed
      (bind _aschangeling_roomba (Utilities|Casting|CastToChangelingRoomba Target)
        (:then
          (Default|DoAirBonk _aschangeling_roomba)
          (Physics|SetPhysicsLinearVelocity (Variables|/Game/Blueprints/Misc/ChangelingRoomba.ChangelingRoomba_C|GetRoomba _aschangeling_roomba) Velocity false "None"))
        (:CastFailed
          (for _array_element (Actor|GetComponentsByClass Target "/Script/Engine.PrimitiveComponent")
            (if (Physics|IsSimulatingPhysics _array_element "None")
              (Physics|SetPhysicsLinearVelocity _array_element Velocity false "None"))))))))