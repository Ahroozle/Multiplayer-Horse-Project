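; Teleport spell controller that moves a chosen actor to a player-picked location and height.
; The owning player's instance gathers arguments in sequence with a Bezier helper arrow, relaying each, plus distance-based stamina cost, to its paired instance.
; The paired instance casts: it relocates the target, spawns tinted particles along the arc and inflicts stamina cost.
; Targets attached to a MagicGrab also trigger the grabber's telegrab magic on the server.
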(event Custom|OnReceiveArg1
  (params (ActorArg :type Actor%20Object%20Reference))
  (EventDispatchers|UnbindEventfromOnReceiveActorArg (delegate Custom|OnReceiveArg1))
  (Variables|Default|SetTarget ActorArg)
  (bind _paired (Variables|Default|GetPaired)
    (:then
      (CallFunction|TransmitArg1 _paired ActorArg))
    (:else
      _))
  (EventDispatchers|BindEventtoOnReceiveLocationArg (delegate Custom|OnReceiveArg2))
  (Class|MagicUI|RequestArg "Location")
  (CallFunction|MakeHelperArrow))

(event Custom|TransmitMagicOn
  (params (Obs :type Observer%20BP%20Object%20Reference))
  (CallFunction|FinishTransmitMagicon Obs))

(event Custom|FinishTransmitMagicOn
  (params (Obs :type Observer%20BP%20Object%20Reference))
  (CallFunction|SetObs Obs)
  (CallFunction|SetBodyMagic true false))

(event Custom|OnReceiveArg2
  (params (LocationArg :type Vector))
  (EventDispatchers|UnbindEventfromOnReceiveLocationArg (delegate Custom|OnReceiveArg2))
  (Variables|Default|SetToLoc LocationArg)
  (bind _paired (Variables|Default|GetPaired)
    (:then
      (CallFunction|TransmitArg2 _paired LocationArg))
    (:else
      _))
  (EventDispatchers|BindEventtoOnReceiveHeightArg (delegate Custom|OnReceiveArg3))
  (Class|MagicUI|RequestArg "Height")
  (bind _bezarrow (Variables|Default|GetBezArrow)
    (:then
      (Variables|/Game/Blueprints/Magic/UniversalSpellUIHelpers/SpellHelper_BezArrow.SpellHelper_BezArrow_C|SetEnd _bezarrow (Variables|Default|GetNewestArg)))
    (:else)))

(event Custom|FinishTransmitArg3
  (params (Arg3 :type Vector) (BezLocs :type Array%20of%20Vectors) (Obs :type Observer%20BP%20Object%20Reference) (StamCost :type Float%20%28single-precision%29))
  (Variables|Default|SetToLoc Arg3)
  (Variables|Default|SetBezPieces BezLocs)
  (bind _bodyref (Variables|Default|GetBodyRef)
    (:then
      (bind _stamwidgref (Variables|/Game/Blueprints/Entities/PlayerEntityTypes/PlayerEntityBaseBP.PlayerEntityBaseBP_C|GetStamWidgRef _bodyref)
        (:then
          (Default|ShowCost _stamwidgref StamCost))
        (:else
          _)))
    (:else
      _))
  (CallFunction|CastSpell Obs)
  (Default|CallOnSpellFinished)
  (CallFunction|SetBodyMagic false false)
  (Class|MagicUI|Die))

(event Custom|FinishTransmitArg1
  (params (Arg1 :type Actor%20Object%20Reference))
  (Variables|Default|SetTarget Arg1))

(event Custom|FinishTransmitArg2
  (params (Arg2 :type Vector))
  (Variables|Default|SetToLoc Arg2))

(event Custom|TransmitArg1
  (params (Arg1 :type Actor%20Object%20Reference))
  (CallFunction|FinishTransmitArg1 Arg1))

(event Custom|OnReceiveArg3
  (params (HeightArg :type Vector))
  (EventDispatchers|UnbindEventfromOnReceiveHeightArg (delegate Custom|OnReceiveArg3))
  (Variables|Default|SetToLoc HeightArg)
  (bind _paired (Variables|Default|GetPaired)
    (:then
      (CallFunction|TransmitArg3 _paired HeightArg (CallFunction|GetArrowLocs) (Variables|Default|GetObsRef) (CallFunction|GetCurrentStaminaCost)))
    (:else
      _))
  (bind _bezarrow (Variables|Default|GetBezArrow)
    (:then
      (Actor|DestroyActor _bezarrow)
      (Class|MagicUI|Die))
    (:else)))

(event Custom|TransmitArg3
  (params (Arg3 :type Vector) (BezLocs :type Array%20of%20Vectors) (Obs :type Observer%20BP%20Object%20Reference) (StamCost :type Float%20%28single-precision%29))
  (CallFunction|FinishTransmitArg3 Arg3 BezLocs Obs StamCost))

(event Custom|TransmitArg2
  (params (Arg2 :type Vector))
  (CallFunction|FinishTransmitArg2 Arg2))

(event Custom|ServerDie
  (CallFunction|MulticastServerDie))

(event Custom|MulticastServerDie
  (|CallParentFunction))

(event EventInit
  (|CallParentFunction)
  (if (== (Game|GetPlayerController 0) (Components|GetOwner))
    (EventDispatchers|AssignOnReceiveActorArg (delegate Custom|OnReceiveArg1))
    (Class|MagicUI|RequestArg "Actor")
    (bind _paired (Variables|Default|GetPaired)
      (:then
        (CallFunction|TransmitMagicon _paired (Variables|Default|GetObsRef)))
      (:else))))

(event EventCancelSpell
  (bind _bezarrow (Variables|Default|GetBezArrow)
    (:then
      (Actor|DestroyActor _bezarrow))
    (:else
      _))
  (Class|MagicUI|Die)
  (bind _bodyref (Variables|Default|GetBodyRef)
    (:then
      (bind _stamwidgref (Variables|/Game/Blueprints/Entities/PlayerEntityTypes/PlayerEntityBaseBP.PlayerEntityBaseBP_C|GetStamWidgRef _bodyref)
        (:then
          (Default|ClearShownCost _stamwidgref))
        (:else
          _)))
    (:else
      _))
  (bind _paired (Variables|Default|GetPaired)
    (:then
      (CallFunction|ServerDie _paired))
    (:else)))

(fn ConstructionScript
  (|CallParentFunction))

(fn GetCurrentStaminaCost
  (bind _target (Variables|Default|GetTarget)
    (:then
      (bind _bodyref (Variables|Default|GetBodyRef)
        (:then
          (bind _newestarg (Variables|Default|GetNewestArg)
            (:then
              (LocalVariables|SetOtherLoc (Transformation|GetWorldLocation _newestarg)))
            (:else
              (LocalVariables|SetOtherLoc (Variables|Default|GetToLoc))))
          (return (* (Variables|/Game/Blueprints/Entities/PlayerEntityTypes/PlayerEntityBaseBP.PlayerEntityBaseBP_C|GetMagicCostMultiplier _bodyref) (/ (Math|Vector|VectorLength (- (LocalVariables|GetOtherLoc) (Transformation|GetActorLocation _target))) (LocalVariables|GetStamRatioDist)))))
        (:else
          _)))
    (:else
      _))
  (return 0.0))

(fn CastSpell
  (params (Caster :type Actor%20Object%20Reference))
  (bind _toloc (Variables|Default|GetToLoc))
  (bind _asobserver_bp (Utilities|Casting|CastToObserverBP Caster)
    (:then
      (if (>= (Utilities|Array|FindItem (Variables|/Game/Blueprints/Entities/PlayerEntityTypes/PlayerEntityBaseBP.PlayerEntityBaseBP_C|GetColorSchemeNames (Variables|/Game/Blueprints/ObserverBP.ObserverBP_C|GetBody _asobserver_bp)) "Magic") 0)
        (LocalVariables|SetChosenColor (Utilities|Array|Get(acopy) (.Colors (Utilities|Struct|BreakCharColorSchemePart (Utilities|Array|Get(acopy) (Variables|/Game/Blueprints/Entities/PlayerEntityTypes/PlayerEntityBaseBP.PlayerEntityBaseBP_C|GetColorSchemeData (Variables|/Game/Blueprints/ObserverBP.ObserverBP_C|GetBody _asobserver_bp)) (Utilities|Array|FindItem (Variables|/Game/Blueprints/Entities/PlayerEntityTypes/PlayerEntityBaseBP.PlayerEntityBaseBP_C|GetColorSchemeNames (Variables|/Game/Blueprints/ObserverBP.ObserverBP_C|GetBody _asobserver_bp)) "Magic"))))))
        (else
          (LocalVariables|SetChosenColor (CallFunction|GetMaterialColor) :!label _label))))
    (:CastFailed
      (goto _label)))
  (bind _target (Variables|Default|GetTarget)
    (:then
      (bind _asmagic_grab (Utilities|Casting|CastToMagicGrab (Actor|GetAttachParentActor _target))
        (:then
          (if (Networking|IsServer)
            (Default|CastMagic (.AsObserver%20BP (Utilities|Casting|CastToObserverBP (Components|GetOwner (Components|GetOwner _asmagic_grab)))) "/Game/Blueprints/Magic/TelegrabMagicUI.TelegrabMagicUI_C")))
        (:CastFailed
          _))
      (bind _returnvalue (Effects|SpawnEmitteratLocation "/Game/Assets/VFX/MagicFX/Teleport/Teleport_StartPoint.Teleport_StartPoint" (Transformation|GetActorLocation _target)))
      (Transformation|SetActorLocation _target _toloc false false)
      (bind _returnvalue_2 (Effects|SpawnEmitteratLocation "/Game/Assets/VFX/MagicFX/Teleport/Teleport_EndPoint.Teleport_EndPoint" _toloc))
      (bind _returnvalue_3 (Effects|SpawnEmitteratLocation "/Game/Assets/VFX/MagicFX/Teleport/Teleport_Line.Teleport_Line" (Transformation|GetActorLocation _target)))
      (Effects|Components|ParticleSystem|SetColorParameter _returnvalue_3 "MagicColor" (LocalVariables|GetChosenColor))
      (for _array_element (Variables|Default|GetBezPieces)
        (Class|ParticleSystemComponent|GenerateParticleEvent _returnvalue_3 "LineBurst" 0.0 _array_element "0, 0, 0" "0, 0, 0"))
      (Utilities|IsValid (Variables|/Game/Blueprints/ObserverBP.ObserverBP_C|GetBody _asobserver_bp)
        (:Is%20Valid
          (Components|Activation|Deactivate (Variables|/Game/Blueprints/Entities/PlayerEntityTypes/PlayerEntityBaseBP.PlayerEntityBaseBP_C|GetDust (Variables|/Game/Blueprints/ObserverBP.ObserverBP_C|GetBody _asobserver_bp)))
          (bind _stamwidgref (Variables|/Game/Blueprints/Entities/PlayerEntityTypes/PlayerEntityBaseBP.PlayerEntityBaseBP_C|GetStamWidgRef (Variables|/Game/Blueprints/ObserverBP.ObserverBP_C|GetBody _asobserver_bp))
            (:then
              (Default|InflictShownCost _stamwidgref))
            (:else
              _)))
        (:Is%20Not%20Valid
          _))
      (return false))
    (:else
      (return false))))

(fn MakeHelperArrow
  (bind _previousargs (Variables|Default|GetPreviousArgs))
  (bind _returnvalue (Game|SpawnActorfromClass "/Game/Blueprints/Magic/UniversalSpellUIHelpers/SpellHelper_BezArrow.SpellHelper_BezArrow_C" (Math|Transform|MakeTransform "0, 0, 0" "0, 0, 0" "1,1,1") "Undefined" (Variables|Default|GetObsRef) (Utilities|Array|Get(acopy) _previousargs (Utilities|Array|LastIndex _previousargs)) (Variables|Default|GetNewestArg) 5e+02 "0.000000,0.000000,1.000000" 15 false))
  (bind _output_get (Variables|Default|SetBezArrow _returnvalue))
  (Variables|/Game/Blueprints/Magic/UniversalSpellUIHelpers/SpellHelper_BezArrow.SpellHelper_BezArrow_C|SetColor _output_get (CallFunction|GetMaterialColor)))

(fn GetArrowLocs
  (for _array_element (Variables|/Game/Blueprints/Magic/UniversalSpellUIHelpers/SpellHelper_BezArrow.SpellHelper_BezArrow_C|GetSegSprites (Variables|Default|GetBezArrow))
    (Utilities|Array|Add (LocalVariables|GetBezLocs) (Transformation|GetWorldLocation _array_element)))
  (return (LocalVariables|GetBezLocs)))

(fn SetPaired
  (params (Paired :type Magic%20UI%20Object%20Reference))
  (bind _asteleport_magic_ui (Utilities|Casting|CastToTeleportMagicUI Paired)
    (:then
      (Variables|Default|SetPaired _asteleport_magic_ui))
    (:CastFailed
      _))
  (return false))