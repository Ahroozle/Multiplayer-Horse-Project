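; Arrow spell controller that has the player pick a location, then fires a fast magic arrow toward it from the caster's magic tip.
; The locally owned instance requests the location and relays it through its Paired instance, which casts and then dies.
; Casting spawns a MagicArrow tinted by the body's Magic color scheme, plays the shot sound and inflicts the shown stamina cost.
; Cancelling clears that cost and tears down the paired instance through a server-to-multicast death call.
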(event Custom|TransmitMagicOn
  (params (Obs :type Observer%20BP%20Object%20Reference))
  (CallFunction|FinishTransmitMagicon Obs))

(event Custom|FinishTransmitMagicOn
  (params (Obs :type Observer%20BP%20Object%20Reference))
  (CallFunction|SetObs Obs)
  (CallFunction|SetBodyMagic true false))

(event Custom|OnReceiveArg1
  (params (LocationArg :type Vector))
  (EventDispatchers|UnbindEventfromOnReceiveLocationArg (delegate Custom|OnReceiveArg1))
  (bind _paired (Variables|Default|GetPaired)
    (:then
      (CallFunction|TransmitArg1 _paired LocationArg (Variables|Default|GetObsRef))
      (Class|MagicUI|Die))
    (:else)))

(event Custom|FinishTransmitFinish
  (params (Obs :type Observer%20BP%20Object%20Reference))
  (CallFunction|CastSpell Obs)
  (Default|CallOnSpellFinished)
  (Class|MagicUI|Die))

(event Custom|TransmitFinish
  (params (Obs :type Observer%20BP%20Object%20Reference))
  (CallFunction|FinishTransmitFinish Obs))

(event Custom|FinishTransmitArg1
  (params (Arg1 :type Vector) (Obs :type Observer%20BP%20Object%20Reference))
  (Variables|Default|SetTargetLoc Arg1)
  (CallFunction|CastSpell Obs)
  (Default|CallOnSpellFinished)
  (CallFunction|SetBodyMagic false false)
  (Class|MagicUI|Die))

(event Custom|TransmitArg1
  (params (Arg1 :type Vector) (Obs :type Observer%20BP%20Object%20Reference))
  (CallFunction|FinishTransmitArg1 Arg1 Obs))

(event Custom|ServerDie
  (CallFunction|MulticastServerDie))

(event Custom|MulticastServerDie
  (|CallParentFunction))

(event EventInit
  (|CallParentFunction)
  (if (== (Game|GetPlayerController 0) (Components|GetOwner))
    (EventDispatchers|BindEventtoOnReceiveLocationArg (delegate Custom|OnReceiveArg1))
    (Class|MagicUI|RequestArg "Location_Any"))
  (bind _paired (Variables|Default|GetPaired)
    (:then
      (CallFunction|TransmitMagicon _paired (Variables|Default|GetObsRef)))
    (:else)))

(event EventCancelSpell
  (bind _bodyref (Variables|Default|GetBodyRef)
    (:then
      (bind _stamwidgref (Variables|/Game/Blueprints/Entities/PlayerEntityTypes/PlayerEntityBaseBP.PlayerEntityBaseBP_C|GetStamWidgRef _bodyref)
        (:then
          (Default|ClearShownCost _stamwidgref))
        (:else
          _)))
    (:else
      _))
  (Class|MagicUI|Die)
  (bind _paired (Variables|Default|GetPaired)
    (:then
      (CallFunction|ServerDie _paired))
    (:else)))

(fn ConstructionScript
  (|CallParentFunction))

(fn CastSpell
  (params (Caster :type Actor%20Object%20Reference))
  (bind _asobserver_bp (Utilities|Casting|CastToObserverBP Caster)
    (:then
      (bind _output_get (Variables|Default|SetObsRef _asobserver_bp))
      (bind _body (Variables|/Game/Blueprints/ObserverBP.ObserverBP_C|GetBody _output_get)
        (:then
          (bind _output_get_2 (Variables|Default|SetBodyRef _body))
          (if (>= (Utilities|Array|FindItem (Variables|/Game/Blueprints/Entities/PlayerEntityTypes/PlayerEntityBaseBP.PlayerEntityBaseBP_C|GetColorSchemeNames _output_get_2) "Magic") 0)
            (Variables|Default|SetChosenColor (Utilities|Array|Get(acopy) (.Colors (Utilities|Struct|BreakCharColorSchemePart (Utilities|Array|Get(acopy) (Variables|/Game/Blueprints/Entities/PlayerEntityTypes/PlayerEntityBaseBP.PlayerEntityBaseBP_C|GetColorSchemeData _output_get_2) (Utilities|Array|FindItem (Variables|/Game/Blueprints/Entities/PlayerEntityTypes/PlayerEntityBaseBP.PlayerEntityBaseBP_C|GetColorSchemeNames _output_get_2) "Magic"))))))
            (else
              (Variables|Default|SetChosenColor (CallFunction|GetMaterialColor))))
          (Game|SpawnActorfromClass "/Game/Blueprints/Misc/MagicArrow.MagicArrow_C" (Math|Transform|MakeTransform (+ (Transformation|GetWorldLocation (Default|GetMagicTip (Variables|Default|GetBodyRef))) (* (Math|Vector|Normalize (- (Variables|Default|GetTargetLoc) (Transformation|GetWorldLocation (Default|GetMagicTip (Variables|Default|GetBodyRef))))) 1e+02)) (Math|Rotator|MakeRotfromXZ (- (Variables|Default|GetTargetLoc) (Transformation|GetWorldLocation (Default|GetMagicTip (Variables|Default|GetBodyRef)))) (Math|Vector|MakeVector 0.0 0.0 1.0)) "1,1,1") "Undefined" (Variables|Default|GetBodyRef) (Variables|Default|GetChosenColor) 1e+04 true false 15.0 false "0.000000,0.000000,0.000000" 0.0 0.0 "0.000000,0.000000,0.000000" "/Game/Assets/Sound/SFX/Arrow/ArrowIdle_Cue.ArrowIdle_Cue" "/Game/Assets/VFX/Arrow/ArrowHit.ArrowHit" "/Game/Assets/Sound/SFX/Arrow/ArrowHit_Cue.ArrowHit_Cue")
          (bind _returnvalue (Class|StaticFuncLib|PlaySound (Transformation|GetWorldTransform (Default|GetMagicTip (Variables|Default|GetBodyRef))) "/Game/Assets/Sound/SFX/Arrow/ArrowShot_Cue.ArrowShot_Cue" (Math|Random|RandomFloatinRange 0.8 1.1)))
          (Default|SetAttenuation (Variables|Default|GetObsRef) _returnvalue)
          (bind _stamwidgref (Variables|/Game/Blueprints/Entities/PlayerEntityTypes/PlayerEntityBaseBP.PlayerEntityBaseBP_C|GetStamWidgRef (Variables|Default|GetBodyRef))
            (:then
              (Default|InflictShownCost _stamwidgref)
              (return false))
            (:else
              (return false))))
        (:else
          _)))
    (:CastFailed
      _))
  (return false))

(fn SetPaired
  (params (Paired :type Magic%20UI%20Object%20Reference))
  (bind _asarrow_magic_ui (Utilities|Casting|CastToArrowMagicUI Paired)
    (:then
      (Variables|Default|SetPaired _asarrow_magic_ui))
    (:CastFailed
      _))
  (return false))

(fn GetCurrentStaminaCost
  (return (Variables|Default|GetStamCost)))