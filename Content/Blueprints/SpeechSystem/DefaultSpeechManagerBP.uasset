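; Default speech manager that runs players' chat commands, selects speech bubble types and toggles the stopped state on player observers.
; HandleCommand routes aliased commands for flap limit, respawn, emotes, dice rolls and help, mostly returning markup-formatted replies.
; Helpers resolve speakers from controllers, observers or entities, and check moderator status by IP against world and universal access lists, gating flap-limit changes.
; Metadata B tags choose the next bubble class, with cutscene variants.
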(event EventUnstopPlayer
  (params (PlayerPawn :type Pawn%20Object%20Reference))
  (bind _asobserver_bp (Utilities|Casting|CastToObserverBP PlayerPawn))
  (Variables|/Game/Blueprints/ObserverBP.ObserverBP_C|SetStopped _asobserver_bp false))

(event EventHandleMetadata
  (params (Message :type Speech%20Parsed%20Message%20Structure%20%28by%20ref%29))
  (bind _speechbubbletypes (Variables|Default|GetSpeechBubbleTypes))
  (bind _incutscene (Variables|Default|GetInCutscene))
  (bind _value (Utilities|Map|Find _speechbubbletypes "Default"))
  (bind (_normal _cutscene) (Utilities|Struct|BreakBubbleType _value))
  (for _array_element (.MetadataTags (Utilities|Struct|BreakSpeechParsedMessage Message))
    (if (> (Utilities|Array|Length (Utilities|String|ParseIntoArray (.TagArgs (Utilities|Struct|BreakSpeechTag _array_element)) " ")) 0)
      (switch name (Utilities|String|StringToName (Utilities|Array|Get(acopy) (Utilities|String|ParseIntoArray (.TagArgs (Utilities|Struct|BreakSpeechTag _array_element)) " ")))
        (:B
          (if (> (Utilities|Array|Length (Utilities|String|ParseIntoArray (.TagArgs (Utilities|Struct|BreakSpeechTag _array_element)) " ")) 1)
            (if (.ReturnValue (Utilities|Map|Find _speechbubbletypes (Utilities|String|StringToName (Utilities|Array|Get(acopy) (Utilities|String|ParseIntoArray (.TagArgs (Utilities|Struct|BreakSpeechTag _array_element)) " ") 1))))
              (Variables|Default|SetNextBubbleType (.AsSpeech%20Bubble (Utilities|Casting|CastToSpeechBubbleClass (Class|KismetMathLibrary|SelectClass (.Normal (Utilities|Struct|BreakBubbleType (.Value (Utilities|Map|Find _speechbubbletypes (Utilities|String|StringToName (Utilities|Array|Get(acopy) (Utilities|String|ParseIntoArray (.TagArgs (Utilities|Struct|BreakSpeechTag _array_element)) " ") 1)))))) (.Cutscene (Utilities|Struct|BreakBubbleType (.Value (Utilities|Map|Find _speechbubbletypes (Utilities|String|StringToName (Utilities|Array|Get(acopy) (Utilities|String|ParseIntoArray (.TagArgs (Utilities|Struct|BreakSpeechTag _array_element)) " ") 1)))))) _incutscene))))
              (else
                (Variables|Default|SetNextBubbleType (.AsSpeech%20Bubble (Utilities|Casting|CastToSpeechBubbleClass (Class|KismetMathLibrary|SelectClass _normal _cutscene _incutscene))))))))))))

(event EventStopPlayer
  (params (PlayerPawn :type Pawn%20Object%20Reference))
  (bind _asobserver_bp (Utilities|Casting|CastToObserverBP PlayerPawn))
  (Variables|/Game/Blueprints/ObserverBP.ObserverBP_C|SetStopped _asobserver_bp true))

(fn ConstructionScript)

(fn HandleCommand
  (params (Caller :type Object%20Object%20Reference) (RawCommand :type String))
  (bind (_lefts _rights _returnvalue) (Utilities|String|Split RawCommand " "))
  (bind _asactor (Utilities|Casting|CastToActor Caller))
  (bind _returnvalue_2 (CallFunction|GetSpeakerName _asactor))
  (bind _array (Utilities|Array|MakeArray _returnvalue_2))
  (if _returnvalue
    (LocalVariables|SetCommand (Utilities|String|StringToName _lefts))
    (LocalVariables|SetArgs _rights)
    (else
      (LocalVariables|SetCommand (Utilities|String|StringToName RawCommand))))
  (switch name (LocalVariables|GetCommand)
    (:Default
      (return "" (Utilities|Array|MakeArray) false))
    (:flaplimit
      _)
    (:flaps
      _)
    (:respawn
      (bind _msg (CommandHelpers|HandleRespawn _asactor :!label _label))
      (return _msg _array false))
    (:resp
      (goto _label))
    (:me
      (bind _msg_2 (CommandHelpers|HandleOWO (LocalVariables|GetArgs)))
      (return _msg_2 (Utilities|Array|MakeArray) false))
    (:roll
      (bind _msg_3 (CommandHelpers|HandleRoll (LocalVariables|GetArgs) :!label _label_2))
      (return _msg_3 _array false))
    (:rand
      (goto _label_2))
    (:random
      (goto _label_2))
    (:dice
      (goto _label_2))
    (:help
      (CommandHelpers|HandleHelp _asactor (LocalVariables|GetArgs))
      (return "" _array false)))
  (bind _msg_4 (CommandHelpers|HandleFlaplimit _asactor (LocalVariables|GetArgs)))
  (return _msg_4 _array false))

(fn SpeakerIsAPlayer
  (params (Speaker :type Actor%20Object%20Reference))
  (return (Math|Boolean|ORBoolean (.bSuccess (Utilities|Casting|CastToPlayerController Speaker)) (.bSuccess (Utilities|Casting|CastToObserverBP Speaker)) (.bSuccess (Utilities|Casting|CastToPlayerEntityBaseBP Speaker)))))

(fn PlayerIsModerator
  (params (Player :type Actor%20Object%20Reference))
  (bind _returnvalue (Class|StaticFuncLib|RetrieveGameInstance))
  (bind (_worldacl _returnvalue_2) (Class|MPHorsoGameInstance|GetWorldAccessControlList _returnvalue))
  (bind _asplayer_controller (Utilities|Casting|CastToPlayerController Player)
    (:then
      (LocalVariables|SetRetrievedController _asplayer_controller))
    (:CastFailed
      (bind _asobserver_bp (Utilities|Casting|CastToObserverBP Player)
        (:then
          (bind _asplayer_controller_2 (Utilities|Casting|CastToPlayerController (Pawn|GetController _asobserver_bp))
            (:then
              (LocalVariables|SetRetrievedController _asplayer_controller_2))
            (:CastFailed
              (return false))))
        (:CastFailed
          (bind _asplayer_entity_base_bp (Utilities|Casting|CastToPlayerEntityBaseBP Player)
            (:then
              (bind _asobserver_bp_2 (Utilities|Casting|CastToObserverBP (Components|GetOwner _asplayer_entity_base_bp))
                (:then
                  (bind _asplayer_controller_3 (Utilities|Casting|CastToPlayerController (Pawn|GetController _asobserver_bp_2))
                    (:then
                      (LocalVariables|SetRetrievedController _asplayer_controller_3))
                    (:CastFailed
                      (return false))))
                (:CastFailed
                  (return false))))
            (:CastFailed
              (return false)))))))
  (Utilities|IsValid _returnvalue
    (:Is%20Valid
      (if (.ReturnValue (Class|MPHorsoGameInstance|GetPlayerIP _returnvalue (LocalVariables|GetRetrievedController)))
        (if _returnvalue_2
          (return (or (Class|AccessControlListFuncLib|IsModerator _returnvalue _worldacl (.OutIP (Class|MPHorsoGameInstance|GetPlayerIP _returnvalue (LocalVariables|GetRetrievedController)))) (Class|AccessControlListFuncLib|IsModerator _returnvalue (Class|MPHorsoGameInstance|GetUniversalAccessControlList _returnvalue) (.OutIP (Class|MPHorsoGameInstance|GetPlayerIP _returnvalue (LocalVariables|GetRetrievedController))))))
          (else
            (return (Class|AccessControlListFuncLib|IsModerator _returnvalue (Class|MPHorsoGameInstance|GetUniversalAccessControlList _returnvalue) (.OutIP (Class|MPHorsoGameInstance|GetPlayerIP _returnvalue (LocalVariables|GetRetrievedController)))))))
        (else
          _)))
    (:Is%20Not%20Valid
      _))
  (return false))

(fn GetSpeakerName
  (params (Speaker :type Actor%20Object%20Reference))
  (bind _asobserver_bp (Utilities|Casting|CastToObserverBP Speaker)
    (:then
      (return (Utilities|String|ToString(Name) (Variables|/Game/Blueprints/ObserverBP.ObserverBP_C|GetStoredName _asobserver_bp))))
    (:CastFailed
      (bind _asplayer_controller (Utilities|Casting|CastToPlayerController Speaker)
        (:then
          (bind _asobserver_bp_2 (Utilities|Casting|CastToObserverBP (Pawn|GetControlledPawn _asplayer_controller))
            (:then
              (return (Utilities|String|ToString(Name) (Variables|/Game/Blueprints/ObserverBP.ObserverBP_C|GetStoredName _asobserver_bp_2))))
            (:CastFailed
              _)))
        (:CastFailed
          (bind _asplayer_entity_base_bp (Utilities|Casting|CastToPlayerEntityBaseBP Speaker)
            (:then
              (bind _asobserver_bp_3 (Utilities|Casting|CastToObserverBP (Components|GetOwner _asplayer_entity_base_bp))
                (:then
                  (return (Utilities|String|ToString(Name) (Variables|/Game/Blueprints/ObserverBP.ObserverBP_C|GetStoredName _asobserver_bp_3))))
                (:CastFailed
                  _)))
            (:CastFailed
              _))))
      (return ""))))

(fn HandleFlaplimit
  (params (Caller :type Actor%20Object%20Reference) (Args :type String))
  (bind _observer (CallFunction|GetSpeakerObserver Caller))
  (bind _body (Variables|/Game/Blueprints/ObserverBP.ObserverBP_C|GetBody _observer))
  (if (Class|KismetStringLibrary|IsNumeric Args)
    (if (CallFunction|PlayerIsModerator Caller)
      (if (Utilities|Enum|Equal(Enum) (Variables|/Game/Blueprints/Entities/PlayerEntityTypes/PlayerEntityBaseBP.PlayerEntityBaseBP_C|GetAbility _body) "NewEnumerator2")
        (bind _output_get (Variables|/Script/Engine.Character|SetJumpMaxCount _body (Math|Integer|Max(Integer) (+ (Math|Conversions|ToInteger(Byte) Args) 1) 4)))
        (return (Utilities|String|Append "[c/00ffff:Flap limit changed to " (Utilities|String|ToString(Integer) (- _output_get 1)) " (Minimum allowed: 3 flaps)]"))
        (else
          (return "[c/ff0000:Flaplimit Error: The calling player is currently unable to fly and therefore unable to have their flap limit changed.]")))
      (else
        (return "[c/ff0000:Flaplimit Error: You aren't a moderator.]")))
    (else
      (return (Utilities|String|Append "[c/ff0000:Flaplimit Error: parameter '" Args "' is not a number.]")))))

(fn HandleRespawn
  (params (Caller :type Actor%20Object%20Reference))
  (bind _observer (CallFunction|GetSpeakerObserver Caller))
  (bind _body (Variables|/Game/Blueprints/ObserverBP.ObserverBP_C|GetBody _observer))
  (Utilities|IsValid _observer
    (:Is%20Valid
      (bind _outactors (Actor|GetAllActorsOfClass "/Game/Blueprints/Misc/RespawnNode.RespawnNode_C"))
      (if (> (Utilities|Array|Length _outactors) 0)
        (Transformation|SetActorLocation _body (Transformation|GetActorLocation (Utilities|Array|Get(acopy) _outactors)) false false)
        (else
          (bind _outactors_2 (Actor|GetAllActorsOfClass "/Script/Engine.PlayerStart"))
          (if (> (Utilities|Array|Length _outactors_2) 0)
            (Transformation|SetActorLocation _body (Transformation|GetActorLocation (Utilities|Array|Get(acopy) _outactors_2)) false false)
            (else
              (return "[c/ff0000:Respawn Error: Couldn't find a valid respawn point.]")))))
      (return "[c/00ffff:Player successfully respawned.]"))
    (:Is%20Not%20Valid
      (Development|PrintString "DefaultCommandBlock::ExecuteRespawn: Couldn't retrieve an Observer reference from the caller!")
      (return "[c/ff0000:Respawn Error: Couldn't retrieve the calling player.]"))))

(fn HandleOWO
  (params (Args :type String))
  (return (Utilities|String|Append "*[emph:" Args "]*")))

(fn HandleRoll
  (params (Args :type String))
  (bind _returnvalue (Utilities|String|Trim Args))
  (bind _returnvalue_2 (Utilities|String|TrimTrailing _returnvalue))
  (bind (_lefts _rights _returnvalue_3) (Utilities|String|Split _returnvalue_2 "d"))
  (bind (_lefts_2 _rights_2 _returnvalue_4) (Utilities|String|Split _returnvalue_2 "~"))
  (bind _returnvalue_5 (Math|Conversions|ToInteger(Byte) _rights))
  (bind _returnvalue_6 (Math|Conversions|ToInteger(Byte) _lefts))
  (if (> (Utilities|String|Len Args) 0)
    (if _returnvalue_3
      (if (and (Class|KismetStringLibrary|IsNumeric _lefts) (Class|KismetStringLibrary|IsNumeric _rights))
        (if (> _returnvalue_6 0)
          (if (<= _returnvalue_6 1000)
            (if (> _returnvalue_5 1)
              (bind _returnvalue_7 (Class|CutsceneFuncLib|Roll _returnvalue_6 _returnvalue_5))
              (return (Utilities|String|Append "[c/00ffff:Rolled " _lefts "d" _rights ", result: " (Utilities|String|ToString(Integer) _returnvalue_7) "]"))
              (else
                (return "[c/ff0000:Roll Error: Was asked to roll a dice which has less than 2 sides.]")))
            (else
              (return "[c/ff0000:Roll Error: Was asked to roll more than 1000 dice, which is the maximum amount of die allowed to be rolled at once.]")))
          (else
            (return "[c/ff0000:Roll Error: Was asked to roll less than 1 dice.]")))
        (else
          (return "[c/ff0000:Roll Error: One of the input values wasn't a number.]")))
      (elif _returnvalue_4
        (if (and (Class|KismetStringLibrary|IsNumeric _lefts_2) (Class|KismetStringLibrary|IsNumeric _rights_2))
          (return (Utilities|String|Append "[c/00ffff:Picked a number from " _lefts_2 " to " _rights_2 ", result: " (Utilities|String|ToString(Integer) (Math|Random|RandomIntegerinRange (Math|Conversions|ToInteger(Byte) _lefts_2) (Math|Conversions|ToInteger(Byte) _rights_2))) "]"))
          (else
            (return "[c/ff0000:Roll Error: One of the input values wasn't a number.]")))
        (else
          (return (Utilities|String|Append "[c/ff0000:Roll Error: parameter '" _returnvalue_2 "' doesn't conform to XdY syntax, nor X~Y syntax.]")))))
    (else
      (bind _returnvalue_8 (Class|CutsceneFuncLib|Roll 1 100))
      (return (Utilities|String|Append "[c/00ffff:Rolled 1d100, result: " (Utilities|String|ToString(Integer) _returnvalue_8) "]")))))

(fn HandleHelp
  (params (Caller :type Actor%20Object%20Reference) (Args :type String))
  (bind _observer (CallFunction|GetSpeakerObserver Caller))
  (Utilities|IsValid _observer
    (:Is%20Valid
      (Default|SpawnHelp _observer Args))))

(fn GetSpeakerObserver
  (params (Speaker :type Actor%20Object%20Reference))
  (bind _asobserver_bp (Utilities|Casting|CastToObserverBP Speaker)
    (:then
      (return _asobserver_bp))
    (:CastFailed
      (bind _asplayer_controller (Utilities|Casting|CastToPlayerController Speaker)
        (:then
          (bind _asobserver_bp_2 (Utilities|Casting|CastToObserverBP (Pawn|GetControlledPawn _asplayer_controller))
            (:then
              (return _asobserver_bp_2))
            (:CastFailed
              _)))
        (:CastFailed
          (bind _asplayer_entity_base_bp (Utilities|Casting|CastToPlayerEntityBaseBP Speaker)
            (:then
              (bind _asobserver_bp_3 (Utilities|Casting|CastToObserverBP (Components|GetOwner _asplayer_entity_base_bp))
                (:then
                  (return _asobserver_bp_3))
                (:CastFailed
                  _)))
            (:CastFailed
              _))))
      (return 0))))

(fn GetPlayerbyIPorUID
  (params (IP_Or_UID :type String))
  (bind _returnvalue (Math|Conversions|ToInteger(Byte) IP_Or_UID))
  (bind _self self)
  (bind _returnvalue_2 (Class|MPHorsoNetLibrary|GetPlayerbyUID _self _returnvalue))
  (bind (_outparts _outerrorstring _returnvalue_3) (Class|MPHorsoNetLibrary|FormatIPv4 IP_Or_UID))
  (if _returnvalue_3
    (return (Class|MPHorsoNetLibrary|GetPlayerbyIP _self _outerrorstring) _outerrorstring false)
    (elif (Class|KismetStringLibrary|IsNumeric IP_Or_UID)
      (return _returnvalue_2 (Class|MPHorsoNetLibrary|GetPlayerIP _returnvalue_2) true)
      (else
        (return 0 "" false)))))