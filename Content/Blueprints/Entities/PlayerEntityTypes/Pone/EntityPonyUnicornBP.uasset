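; Unicorn pony player entity Blueprint that extends a parent pony entity with a horn tip and magic on/off body animations.
; Magic events play matching animations on both the FrontBody and BackBody sprites.
; After parent facing logic, DoMoveFace shows HornTip and mirrors its Y offset only when FrontBody visibility changes, tracked by NeedsFlip.
; GetMagicTip exposes HornTip as the magic origin component.
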(event EventDoMoveFace
  (params (HeadingVector :type Vector))
  (bind _frontbody (Variables|Default|GetFrontBody))
  (bind _horntip (Variables|Default|GetHornTip))
  (bind _returnvalue (Rendering|IsVisible _frontbody))
  (|CallParentFunction HeadingVector)
  (Rendering|SetVisibility (Variables|Default|GetHornTip) true true)
  (if (Math|Boolean|NotEqual(Boolean) _returnvalue (Variables|Default|GetNeedsFlip))
    (bind _output_get (Variables|Default|SetNeedsFlip _returnvalue))
    (if _output_get
      (Transformation|SetRelativeLocation _horntip "36.0,1.000000,39.0" false false)
      (else
        (Transformation|SetRelativeLocation _horntip "36.0,-1.000000,39.0" false false)))))

(event EventPlayMagiconAnimation
  (Class|SkeletalSpriteBodyComponent|PlayAnimation (Variables|Default|GetFrontBody) "/Game/Blueprints/SkeletalSpriteAnimations/PonyAnims/PonyAnim_MagicOn.PonyAnim_MagicOn_C")
  (Class|SkeletalSpriteBodyComponent|PlayAnimation (Variables|Default|GetBackBody) "/Game/Blueprints/SkeletalSpriteAnimations/PonyAnims_Back/PonyAnim_Back_MagicOn.PonyAnim_Back_MagicOn_C"))

(event EventPlayMagicOffAnimation
  (Class|SkeletalSpriteBodyComponent|PlayAnimation (Variables|Default|GetFrontBody) "/Game/Blueprints/SkeletalSpriteAnimations/PonyAnims/PonyAnim_MagicOff.PonyAnim_MagicOff_C")
  (Class|SkeletalSpriteBodyComponent|PlayAnimation (Variables|Default|GetBackBody) "/Game/Blueprints/SkeletalSpriteAnimations/PonyAnims_Back/PonyAnim_Back_MagicOff.PonyAnim_Back_MagicOff_C"))

(fn ConstructionScript
  (|CallParentFunction))

(fn GetMagicTip
  (return (Variables|Default|GetHornTip)))