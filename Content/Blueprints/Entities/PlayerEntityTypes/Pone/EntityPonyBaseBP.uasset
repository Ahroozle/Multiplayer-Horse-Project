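; Base Blueprint for pony entities, handling 2D body animation and head look-at.
; Walk, gallop, stand and jump events play paired sprite and offset animations on FrontBody and BackBody, with Running switching walk to gallop.
; Look aims both head bones at LookTarget using dot products: X-scale negation flips them, rotation tilts them, and vertical alignment picks a pupil animation.
; ResetLook restores normal pupils and front head scale.
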(event EventBeginPlay
  (|CallParentFunction))

(event Collision|EventActorBeginOverlap
  (params (OtherActor :type Actor%20Object%20Reference)))

(event EventPlayJumpAnimation
  (Class|SkeletalSpriteBodyComponent|PlayAnimation (Variables|Default|GetFrontBody) "/Game/Blueprints/SkeletalSpriteAnimations/PonyAnims/PonyAnim_Jump.PonyAnim_Jump_C" "/Game/Blueprints/SkeletalSpriteAnimations/0_OffsetAnims/PonyAnim_StandOffset.PonyAnim_StandOffset_C")
  (Class|SkeletalSpriteBodyComponent|PlayAnimation (Variables|Default|GetBackBody) "/Game/Blueprints/SkeletalSpriteAnimations/PonyAnims_Back/PonyAnim_Back_Jump.PonyAnim_Back_Jump_C" "/Game/Blueprints/SkeletalSpriteAnimations/0_OffsetAnims/Back/PonyAnim_Back_StandOffset.PonyAnim_Back_StandOffset_C"))

(event EventPlayWalkAnimation
  (Variables|Default|SetIsWalking true)
  (if (Variables|Default|GetRunning)
    (CallFunction|PlayGallopAnimation)
    (else
      (Class|SkeletalSpriteBodyComponent|PlayAnimation (Variables|Default|GetFrontBody) "/Game/Blueprints/SkeletalSpriteAnimations/PonyAnims/PonyAnim_Walk.PonyAnim_Walk_C" "/Game/Blueprints/SkeletalSpriteAnimations/0_OffsetAnims/PonyAnim_WalkOffset.PonyAnim_WalkOffset_C")
      (Class|SkeletalSpriteBodyComponent|PlayAnimation (Variables|Default|GetBackBody) "/Game/Blueprints/SkeletalSpriteAnimations/PonyAnims_Back/PonyAnim_Back_Walk.PonyAnim_Back_Walk_C" "/Game/Blueprints/SkeletalSpriteAnimations/0_OffsetAnims/Back/PonyAnim_Back_WalkOffset.PonyAnim_Back_WalkOffset_C"))))

(event EventPlayStandAnimation
  (Variables|Default|SetIsWalking false)
  (Class|SkeletalSpriteBodyComponent|PlayAnimation (Variables|Default|GetFrontBody) "/Game/Blueprints/SkeletalSpriteAnimations/PonyAnims/PonyAnim_Stand.PonyAnim_Stand_C" "/Game/Blueprints/SkeletalSpriteAnimations/0_OffsetAnims/PonyAnim_StandOffset.PonyAnim_StandOffset_C")
  (Class|SkeletalSpriteBodyComponent|PlayAnimation (Variables|Default|GetBackBody) "/Game/Blueprints/SkeletalSpriteAnimations/PonyAnims_Back/PonyAnim_Back_Stand.PonyAnim_Back_Stand_C" "/Game/Blueprints/SkeletalSpriteAnimations/0_OffsetAnims/Back/PonyAnim_Back_StandOffset.PonyAnim_Back_StandOffset_C"))

(event EventTick
  (params (DeltaSeconds :type Float%20%28single-precision%29))
  (|CallParentFunction DeltaSeconds))

(event EventLook
  (bind (_retrievedbone _returnvalue) (Class|SkeletalSpriteBodyComponent|GetBone (Variables|Default|GetFrontBody) "Head"))
  (bind (_retrievedbone_2 _returnvalue_2) (Class|SkeletalSpriteBodyComponent|GetBone (Variables|Default|GetBackBody) "BackHead"))
  (if (and _returnvalue _returnvalue_2)
    (CallFunction|InternalLook _retrievedbone _retrievedbone_2)))

(event EventResetLook
  (bind _frontbody (Variables|Default|GetFrontBody))
  (Class|SkeletalSpriteBodyComponent|PlayAnimation _frontbody "/Game/Blueprints/SkeletalSpriteAnimations/PonyAnims/Eye/PonyAnim_NormalLook.PonyAnim_NormalLook_C")
  (bind (_retrievedbone _returnvalue) (Class|SkeletalSpriteBodyComponent|GetBone _frontbody "Head"))
  (if _returnvalue
    (Transformation|SetRelativeScale3D _retrievedbone "1.000000,1.000000,1.000000")))

(event EventPlayGallopAnimation
  (Class|SkeletalSpriteBodyComponent|PlayAnimation (Variables|Default|GetFrontBody) "/Game/Blueprints/SkeletalSpriteAnimations/PonyAnims/PonyAnim_Gallop.PonyAnim_Gallop_C" "/Game/Blueprints/SkeletalSpriteAnimations/0_OffsetAnims/PonyAnim_GallopOffset.PonyAnim_GallopOffset_C")
  (Class|SkeletalSpriteBodyComponent|PlayAnimation (Variables|Default|GetBackBody) "/Game/Blueprints/SkeletalSpriteAnimations/PonyAnims_Back/PonyAnim_Back_Gallop.PonyAnim_Back_Gallop_C" "/Game/Blueprints/SkeletalSpriteAnimations/0_OffsetAnims/Back/PonyAnim_Back_GallopOffset.PonyAnim_Back_GallopOffset_C"))

(fn ConstructionScript
  (|CallParentFunction))

(fn InternalLook
  (params (HeadRef :type Scene%20Component%20Object%20Reference) (BackHeadRef :type Scene%20Component%20Object%20Reference))
  (bind _looktarget (Variables|Default|GetLookTarget)
    (:then
      (LocalVariables|SetToTarget (Math|Vector|Normalize (- (Transformation|GetWorldLocation _looktarget) (Transformation|GetWorldLocation HeadRef))))
      (CallFunction|InternalLookTurnHead (LocalVariables|GetToTarget) (* (Math|Vector|GetForwardVector HeadRef) (.x (Transformation|GetWorldScale HeadRef))) (LocalVariables|GetTurnThreshold) HeadRef)
      (CallFunction|InternalLookAngleHead true (LocalVariables|GetToTarget) HeadRef)
      (CallFunction|InternalLookTurnHead (LocalVariables|GetToTarget) (* (Math|Vector|GetForwardVector BackHeadRef) (.x (Transformation|GetWorldScale BackHeadRef))) (LocalVariables|GetTurnThreshold) BackHeadRef)
      (CallFunction|InternalLookAngleHead true (LocalVariables|GetToTarget) BackHeadRef)
      (bind _animclass (CallFunction|InternalLookMovePupils (LocalVariables|GetToTarget) HeadRef))
      (Class|SkeletalSpriteBodyComponent|PlayAnimation (Variables|Default|GetFrontBody) _animclass))
    (:else)))

(fn InternalLookTurnHead
  (params (ToTarg :type Vector) (RealForward :type Vector) (TurnThreshold :type Float%20%28single-precision%29) (HeadRef :type Scene%20Component%20Object%20Reference))
  (if (< (Math|Vector|DotProduct ToTarg RealForward) TurnThreshold)
    (Transformation|SetRelativeScale3D HeadRef (* (Variables|/Script/Engine.SceneComponent|GetRelativeScale3D HeadRef) "-1.000000,1.000000,1.000000"))))

(fn InternalLookAngleHead
  (params (Bobble :type Boolean) (ToTarg :type Vector) (HeadRef :type Scene%20Component%20Object%20Reference))
  (bind _returnvalue (Transformation|GetWorldScale HeadRef))
  (bind _nobobble_steps (LocalVariables|GetNoBobble_Steps))
  (if Bobble
    (LocalVariables|SetFinalRes (Math|Rotator|MakeRotator 0.0 (* 35.0 (Math|Vector|DotProduct ToTarg (Math|Vector|GetUpVector HeadRef)) (.x _returnvalue)) 0.0))
    (else
      (LocalVariables|SetFinalRes (Math|Rotator|MakeRotator 0.0 (* 17.0 (.x _returnvalue) (Math|Conversions|ToFloat(Integer) (/ (Math|Float|Floor (* _nobobble_steps (Math|Vector|DotProduct ToTarg "0, 0,1.000000"))) _nobobble_steps))) 0.0))))
  (Transformation|SetRelativeRotation HeadRef (LocalVariables|GetFinalRes) false false))

(fn InternalLookMovePupils
  (params (ToTarg :type Vector) (HeadRef :type Scene%20Component%20Object%20Reference))
  (LocalVariables|SetDotRes (Math|Vector|DotProduct ToTarg (Math|Vector|GetUpVector HeadRef)))
  (if (>= (LocalVariables|GetDotRes) 0.75)
    (return "/Game/Blueprints/SkeletalSpriteAnimations/PonyAnims/Eye/PonyAnim_UpLook.PonyAnim_UpLook_C")
    (elif (>= (LocalVariables|GetDotRes) 0.25)
      (return "/Game/Blueprints/SkeletalSpriteAnimations/PonyAnims/Eye/PonyAnim_UpRightLook.PonyAnim_UpRightLook_C")
      (elif (>= (LocalVariables|GetDotRes) -0.25)
        (return "/Game/Blueprints/SkeletalSpriteAnimations/PonyAnims/Eye/PonyAnim_NormalLook.PonyAnim_NormalLook_C")
        (elif (>= (LocalVariables|GetDotRes) -0.75)
          (return "/Game/Blueprints/SkeletalSpriteAnimations/PonyAnims/Eye/PonyAnim_DownRightLook.PonyAnim_DownRightLook_C")
          (else
            (return "/Game/Blueprints/SkeletalSpriteAnimations/PonyAnims/Eye/PonyAnim_DownLook.PonyAnim_DownLook_C")))))))