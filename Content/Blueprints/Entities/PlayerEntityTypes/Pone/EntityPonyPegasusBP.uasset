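; Pegasus variant of the player pony entity, adding stamina-based wing flaps on repeated jumps.
; With the matching ability, each jump past the first spends stamina and plays a flap on front and back body sprites, or a final flap when tired or drained.
; CanJumpInternal blocks further air jumps when FlyTired.
; Landing restores blinking, and standing closes the wings, adding sweat when tired.
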(event Custom|RepLanded
  (params (Hit :type Hit%20Result%20Structure))
  (|CallParentFunction (stale EventOnLanded Hit))
  (Variables|Default|SetShouldBlink true))

(event EventDoJump
  (params (Pressed :type Boolean))
  (bind _frontbody (Variables|Default|GetFrontBody))
  (bind _backbody (Variables|Default|GetBackBody))
  (if (or (> (Variables|Default|GetStaminaCurrent) 0.0) (> (Variables|Default|GetTempStamina) 0.0))
    (|CallParentFunction Pressed)
    (if (and Pressed (Utilities|Enum|Equal(Enum) (Variables|Default|GetAbility) "NewEnumerator2"))
      (if (> (Variables|Default|GetJumpCount) 1)
        (if (not (Variables|Default|GetTired))
          (Default|DepleteStamina (Variables|Default|GetStamWidgRef) "Fly" (Utilities|Struct|MakeStaminaCost (Variables|Default|GetFlapCost) false))
          (if (or (not (<= (Variables|Default|GetStaminaCurrent) 0.0)) (> (Variables|Default|GetTempStamina) 0.0))
            (Class|SkeletalSpriteBodyComponent|PlayAnimation _frontbody "/Game/Blueprints/SkeletalSpriteAnimations/PonyAnims/Wing/PonyAnim_Flap.PonyAnim_Flap_C")
            (Class|SkeletalSpriteBodyComponent|PlayAnimation _backbody "/Game/Blueprints/SkeletalSpriteAnimations/PonyAnims_Back/Wing/PonyAnim_Back_Flap.PonyAnim_Back_Flap_C")
            (Default|CallFlappedDelegate)
            (else
              (Variables|Default|SetShouldBlink false :!label _label)
              (Class|SkeletalSpriteBodyComponent|PlayAnimation _frontbody "/Game/Blueprints/SkeletalSpriteAnimations/PonyAnims/Wing/PonyAnim_FinalFlap.PonyAnim_FinalFlap_C")
              (Class|SkeletalSpriteBodyComponent|PlayAnimation _backbody "/Game/Blueprints/SkeletalSpriteAnimations/PonyAnims_Back/Wing/PonyAnim_Back_FinalFlap.PonyAnim_Back_FinalFlap_C")
              (Default|CallFlappedDelegate)))
          (else
            (goto _label)))))))

(event EventPlayStandAnimation
  (bind _frontbody (Variables|Default|GetFrontBody))
  (|CallParentFunction)
  (Class|SkeletalSpriteBodyComponent|PlayAnimation _frontbody "/Game/Blueprints/SkeletalSpriteAnimations/PonyAnims/PonyAnim_Unstrain.PonyAnim_Unstrain_C")
  (Class|SkeletalSpriteBodyComponent|PlayAnimation _frontbody "/Game/Blueprints/SkeletalSpriteAnimations/PonyAnims/Wing/PonyAnim_CloseWings.PonyAnim_CloseWings_C")
  (Class|SkeletalSpriteBodyComponent|PlayAnimation (Variables|Default|GetBackBody) "/Game/Blueprints/SkeletalSpriteAnimations/PonyAnims_Back/Wing/PonyAnim_Back_CloseWings.PonyAnim_Back_CloseWings_C")
  (if (Variables|Default|GetTired)
    (Class|SkeletalSpriteBodyComponent|PlayAnimation (Variables|Default|GetFrontBody) "/Game/Blueprints/SkeletalSpriteAnimations/PonyAnims/FaceEffect/PonyAnim_Sweat.PonyAnim_Sweat_C")
    (Class|SkeletalSpriteBodyComponent|PlayAnimation (Variables|Default|GetBackBody) "/Game/Blueprints/SkeletalSpriteAnimations/PonyAnims_Back/FaceEffect/PonyAnim_Back_Sweat.PonyAnim_Back_Sweat_C")))

(event EventOnLanded
  (params (Hit :type Hit%20Result%20Structure%20%28by%20ref%29))
  (|CallParentFunction Hit)
  (Variables|Default|SetShouldBlink true))

(fn ConstructionScript
  (|CallParentFunction))

(fn CanJumpInternal
  (return (or (<= (Variables|Default|GetJumpCount) 1) (not (Variables|Default|GetFlyTired)))))