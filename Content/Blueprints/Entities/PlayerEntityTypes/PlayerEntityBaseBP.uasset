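; Base character for player pony entities, handling movement, jumping, stamina and sprite presentation, with animation hooks left for child classes to override.
; Front and back sprite bodies face the camera, mirroring and swapping by movement heading, with recolorable bones and random blinking.
; Stamina widget events drive running cost, exhaustion and sustained spell cancellation.
; It records last grounded positions for navmesh-projected position reverts, and replicates dust and landing effects through multicasts.
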(event Custom|OnStamOut
  (Variables|Speed|SetCurrSpeed (Variables|Speed|GetLimpSpeed))
  (Variables|StaminaCost|SetTired true)
  (Variables|StaminaCost|SetRunning false)
  (Class|SkeletalSpriteBodyComponent|PlayAnimation (Variables|Default|GetFrontBody) "/Game/Blueprints/SkeletalSpriteAnimations/PonyAnims/FaceEffect/PonyAnim_Sweat.PonyAnim_Sweat_C")
  (Class|SkeletalSpriteBodyComponent|PlayAnimation (Variables|Default|GetBackBody) "/Game/Blueprints/SkeletalSpriteAnimations/PonyAnims_Back/FaceEffect/PonyAnim_Back_Sweat.PonyAnim_Back_Sweat_C")
  (if (Utilities|Enum|Equal(Enum) (Variables|Default|GetAbility) "NewEnumerator1")
    (CallFunction|KillSustainedSpells)))

(event Custom|OnStamFull
  (if (Variables|StaminaCost|GetTired)
    (Variables|Speed|SetCurrSpeed (Variables|Speed|GetWalkSpeed))
    (Variables|StaminaCost|SetTired false)
    (Variables|StaminaCost|SetFlyTired false))
  (Class|SkeletalSpriteBodyComponent|PlayAnimation (Variables|Default|GetFrontBody) "/Game/Blueprints/SkeletalSpriteAnimations/PonyAnims/FaceEffect/PonyAnim_StopFaceEffect1.PonyAnim_StopFaceEffect1_C")
  (Class|SkeletalSpriteBodyComponent|PlayAnimation (Variables|Default|GetBackBody) "/Game/Blueprints/SkeletalSpriteAnimations/PonyAnims_Back/FaceEffect/PonyAnim_Back_StopFaceEffect1.PonyAnim_Back_StopFaceEffect1_C")
  (bind _returnvalue (Utilities|Time|SetTimerbyEvent (delegate Custom|StartStamFlash) 0.01 true)))

(event Custom|SetDustActive_Multicast
  (params (Active :type Boolean))
  (Components|Activation|SetActive (Variables|Default|GetDust) Active false))

(event Custom|DoLandSoundMulticast
  (bind _returnvalue (Class|StaticFuncLib|PlaySound (Math|Transform|MakeTransform (Transformation|GetActorLocation) "0, 0, 0" "1,1,1") "/Game/Assets/Sound/LandStep_Cue.LandStep_Cue" 0.5))
  (if (!= (Pawn|GetController (.AsPawn (Utilities|Casting|CastToPawn (Components|GetOwner)))) (Game|GetPlayerController 0))
    (Audio|Components|Audio|AdjustAttenuation (Variables|/Script/MPHorso.OneShotAudio|GetaudioComp _returnvalue) (Variables|Default|GetAtten))
    (Audio|Components|Audio|Play (Variables|/Script/MPHorso.OneShotAudio|GetaudioComp _returnvalue) 0.0)
    (Transformation|AttachActorToActor _returnvalue self "None" "SnapToTarget" "KeepRelative" "KeepRelative" true))
  (Default|CallLandedDelegate))

(event Custom|PlayWalkAnimation
  (Development|PrintString "EntityBaseBP::PlayWalkAnimation: This function isn't supposed to be used! If you're making a new kind of entity, please override this function."))

(event Custom|TurnMagicOff
  (if (<= (Variables|Default|GetSustainedSpellsCount) 0)
    (CallFunction|PlayMagicOffAnimation)))

(event Custom|PlayStandAnimation
  (Development|PrintString "EntityBaseBP::PlayStandAnimation: This function isn't supposed to be used! If you're making a new kind of entity, please override this function."))

(event Custom|HandleStamFade
  (Rendering|Material|SetScalarParameterValue (UserInterface|GetMaterialInstance (Variables|Default|GetStamina)) "Fade" (Variables|/Game/Blueprints/UI/Stamina/StaminaWidget.StaminaWidget_C|GetCurrFade (Variables|Default|GetStamWidgRef)) :!class /Script/Engine.MaterialInstanceDynamic))

(event Custom|RevertPosition
  (Class|Pawn|ConsumeMovementInputVector)
  (Variables|/Script/Engine.MovementComponent|SetVelocity (Variables|Character|GetCharacterMovement) "0, 0, 0")
  (Transformation|SetActorLocation (+ (AI|Navigation|ProjectPointtoNavigation (Variables|Default|GetLastContactedLocation) 0 0 "1000.000000,1000.000000,1000.000000") (Math|Vector|MakeVector 0.0 0.0 (Components|Capsule|GetScaledCapsuleHalfHeight (Variables|Default|GetCapsuleComponent)))) false false))

(event Custom|OnStamCompletelyOut
  (Variables|StaminaCost|SetTired true)
  (Variables|StaminaCost|SetFlyTired true))

(event Custom|SetLookTarget
  (params (NewLookTarg :type Scene%20Component%20Object%20Reference))
  (Variables|Default|SetLookTarget NewLookTarg))

(event Custom|DoJump
  (params (Pressed :type Boolean))
  (bind _lastvalidfloor (Variables|Default|GetLastValidFloor))
  (bind _hitresult (Utilities|Struct|BreakFindFloorResult _lastvalidfloor))
  (if (and Pressed (Character|CanJump))
    (Utilities|IsValid (.hitactor _hitresult)
      (:Is%20Valid
        (if (and (Utilities|Enum|NotEqual(Enum) (Variables|/Script/Engine.SceneComponent|GetMobility (VehicleSound|GetRootComponent (.hitactor _hitresult))) "Movable") (not (Variables|Default|GetJumped)))
          (Variables|Default|SetLastContactedLocation (Transformation|GetActorLocation) :!label _label)))
      (:Is%20Not%20Valid
        (goto _label)))
    (Variables|Default|SetJumped true)
    (Math|Integer|IncrementInt (Variables|Default|GetJumpCount)
      (:%20%20
        (Character|Jump)))
    (else
      (Character|StopJumping))))

(event Custom|PlayMagicOnAnimation
  (Development|PrintString "EntityBaseBP::PlayMagicOnAnimation: This function isn't supposed to be used! If you're making a new kind of entity, please override this function."))

(event Custom|TurnMagicOn
  (if (<= (Variables|Default|GetSustainedSpellsCount) 0)
    (CallFunction|PlayMagiconAnimation)))

(event Custom|StartStamFlash
  (bind _output_get (Variables|StaminaCost|SetFlashTime (Math|Interpolation|FInterpTo (Variables|StaminaCost|GetFlashTime) 1.0 (Utilities|Time|GetWorldDeltaSeconds) 1e+01)))
  (Rendering|Material|SetScalarParameterValue (UserInterface|GetMaterialInstance (Variables|Default|GetStamina)) "Flash" _output_get :!class /Script/Engine.MaterialInstanceDynamic)
  (if (Math|Float|NearlyEqual(Float) _output_get 1.0 0.01)
    (Utilities|Time|ClearandInvalidateTimerbyHandle (stale Custom|OnStamFull _returnvalue))
    (bind _returnvalue (Utilities|Time|SetTimerbyEvent (delegate Custom|EndStamFlash) 0.01 true))))

(event Custom|SetRunning
  (params (Running :type Boolean))
  (if (not (Variables|StaminaCost|GetTired))
    (bind _output_get (Variables|StaminaCost|SetRunning Running))
    (if _output_get
      (Variables|Speed|SetCurrSpeed (Variables|Speed|GetRunSpeed))
      (else
        (Variables|Speed|SetCurrSpeed (Variables|Speed|GetWalkSpeed))))))

(event Custom|PlayJumpAnimation
  (Development|PrintString "EntityBaseBP::PlayJumpAnimation: This function isn't supposed to be used! If you're making a new kind of entity, please override this function."))

(event Custom|EndStamFlash
  (bind _output_get (Variables|StaminaCost|SetFlashTime (Math|Interpolation|FInterpTo (Variables|StaminaCost|GetFlashTime) 0.0 (Utilities|Time|GetWorldDeltaSeconds) 1e+01)))
  (Rendering|Material|SetScalarParameterValue (UserInterface|GetMaterialInstance (Variables|Default|GetStamina)) "Flash" _output_get :!class /Script/Engine.MaterialInstanceDynamic)
  (if (Math|Float|NearlyEqual(Float) _output_get 0.0 0.01)
    (Utilities|Time|ClearandInvalidateTimerbyHandle (stale Custom|StartStamFlash _returnvalue))
    (Variables|StaminaCost|SetFlashTime 0.0)
    (Rendering|Material|SetScalarParameterValue (UserInterface|GetMaterialInstance (Variables|Default|GetStamina)) "Flash" 0.0 :!class /Script/Engine.MaterialInstanceDynamic)))

(event Custom|PlayMagicOffAnimation
  (Development|PrintString "EntityBaseBP::PlayMagicOffAnimation: This function isn't supposed to be used! If you're making a new kind of entity, please override this function."))

(event Custom|ResetLook
  (Development|PrintString "EntityBaseBP::ResetLook: This function isn't supposed to be used! If you're making a new kind of entity, please override this function."))

(event Custom|MulticastJumpCountEdit
  (params (NewJumpCount :type Integer))
  (Variables|Default|SetJumpMaxCount NewJumpCount))

(event Custom|SetDustActive
  (params (Active :type Boolean))
  (CallFunction|SetDustActiveServer Active))

(event Custom|MakeGallopPoof
  (params (InputVec :type Vector))
  (CallFunction|MakeGallopPoofServer InputVec))

(event Custom|MakeGallopPoof_Server
  (params (InputVec :type Vector))
  (CallFunction|MakeGallopPoofMulticast InputVec))

(event Custom|MakeGallopPoof_Multicast
  (params (InputVec :type Vector))
  (Effects|SpawnEmitteratLocation "/Game/Assets/VFX/DustPoofGallop.DustPoofGallop" (Transformation|GetWorldLocation (Variables|Default|GetDust)) (Math|Rotator|MakeRotfromXZ InputVec (Math|Vector|MakeVector 0.0 0.0 1.0))))

(event Custom|MakeDustPoof
  (CallFunction|MakeDustPoofServer))

(event Custom|MakeDustPoof_Server
  (CallFunction|MakeDustPoofMulticast))

(event Custom|MakeDustPoof_Multicast
  (Effects|SpawnEmitteratLocation "/Game/Assets/VFX/DustPoof.DustPoof" (Transformation|GetWorldLocation (Variables|Default|GetDust))))

(event Custom|PlayGallopAnimation
  (Development|PrintString "EntityBaseBP::PlayGallopAnimation: This function isn't supposed to be used! If you're making a new kind of entity, please override this function."))

(event Custom|Move
  (params (WorldDir :type Vector) (ScaleVal :type Float%20%28single-precision%29))
  (Pawn|Input|AddMovementInput WorldDir ScaleVal false)
  (CallFunction|DoMoveFace (* WorldDir ScaleVal)))

(event Custom|SetDustActive_Server
  (params (Active :type Boolean))
  (CallFunction|SetDustActiveMulticast Active))

(event Custom|Look
  (Development|PrintString "EntityBaseBP::Look: This function isn't supposed to be used! If you're making a new kind of entity, please override this function."))

(event Custom|BindStaminaWidget
  (bind _output_get (Variables|Default|SetStamWidgRef (.AsStamina%20Widget (Utilities|Casting|CastToStaminaWidget (UserInterface|GetUserWidgetObject (Variables|Default|GetStamina))))))
  (EventDispatchers|AssignStamOut _output_get (delegate Custom|OnStamOut))
  (EventDispatchers|AssignStamFull _output_get (delegate Custom|OnStamFull))
  (EventDispatchers|AssignStamCompletelyOut _output_get (delegate Custom|OnStamCompletelyOut))
  (Utilities|Time|SetTimerbyEvent (delegate Custom|HandleStamFade) 0.01 true))

(event EventBeginPlay
  (Variables|Speed|SetCurrSpeed (Variables|Speed|GetWalkSpeed))
  (CallFunction|BindStaminaWidget)
  (bind _asname_tag_widget (Utilities|Casting|CastToNameTagWidget (UserInterface|GetUserWidgetObject (Variables|Default|GetNameTag))))
  (bind _asobserver_bp (Utilities|Casting|CastToObserverBP (Components|GetOwner)))
  (Variables|/Game/Blueprints/UI/NameTagWidget.NameTagWidget_C|SetObsRef _asname_tag_widget _asobserver_bp)
  (bind _asspeech_test (Utilities|Casting|CastToSpeechTest (UserInterface|GetUserWidgetObject (Variables|Default|GetSpeechBubble))))
  (Variables|/Game/Blueprints/UI/SpeechTest.SpeechTest_C|SetParentEntity _asspeech_test self)
  (Variables|Default|SetLastContactedLocation (Transformation|GetActorLocation))
  (CallFunction|SetColors (Variables|Default|GetColorSchemeNames) (Variables|Default|GetColorSchemeColors))
  (Utilities|Time|SetTimerbyFunctionName 0 "Blink" 0.1 true))

(event EventOnLanded
  (params (Hit :type Hit%20Result%20Structure%20%28by%20ref%29))
  (Variables|Default|SetJumped false)
  (CallFunction|PlayStandAnimation)
  (CallFunction|SetDustActive true)
  (CallFunction|MakeDustPoof)
  (CallFunction|DoLandSoundMulticast))

(event EventOnWalkingOffLedge
  (params (PreviousFloorImpactNormal :type Vector%20%28by%20ref%29) (PreviousFloorContactNormal :type Vector%20%28by%20ref%29) (PreviousLocation :type Vector%20%28by%20ref%29) (TimeDelta :type Float%20%28single-precision%29))
  (bind _lastvalidfloor (Variables|Default|GetLastValidFloor))
  (bind _hitresult (Utilities|Struct|BreakFindFloorResult _lastvalidfloor))
  (CallFunction|SetDustActive false)
  (CallFunction|DoFixingJump)
  (Utilities|IsValid (.hitactor _hitresult)
    (:Is%20Valid
      (if (Utilities|Enum|NotEqual(Enum) (Variables|/Script/Engine.SceneComponent|GetMobility (VehicleSound|GetRootComponent (.hitactor _hitresult))) "Movable")
        (Variables|Default|SetLastContactedLocation PreviousLocation :!label _label)))
    (:Is%20Not%20Valid
      (goto _label)))
  (CallFunction|PlayJumpAnimation)
  (|CallParentFunction PreviousFloorImpactNormal PreviousFloorContactNormal PreviousLocation TimeDelta))

(event MouseInput|EventActorEndCursorOver)

(event EventTick
  (params (DeltaSeconds :type Float%20%28single-precision%29))
  (CallFunction|UpdateWalkSpeed)
  (CallFunction|UpdateRunningCost)
  (CallFunction|Face)
  (CallFunction|UpdateLastValidFloor)
  (Variables|Default|GetLookTarget
    (:then
      (CallFunction|Look)
      (goto _label Reset))
    (:else
      (Utilities|FlowControl|DoOnce false :!label _label
        (:Completed
          (CallFunction|ResetLook))))))

(event MouseInput|EventActorBeginCursorOver)

(event EventOnJumped
  (|CallParentFunction)
  (CallFunction|SetDustActive false))

(fn ConstructionScript
  (Variables|/Game/Blueprints/UI/Stamina/StaminaWidget.StaminaWidget_C|SetFocus (.AsStamina%20Widget (Utilities|Casting|CastToStaminaWidget (UserInterface|GetUserWidgetObject (Variables|Default|GetStamina)))) self))

(fn Face
  (bind _returnvalue (Class|StaticFuncLib|RetrieveGameInstance))
  (bind _backbody (Variables|Default|GetBackBody))
  (bind _frontbody (Variables|Default|GetFrontBody))
  (bind _returnvalue_2 (Class|MPHorsoGameInstance|GetRelevantCamera _returnvalue))
  (bind _returnvalue_3 (Math|Vector|GetUpVector _frontbody))
  (bind _returnvalue_4 (Math|Vector|GetForwardVector _returnvalue_2))
  (bind _returnvalue_5 (Math|Vector|NegateVector _returnvalue_4))
  (bind _returnvalue_6 (Math|Rotator|MakeRotfromZY _returnvalue_3 _returnvalue_5))
  (bind _returnvalue_7 (Math|Rotator|CombineRotators _returnvalue_6 "0,90.000000, 0"))
  (if (not (Networking|IsDedicatedServer))
    (Utilities|IsValid _returnvalue_2
      (:Is%20Valid
        (Utilities|FlowControl|Sequence
          (:then_0
            (Transformation|SetWorldRotation _frontbody _returnvalue_6 false false)
            (Transformation|SetWorldRotation (Variables|Default|GetSpeechBubble) _returnvalue_7 false false)
            (Transformation|SetWorldRotation (Variables|Default|GetStamAnchor) _returnvalue_7 false false))
          (:then_1
            (Transformation|SetWorldRotation _backbody (Math|Rotator|MakeRotfromZY (Math|Vector|GetUpVector _backbody) _returnvalue_5) false false)))))))

(fn DoMoveFace
  (params (HeadingVector :type Vector))
  (bind _returnvalue (Class|StaticFuncLib|RetrieveGameInstance))
  (bind _returnvalue_2 (Class|MPHorsoGameInstance|GetRelevantCamera _returnvalue))
  (bind _returnvalue_3 (Math|Vector|GetRightVector _returnvalue_2))
  (bind _returnvalue_4 (Math|Vector|GetForwardVector _returnvalue_2))
  (bind _returnvalue_5 (Math|Vector|DotProduct HeadingVector _returnvalue_4))
  (bind _returnvalue_6 (Math|Vector|DotProduct HeadingVector _returnvalue_3))
  (bind _returnvalue_7 (Math|Float|Sign(Float) _returnvalue_5))
  (bind _returnvalue_8 (Math|Float|Sign(Float) _returnvalue_6))
  (bind _returnvalue_9 (> _returnvalue_7 0.0))
  (Utilities|IsValid _returnvalue_2
    (:Is%20Valid
      (if (and (!= _returnvalue_8 0.0) (> (Math|Float|Absolute(Float) _returnvalue_6) 0.1))
        (Transformation|SetRelativeScale3D (Variables|Default|GetFrontBody) (Math|Vector|MakeVector _returnvalue_8 1.0 1.0))
        (Transformation|SetRelativeLocation (Variables|Default|GetStamina) (Math|Vector|MakeVector 0.0 (* _returnvalue_8 62.0) 46.0) false false)
        (Widget|Transform|SetRenderScale (Variables|/Game/Blueprints/UI/Stamina/StaminaWidget.StaminaWidget_C|GetDotPanel (Variables|Default|GetStamWidgRef)) (Math|Vector2D|MakeVector2D _returnvalue_8 1.0)))
      (if (and (!= _returnvalue_7 0.0) (> (Math|Float|Absolute(Float) _returnvalue_5) 0.1))
        (Rendering|SetVisibility (Variables|Default|GetFrontBody) (not _returnvalue_9) true)
        (Rendering|SetVisibility (Variables|Default|GetBackBody) _returnvalue_9 true)))))

(fn OnRepJumped
  (if (not (Variables|Default|GetJumped))
    (CallFunction|PlayStandAnimation)
    (Variables|Default|SetJumpCount 0)))

(fn UpdateLastValidFloor
  (bind _charactermovement (Variables|Character|GetCharacterMovement))
  (bind _currentfloor (Variables|/Script/Engine.CharacterMovementComponent|GetCurrentFloor _charactermovement))
  (Utilities|IsValid (.HitActor (Collision|BreakHitResult (Utilities|Struct|BreakFindFloorResult _currentfloor)))
    (:Is%20Valid
      (Variables|Default|SetLastValidFloor _currentfloor))))

(fn DoFixingJump
  (LocalVariables|SetStoredLCL (Variables|Default|GetLastContactedLocation))
  (CallFunction|DoJump true)
  (CallFunction|DoJump false)
  (Variables|Default|SetLastContactedLocation (LocalVariables|GetStoredLCL)))

(fn Blink
  (if (Math|Boolean|ANDBoolean (Variables|Blink|GetShouldBlink) (not (Utilities|Time|IsValidTimerHandle (Variables|Blink|GetBlinkCooldown))) (< (Math|Random|RandomFloat) 0.01))
    (Class|SkeletalSpriteBodyComponent|PlayAnimation (Variables|Default|GetFrontBody) "/Game/Blueprints/SkeletalSpriteAnimations/PonyAnims/Eye/PonyAnim_Blink.PonyAnim_Blink_C")
    (bind _returnvalue (Utilities|Time|SetTimerbyFunctionName 0 "BlinkCool" (LocalVariables|GetCooldown)))
    (Variables|Blink|SetBlinkCooldown _returnvalue)))

(fn BlinkCool
  (Utilities|Time|InvalidateTimerHandle (Variables|Blink|GetBlinkCooldown)))

(fn GetMagicTip
  (return 0))

(fn DestroyComponentProxy
  (params (Component :type Actor%20Component%20Object%20Reference))
  (Components|DestroyComponent Component))

(fn UpdateSustainedSpells
  (params (SpellName :type Name) (Add :type Boolean))
  (bind _sustainedspells (Variables|Default|GetSustainedSpells))
  (if Add
    (Utilities|Set|Add _sustainedspells SpellName)
    (else
      (Utilities|Set|Remove _sustainedspells SpellName)))
  (Variables|Default|SetSustainedSpellsCount (Utilities|Set|Length (Variables|Default|GetSustainedSpells))))

(fn SustainedSpellsContains
  (params (SpellName :type Name))
  (return (Utilities|Set|Contains (Variables|Default|GetSustainedSpells) SpellName)))

(fn HandleDropShadow)

(fn SetColors
  (params (ColorSchemeNames :type Array%20of%20Names) (ColorSchemeColors :type Array%20of%20Linear%20Color%20Structures))
  (Variables|Default|SetColorSchemeNames ColorSchemeNames)
  (Variables|Default|SetColorSchemeColors ColorSchemeColors)
  (for (_array_element _array_index) ColorSchemeNames
    (bind (_retrievedbone _returnvalue) (Class|SkeletalSpriteBodyComponent|GetBone (Variables|Default|GetFrontBody) _array_element))
    (if _returnvalue
      (Sprite|SetSpriteColor _retrievedbone (Utilities|Array|Get(acopy) ColorSchemeColors _array_index))
      (else
        (bind (_retrievedbone_2 _returnvalue_2) (Class|SkeletalSpriteBodyComponent|GetBone (Variables|Default|GetBackBody) _array_element))
        (if _returnvalue_2
          (Sprite|SetSpriteColor _retrievedbone_2 (Utilities|Array|Get(acopy) ColorSchemeColors _array_index)))))))

(fn UpdateWalkSpeed
  (bind _charactermovement (Variables|Character|GetCharacterMovement))
  (if (not (Math|Float|NearlyEqual(Float) (Variables|Speed|GetCurrSpeed) (Variables|/Script/Engine.CharacterMovementComponent|GetMaxWalkSpeed (Variables|Character|GetCharacterMovement)) 0.01))
    (Variables|/Script/Engine.CharacterMovementComponent|SetMaxWalkSpeed _charactermovement (Math|Interpolation|FInterpTo (Variables|/Script/Engine.CharacterMovementComponent|GetMaxWalkSpeed _charactermovement) (Variables|Speed|GetCurrSpeed) (Utilities|Time|GetWorldDeltaSeconds) 4.0))
    (if (Math|Float|NearlyEqual(Float) (Variables|Speed|GetCurrSpeed) (Variables|/Script/Engine.CharacterMovementComponent|GetMaxWalkSpeed (Variables|Character|GetCharacterMovement)) 0.01)
      (Variables|/Script/Engine.CharacterMovementComponent|SetMaxWalkSpeed (Variables|Character|GetCharacterMovement) (Variables|Speed|GetCurrSpeed)))))

(fn UpdateRunningCost
  (bind _returnvalue (Class|Pawn|GetLastMovementInputVector))
  (if (Variables|StaminaCost|GetRunning)
    (if (> (Math|Vector|VectorLength _returnvalue) 0.0)
      (if (not (Variables|StaminaCost|GetRunCostApplied))
        (Variables|Default|SetKeptInput _returnvalue)
        (Variables|StaminaCost|SetRunCostApplied true))
      (elif (Variables|StaminaCost|GetRunCostApplied)
        (Variables|StaminaCost|SetRunCostApplied false)))
    (elif (Variables|StaminaCost|GetRunCostApplied)
      (Variables|StaminaCost|SetRunCostApplied false))))

(fn OnRepRunCostApplied
  (if (Variables|StaminaCost|GetRunCostApplied)
    (Default|DepleteStamina (Variables|Default|GetStamWidgRef) "Run" (Utilities|Struct|MakeStaminaCost (Variables|StaminaCost|GetRunCost) true))
    (if (and (Utilities|Enum|Equal(Enum) (Class|Actor|GetRemoteRole) "ROLE_SimulatedProxy") (AI|Components|NavMovement|IsMovingonGround (Variables|Character|GetCharacterMovement)))
      (CallFunction|MakeGallopPoof (Variables|Default|GetKeptInput)))
    (else
      (Default|StopContinuousDepletion (Variables|Default|GetStamWidgRef) "Run"))))

(fn OnRepKeptInput
  (Variables|StaminaCost|SetRunCostApplied true))

(fn KillSustainedSpells
  (bind _sustainedspells (Variables|Default|GetSustainedSpells))
  (bind _result (Utilities|Set|ToArray _sustainedspells))
  (for _array_element _result
    (bind _retrievedspell (Class|MagicActionsLibrary|GetSpell _array_element))
    (Class|MagicActionsLibrary|ExecuteSpell (Components|GetOwner) _retrievedspell))
  (Utilities|Set|Clear _sustainedspells)
  (CallFunction|TurnMagicOff))

(fn IsCurrentlyManipulable
  (params (Querier :type Controller%20Object%20Reference))
  (return true))